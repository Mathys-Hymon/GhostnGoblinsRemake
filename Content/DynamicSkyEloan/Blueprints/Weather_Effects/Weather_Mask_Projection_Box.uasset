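; Placeable weather mask projection box actor that configures a projection component to mask snow/dust and wetness within a box volume.
; The construction script keeps rotation yaw-only, scales the component from the box extent, copies mask, blur, capture pixel size and occlusion-exclusion settings, then triggers an editor update.
; Helper functions force a component update and open the weather mask readme on the level's Ultra Dynamic Weather actor.
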(fn `Force Update`
  (`/Game/DynamicSkyEloan/Blueprints/Weather_Effects/System/WeatherMask.Force Update` (`self.Weather_Mask_Projection_Box_Component`)))

(fn `UserConstructionScript`
  (`self.K2_SetActorRotation` (`KismetMathLibrary.MakeRotator` 0.0 0.0 (.yaw (`self.K2_GetActorRotation`))))
  (`SceneComponent.SetRelativeScale3D` (`self.Weather_Mask_Projection_Box_Component`) (/ (`self.Box Extent`) 50.0))
  (set `/Game/DynamicSkyEloan/Blueprints/Weather_Effects/System/WeatherMask.Mask Snow/Dust` (`self.Mask Snow / Dust`) (`self.Weather_Mask_Projection_Box_Component`))
  (set `/Game/DynamicSkyEloan/Blueprints/Weather_Effects/System/WeatherMask.Mask Wetness` (`self.Mask Wetness`) (`self.Weather_Mask_Projection_Box_Component`))
  (set `/Game/DynamicSkyEloan/Blueprints/Weather_Effects/Components/Weather_Mask_Projection_Box_Component.Blur Radius` (`self.Blur Radius`) (`self.Weather_Mask_Projection_Box_Component`))
  (set `/Game/DynamicSkyEloan/Blueprints/Weather_Effects/Components/Weather_Mask_Projection_Box_Component.Blur Slope (Snow/Dust)` (`self.Blur Slope (Snow/Dust)`) (`self.Weather_Mask_Projection_Box_Component`))
  (set `/Game/DynamicSkyEloan/Blueprints/Weather_Effects/Components/Weather_Mask_Projection_Box_Component.Blur Slope (Wetness)` (`self.Blur Slope (Wetness)`) (`self.Weather_Mask_Projection_Box_Component`))
  (set `/Game/DynamicSkyEloan/Blueprints/Weather_Effects/Components/Weather_Mask_Projection_Box_Component.Capture Pixel Size` (`self.Capture Pixel Size`) (`self.Weather_Mask_Projection_Box_Component`))
  (set `/Game/DynamicSkyEloan/Blueprints/Weather_Effects/Components/Weather_Mask_Projection_Box_Component.Exclude Actors from Occlusion` (`self.Exclude Actors from Occlusion`) (`self.Weather_Mask_Projection_Box_Component`))
  (`/Game/DynamicSkyEloan/Blueprints/Weather_Effects/System/WeatherMask.Editor Update` (`self.Weather_Mask_Projection_Box_Component`)))

(fn `📘 Weather Mask Tools`
  (bind _returnvalue (`GameplayStatics.GetActorOfClass` "/Game/DynamicSkyEloan/Blueprints/Ultra_Dynamic_Weather.Ultra_Dynamic_Weather_C"))
  (`/Engine/EditorBlueprintResources/StandardMacros.IsValid` _returnvalue
    (:`Is Valid`
      (`/Game/DynamicSkyEloan/Blueprints/Ultra_Dynamic_Weather.Open Editor Readme Entry` _returnvalue "WeatherMaskBrushes"))))