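; Placeable brush actor for Ultra Dynamic Weather that masks snow/dust and wetness through its Weather Mask Brush component.
; Construction keeps only the actor's yaw, zeroing pitch and roll, then copies the brush, mask and cancel-masks-above settings to the component and triggers its editor update.
; A Weather Mask Tools function finds the weather actor and opens its readme entry on mask brushes.
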(fn `UserConstructionScript`
  (`self.K2_SetActorRotation` (`KismetMathLibrary.MakeRotator` 0.0 0.0 (.yaw (`self.K2_GetActorRotation`))))
  (set `/Game/DynamicSkyEloan/Blueprints/Weather_Effects/Components/Weather_Mask_Brush_Component.Cancel Masks Above` (`self.Cancel Masks Above`) (`self.Weather_Mask_Brush_Component`))
  (set `/Game/DynamicSkyEloan/Blueprints/Weather_Effects/System/WeatherMask.Mask Snow/Dust` (`self.Mask Snow/Dust`) (`self.Weather_Mask_Brush_Component`))
  (set `/Game/DynamicSkyEloan/Blueprints/Weather_Effects/System/WeatherMask.Mask Wetness` (`self.Mask Wetness`) (`self.Weather_Mask_Brush_Component`))
  (set `/Game/DynamicSkyEloan/Blueprints/Weather_Effects/Components/Weather_Mask_Brush_Component.Brush` (`self.Brush`) (`self.Weather_Mask_Brush_Component`))
  (`/Game/DynamicSkyEloan/Blueprints/Weather_Effects/System/WeatherMask.Editor Update` (`self.Weather_Mask_Brush_Component`)))

(fn `📘 Weather Mask Tools`
  (bind _returnvalue (`GameplayStatics.GetActorOfClass` "/Game/DynamicSkyEloan/Blueprints/Ultra_Dynamic_Weather.Ultra_Dynamic_Weather_C"))
  (`/Engine/EditorBlueprintResources/StandardMacros.IsValid` _returnvalue
    (:`Is Valid`
      (`/Game/DynamicSkyEloan/Blueprints/Ultra_Dynamic_Weather.Open Editor Readme Entry` _returnvalue "WeatherMaskBrushes"))))