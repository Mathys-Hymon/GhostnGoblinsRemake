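; Ultra Dynamic Sky cloud paint container that links itself to the sky actor for painted cloud coverage.
; On BeginPlay it finds the sky and, only in one specific run context, registers itself and updates the painted coverage target.
; When destroyed or removed from the world, it clears the sky's reference and notifies it of the removal.
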(event `self.ReceiveBeginPlay`
  (bind _returnvalue (`GameplayStatics.GetActorOfClass` "/Game/DynamicSkyEloan/Blueprints/Ultra_Dynamic_Sky.Ultra_Dynamic_Sky_C"))
  (`/Engine/EditorBlueprintResources/StandardMacros.IsValid` _returnvalue
    (:`Is Valid`
      (if (`|EnumEquality` (`/Game/DynamicSkyEloan/Blueprints/Ultra_Dynamic_Sky.Run Context` _returnvalue) "NewEnumerator3")
        (set `/Game/DynamicSkyEloan/Blueprints/Ultra_Dynamic_Sky.Cloud Paint Container` self _returnvalue)
        (`/Game/DynamicSkyEloan/Blueprints/Ultra_Dynamic_Sky.Update Painted Cloud Coverage Target` _returnvalue)))))

(event `self.ReceiveEndPlay`
  (params (EndPlayReason :type "EEndPlayReason Enum" :default "Destroyed"))
  (if (`KismetArrayLibrary.Array_Contains` (`|MakeArray` "Destroyed" "RemovedFromWorld" :!type "EEndPlayReason Enum") EndPlayReason)
    (bind _returnvalue (`GameplayStatics.GetActorOfClass` "/Game/DynamicSkyEloan/Blueprints/Ultra_Dynamic_Sky.Ultra_Dynamic_Sky_C"))
    (`/Engine/EditorBlueprintResources/StandardMacros.IsValid` _returnvalue
      (:`Is Valid`
        (set `/Game/DynamicSkyEloan/Blueprints/Ultra_Dynamic_Sky.Cloud Paint Container` null _returnvalue)
        (`/Game/DynamicSkyEloan/Blueprints/Ultra_Dynamic_Sky.Notify of Removed Cloud Paint Container` _returnvalue)))))

(fn `UserConstructionScript`)