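; UDS_RenderTarget_State tracks the world-space placement of a square render target for the Dynamic Sky system.
; It stores the target, buffer, resolution, size and center, returning a linear color that packs corner, size and height.
; Helpers convert world positions and sizes into canvas pixels for brush drawing.
; A recenter check flags when an axis-masked control location drifts over a tenth of the size from center.
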(fn `Canvas Brush Location`
  (params (In :type "Vector2D Structure"))
  (returns (Out :type "Vector2D Structure"))
  (return (/ (- In (`self.Top Corner 2D`)) (`self.Size to Res Ratio`))))

(fn `Canvas Brush Size`
  (params (In :type "Vector2D Structure"))
  (returns (Out :type "Vector2D Structure"))
  (return (/ In (`self.Size to Res Ratio`))))

(fn `Set Location`
  (params (`Center Location` :type "Vector Structure"))
  (returns (`Mapping Vector4` :type "LinearColor Structure"))
  (bind (_x _y) (`KismetMathLibrary.BreakVector2D` (`self.Top Corner 2D`)))
  (bind _output_get (set `self.Center Location` `Center Location`))
  (set `self.Top Corner` (- _output_get (`self.Half Size`)))
  (set `self.Center 2D` (`KismetMathLibrary.Conv_VectorToVector2D` (`self.Center Location`)))
  (set `self.Top Corner 2D` (`KismetMathLibrary.Conv_VectorToVector2D` (`self.Top Corner`)))
  (return (make `LinearColor` _x _y (`self.Size`) (.z (`self.Center Location`)))))

(fn `Set Render Target`
  (params (`Render Target` :type "TextureRenderTarget2D Object Reference") (`Buffer Target` :type "TextureRenderTarget2D Object Reference"))
  (set `self.Render Target` `Render Target`)
  (set `self.Buffer Target` `Buffer Target`)
  (set `self.Resolution` (`TextureRenderTarget2D.SizeX` (`self.Render Target`))))

(fn `Set Size`
  (params (Size :type "Float (double-precision)"))
  (bind _output_get (set `self.Size` Size))
  (set `self.Half Size` (/ _output_get 2.0))
  (set `self.Size to Res Ratio` (/ (`self.Size`) (`KismetMathLibrary.Conv_IntToDouble` (`self.Resolution`)))))

(fn `Target Extent 2D`
  (returns (Extent :type "Vector2D Structure"))
  (bind _returnvalue (/ (`self.Size`) 2.0))
  (return (`KismetMathLibrary.MakeVector2D` _returnvalue _returnvalue)))

(fn `Target Needs Recenter`
  (params (`Control Location` :type "Vector Structure") (`Axis Mask` :type "Vector Structure"))
  (returns (Yes :type Boolean))
  (return (> (`KismetMathLibrary.Vector_GetAbsMax` (* (- `Control Location` (`self.Center Location`)) (`local.Axis Mask`))) (/ (`self.Size`) 10.0))))