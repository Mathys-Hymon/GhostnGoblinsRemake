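; BP_Danger is an actor that follows the player and points toward a referenced object, apparently as a danger direction indicator.
; On BeginPlay it attaches to the player character, keeping its world transform.
; Each tick it rotates along the look-at direction from the player to ParentObjectRef, and destroys itself once that reference is invalid.
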(event `self.ReceiveBeginPlay`
  (`self.K2_AttachToActor` (`GameplayStatics.GetPlayerCharacter` 0) "None" "KeepWorld" "KeepWorld" "KeepWorld"))

(event `self.ReceiveTick`
  (params (DeltaSeconds :type "Float (single-precision)"))
  (`/Engine/EditorBlueprintResources/StandardMacros.IsValid` (`self.parentObjectRef`)
    (:`Is Valid`
      (`self.K2_SetActorRotation` (`KismetMathLibrary.FindLookAtRotation` (`self.K2_GetActorLocation` (`GameplayStatics.GetPlayerCharacter` 0)) (`self.K2_GetActorLocation` (`self.parentObjectRef`)))))
    (:`Is Not Valid`
      (`self.K2_DestroyActor`))))

(fn `UserConstructionScript`)