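; BP_ArmorPiece is a loose physics prop for a piece of player armor or a skeleton part, using an assigned static mesh.
; On BeginPlay it enables physics and, unless IsSkeleton is set, applies a fixed impulse at the player pawn's location to launch it.
; After a delay, skeleton pieces stop simulating and remain in the world, while other pieces destroy themselves.
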(event `self.ReceiveBeginPlay`
  (bind _armorpiece (`self.ArmorPiece`))
  (`StaticMeshComponent.SetStaticMesh` (`self.ArmorPiece`) (`self.staticMesh`))
  (`PrimitiveComponent.SetSimulatePhysics` _armorpiece true)
  (if (not (`self.isSkeleton`))
    (`PrimitiveComponent.AddImpulseAtLocation` _armorpiece (5000.0 5000.0 10000.0) (`self.K2_GetActorLocation` (`GameplayStatics.GetPlayerPawn` 0)) "None"))
  (`KismetSystemLibrary.Delay` 20.0)
  (if (`self.isSkeleton`)
    (`PrimitiveComponent.SetSimulatePhysics` (`self.ArmorPiece`) false)
    (else
      (`self.K2_DestroyActor`))))

(fn `UserConstructionScript`)