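; Player ultimate component that charges from collected souls and unleashes an area beam attack around the player.
; AddSouls counts up to the data asset cost, then enables Use and plays a bar-full sound.
; Use resets and pauses soul gain, spawns beam FX, decal, field actor, sound and rumble, and loops a damage timer for the duration.
; Each tick capsule-traces around the player, applying damage interpolated by distance.
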(event `Add Souls`
  ;[0 0 0] Add souls to player
  (if (`self.canGetSouls`)
    (bind _result (`/Engine/EditorBlueprintResources/StandardMacros.IncrementInt` (`self.souls`))
      (:`  `
        (if (>= _result (`/Game/_Manager/InGame/DataAsset/BP/BP_PlayerDA.ultCost` (`self.dataAsset`)))
          (set `self.canUlt` true)
          (`/Engine/EditorBlueprintResources/StandardMacros.DoOnce` false :!label _label
            (:`Completed`
              (`GameplayStatics.PlaySound2D` (`KismetArrayLibrary.Array_Random` (`/Game/_Manager/InGame/DataAsset/BP/SFX/BP_SFX_DA.ultBarFull` (`self.sfxDataAsset`))) 1.0 1.0 0.0 null null)))
          (else
            (set `self.canUlt` false)
            (goto _label :!via `Reset`)))))))

(event `Use`
  (bind _dataasset (`self.dataAsset`))
  (bind _returnvalue (`Actor.K2_GetActorLocation` (`GameplayStatics.GetPlayerPawn` 0)))
  (bind _ultradius (`/Game/_Manager/InGame/DataAsset/BP/BP_PlayerDA.ultRadius` (`self.dataAsset`)))
  (bind _ultduration (`/Game/_Manager/InGame/DataAsset/BP/BP_PlayerDA.ultDuration` _dataasset))
  (bind _returnvalue_2 (/ (`/Game/_Manager/InGame/DataAsset/BP/BP_PlayerDA.ultHeight` _dataasset) 400.0))
  (bind _returnvalue_3 (/ _ultradius 110.0))
  ;[0 0 0] Find all enemy in range
  (if (`self.canUlt`)
    (`|ExecutionSequence`
      (:`then_0`
        (`KismetSystemLibrary.Delay` (`/Game/_Manager/InGame/DataAsset/BP/BP_PlayerDA.ultDelay` (`self.dataAsset`)))
        (`self.ResetGamepadRumble`)
        (set `self.canGetSouls` false)
        (set `self.canUlt` false)
        (set `self.souls` 0)
        (bind _returnvalue_4 (`KismetSystemLibrary.K2_SetTimerDelegate` (delegate `dealDamage`) 0.1 true true))
        (`|ExecutionSequence`
          (:`then_0`
            (bind _returnvalue_5 (`GameplayStatics.SpawnSound2D` (`KismetArrayLibrary.Array_Random` (`/Game/_Manager/InGame/DataAsset/BP/SFX/BP_SFX_DA.ultimateFX` (`self.sfxDataAsset`))) 1.0 1.0 0.0 null))
            (`KismetSystemLibrary.Delay` _ultduration)
            (`AudioComponent.FadeOut` _returnvalue_5 0.2 0.0 "Linear")
            (`KismetSystemLibrary.K2_PauseTimerHandle` _returnvalue_4)
            (set `self.canGetSouls` true)
            (message `/Game/Blueprints/BPI/Player/BPI_Player.ResetHealth` (`GameplayStatics.GetPlayerPawn` 0)))
          (:`then_1`
            (bind _returnvalue_6 (`NiagaraFunctionLibrary.SpawnSystemAtLocation` "/Game/Imports/VFX/FX_ult/NS_GIGABeam.NS_GIGABeam" _returnvalue (struct) (1.0 1.0 1.0) true true "AutoRelease"))
            (`SceneComponent.SetRelativeScale3D` _returnvalue_6 (`KismetMathLibrary.MakeVector` _returnvalue_2 _returnvalue_2 1.0))
            (`FXSystemComponent.SetFloatParameter` _returnvalue_6 "durationUlt" _ultduration)
            (bind _returnvalue_7 (`|SpawnActorFromClass` "/Game/Blueprints/BP_MasterDecal.BP_MasterDecal_C" (`KismetMathLibrary.MakeTransform` _returnvalue) "AlwaysSpawn" "MultiplyWithRoot" null null))
            (bind _output_get (set `self.decalActor` _returnvalue_7))
            (bind _decal (`/Game/Blueprints/BP_MasterDecal.Decal` _output_get))
            (`DecalComponent.SetDecalMaterial` _decal "/Game/Imports/VFX/FX_ult/MI_ImpactDecalUlt.MI_ImpactDecalUlt")
            (`SceneComponent.SetRelativeScale3D` _decal (`KismetMathLibrary.MakeVector` 1.0 _returnvalue_3 _returnvalue_3))
            (`Actor.SetLifeSpan` _output_get 15.0)
            (bind _returnvalue_8 (`|SpawnActorFromClass` "/Engine/EditorResources/FieldNodes/FS_MasterField.FS_MasterField_C" (`KismetMathLibrary.MakeTransform` _returnvalue (struct) (`KismetMathLibrary.Conv_DoubleToVector` (/ _ultradius 50.0))) "AlwaysSpawn" "MultiplyWithRoot" null null))
            (`Actor.SetLifeSpan` _returnvalue_8 4.0))))
      (:`then_1`
        (`/Engine/EditorBlueprintResources/StandardMacros.DoOnce` false :!label _label_2
          (:`Completed`
            (message `/Game/Blueprints/BPI/PlayerController/BPI_PlayerController.PlayGamepadRumble` (`GameplayStatics.GetPlayerController` 0) "/Game/Haptics/FFE_Ultimate.FFE_Ultimate" false)))))))

(event `ResetGamepadRumble`
  ;[0 0 0] Find all enemy in range
  (goto _label_2 :!via `Reset`))

(event `dealDamage`
  (bind _dataasset (`self.dataAsset`))
  (bind _dataasset_2 (`self.dataAsset`))
  (bind _ultheight (`/Game/_Manager/InGame/DataAsset/BP/BP_PlayerDA.ultHeight` _dataasset_2))
  (bind _returnvalue (+ (`Actor.K2_GetActorLocation` (`GameplayStatics.GetPlayerCharacter` 0)) (`KismetMathLibrary.MakeVector` 0.0 0.0 (+ _ultheight (`/Game/_Manager/InGame/DataAsset/BP/BP_PlayerDA.ultZOffset` _dataasset_2)))))
  ;[0 0 0] Find all enemy in range
  (bind _debugmode (message `/Game/Blueprints/BPI/GameInstance/BPI_GameInstance.GetDebugMode` (`GameplayStatics.GetGameInstance`)))
  (bind _outhits (`KismetSystemLibrary.CapsuleTraceMulti` :`Start` _returnvalue :`End` _returnvalue :`Radius` (`/Game/_Manager/InGame/DataAsset/BP/BP_PlayerDA.ultRadius` _dataasset_2) :`HalfHeight` _ultheight :`TraceChannel` "TraceTypeQuery3" :`DrawDebugType` (select `bool` _debugmode :`true` "ForDuration" :!type "EDrawDebugTrace Enum")))
  ;;[0 0 0] Apply damage
  (for _array_element _outhits
    (bind (_bblockinghit _binitialoverlap _time _distance _location _impactpoint _normal _impactnormal _physmat _hitactor) (`GameplayStatics.BreakHitResult` _array_element))
    (`GameplayStatics.ApplyDamage` _hitactor (`KismetMathLibrary.Lerp` (`/Game/_Manager/InGame/DataAsset/BP/BP_PlayerDA.maxUltDamage` _dataasset) (`/Game/_Manager/InGame/DataAsset/BP/BP_PlayerDA.minUltDamage` _dataasset) (/ (`KismetMathLibrary.Vector_Distance` (`Actor.K2_GetActorLocation` (`GameplayStatics.GetPlayerPawn` 0)) _impactpoint) (`/Game/_Manager/InGame/DataAsset/BP/BP_PlayerDA.ultRadius` (`self.dataAsset`)))) null null "/Game/Blueprints/Characters/Player/BP_UltDamageType.BP_UltDamageType_C")))