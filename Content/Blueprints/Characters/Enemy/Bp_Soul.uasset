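; Soul orb pickup that charges the player's ultimate when absorbed.
; It spawns under physics until a downward trace finds the floor, then bobs on a sine wave with a random time offset.
; Once the player enters the absorb radius, damped acceleration pulls it in with an orbiting effect.
; Sphere overlap with the player consumes it only at low velocity, letting fast orbs circle first.
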(event `self.ReceiveBeginPlay`
  (set `self.randomOffset` (`KismetMathLibrary.RandomFloat`)))

(event `self.ReceiveTick`
  (params (DeltaSeconds :type "Float (single-precision)"))
  (bind _returnvalue (`self.K2_GetActorLocation`))
  (bind _sphere (`self.Sphere`))
  (bind _returnvalue_2 (`SceneComponent.GetRelativeTransform` (`self.Sphere`)))
  (if (`self.initialSpawn`)
    ;[1 1 1] Initial Spawn  Phase - Actor has physics and affected by gravity till near floor
    (bind (_outhit _returnvalue_3) (`KismetSystemLibrary.LineTraceSingle` :`Start` _returnvalue :`End` (+ _returnvalue (* (0.0 0.0 -1.0) 30.0)) :`TraceChannel` "TraceTypeQuery1" :`DrawDebugType` "ForOneFrame"))
    (if _returnvalue_3
      (`PrimitiveComponent.SetEnableGravity` _sphere false)
      ;[1 1 1] Set Up for Idle phase
      (`PrimitiveComponent.SetSimulatePhysics` _sphere false)
      (set `self.initialSpawn` false)
      (set `self.relativeZTransform` (.z (.location (`SceneComponent.GetRelativeTransform` _sphere)))))
    (elif (`self.idle`)
      ;[1 1 1] Bobbing phase - When orb is idle on floor
      (`self.K2_SetActorRelativeLocation` (`KismetMathLibrary.MakeVector` (.x (.location _returnvalue_2)) (.y (.location _returnvalue_2)) (+ (`self.relativeZTransform`) (* (`KismetMathLibrary.DegSin` (* (+ (`self.GetGameTimeSinceCreation`) (`self.randomOffset`)) (`self.bobSpeed`))) (`self.bobDistance`)))))
      ;[1 1 1] Set boolean for next phase
      (set `self.idle` (>= (`KismetMathLibrary.Vector_Distance` (`self.K2_GetActorLocation`) (`self.K2_GetActorLocation` (`GameplayStatics.GetPlayerPawn` 0))) (`self.absorbRadius`)))
      (else
        ;[1 1 1] Absorb phase - attracted towards player at an offset for orbiting effect
        (bind _output_get (set `self.velocity` (* (+ (`self.velocity`) (* (/ (- (`self.K2_GetActorLocation` (`GameplayStatics.GetPlayerPawn` 0)) (`self.K2_GetActorLocation`)) 100.0) (`self.absorbSpeed`))) 0.95)))
        (`self.K2_AddActorWorldOffset` _output_get)))))

(event `self.Sphere.OnComponentBeginOverlap`
  (params (OverlappedComponent :type "PrimitiveComponent Object Reference") (OtherActor :type "Actor Object Reference") (OtherComp :type "PrimitiveComponent Object Reference") (OtherBodyIndex :type Integer) (bFromSweep :type Boolean) (SweepResult :type "HitResult Structure (by ref)"))
  ;[1 1 1] Let orbs rotate a few times before being consumed
  (if (== OtherActor (`GameplayStatics.GetPlayerPawn` 0))
    (if (<= (`KismetMathLibrary.VSize` (`self.velocity`)) 15.0)
      (message `/Game/Blueprints/BPI/Player/BPI_Player.chargeUltimate` OtherActor)
      ;[1 0 0] !! Consume and charge ultimate
      (`self.K2_DestroyActor`))))

(fn `UserConstructionScript`)