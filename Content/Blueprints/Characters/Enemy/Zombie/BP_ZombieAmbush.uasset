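; Zombie ambush volume that spawns a group of zombies when the player enters its box or TriggerAllAmbushes fires.
; Overlap starts a delayed, gated spawn that StopAmbush can cancel, then staggers zombies at random ground-traced points, facing the player with spawn decals and Niagara effects.
; Despawn removes survivors, deducts killed zombies from the next spawn count and reports whether none remain.
; Game-instance debug mode reveals the box and spawn points.
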(event `self.ReceiveBeginPlay`
  ;[0 0 0] Debug
  (bind _instanceref (message `/Game/Blueprints/BPI/GameInstance/BPI_GameInstance.GetInstanceRef` (`GameplayStatics.GetGameInstance`)))
  (add `/Game/_Manager/InGame/GI_Game.debugModeChange` _instanceref (delegate `Debug mode`)))

(event `Debug mode`
  ;[0 0 0] Debug
  (bind _debugmode (message `/Game/Blueprints/BPI/GameInstance/BPI_GameInstance.GetDebugMode` (`GameplayStatics.GetGameInstance`)))
  (`SceneComponent.SetHiddenInGame` (`self.Box`) (not _debugmode) false))

(event `TriggerAllAmbushes`
  (bind _returnvalue (* 0.4 1.0))
  (bind _newvar_location (`KismetMathLibrary.BreakTransform` (`self.NewVar`)))
  (bind (_origin _boxextent) (`KismetSystemLibrary.GetComponentBounds` (`self.Box`)))
  (bind _returnvalue_2 (`KismetMathLibrary.RandomPointInBoundingBox` _origin _boxextent))
  (bind (_returnvalue_roll _returnvalue_pitch _returnvalue_yaw) (`KismetMathLibrary.BreakRotator` (`KismetMathLibrary.FindLookAtRotation` _returnvalue_2 (`self.K2_GetActorLocation` (`GameplayStatics.GetPlayerPawn` 0)))))
  (set `self.ambushActive` false :!label _label) ; Stop ambush from activating multiple times
  (`self.ForLoopDelay` 1 (`self.zombiesToSpawn`) (`KismetMathLibrary.RandomFloatInRange` 0.1 0.2)
    (:`Loop Body`
      ;[1 1 1] Random spawn position inside collider
      (bind (_outhit _returnvalue_3) (`KismetSystemLibrary.LineTraceSingle` _returnvalue_2 (- _returnvalue_2 (0.0 0.0 5000.0)) "TraceTypeQuery1" :!label _label_2))
      (if _returnvalue_3
        (bind _output_get (set `self.NewVar` (`KismetMathLibrary.MakeTransform` (`.ImpactPoint` (`GameplayStatics.BreakHitResult` _outhit)) (`KismetMathLibrary.MakeRotator` 0.0 0.0 _returnvalue_yaw))))
        (bind _returnvalue_4 (`|SpawnActorFromClass` "/Game/Blueprints/BP_MasterDecal.BP_MasterDecal_C" _output_get "AlwaysSpawn" "MultiplyWithRoot" null null))
        (`self.SetLifeSpan` _returnvalue_4 5.0)
        (`NiagaraComponent.SetAsset` (`/Game/Blueprints/BP_MasterDecal.Niagara` _returnvalue_4) "/Game/Imports/VFX/FX_SpawnZombie/NS_SpawnZombie.NS_SpawnZombie" false)
        (bind _decal (`/Game/Blueprints/BP_MasterDecal.Decal` _returnvalue_4))
        (`DecalComponent.SetDecalMaterial` _decal "/Game/Imports/VFX/FX_SpawnZombie/MI_SpawnDecal.MI_SpawnDecal")
        (`SceneComponent.SetRelativeScale3D` _decal (`KismetMathLibrary.MakeVector` 1.0 _returnvalue _returnvalue))
        (bind _returnvalue_5 (`|SpawnActorFromClass` "/Game/Blueprints/Characters/Enemy/Zombie/BP_Zombie.BP_Zombie_C" _output_get "AdjustIfPossibleButAlwaysSpawn" "MultiplyWithRoot" null null))
        (`KismetArrayLibrary.Array_Add` (`self.spawnedZombies`) _returnvalue_5)
        ;[0 0 0] Debug
        (bind _debugmode (message `/Game/Blueprints/BPI/GameInstance/BPI_GameInstance.GetDebugMode` (`GameplayStatics.GetGameInstance`)))
        (if _debugmode
          (`KismetSystemLibrary.DrawDebugSphere` _newvar_location 10.0 12 (struct :`R` 1.0 :`A` 1.0) 10.0)
          (bind _returnvalue_location (`KismetMathLibrary.BreakTransform` (`self.GetTransform` _returnvalue_5)))
          (`KismetSystemLibrary.DrawDebugLine` _newvar_location _returnvalue_location (struct :`R` 1.0 :`A` 1.0) 10.0))
        (else
          (goto _label_2))))))

(event `self.Box.OnComponentBeginOverlap`
  (params (OverlappedComponent :type "PrimitiveComponent Object Reference") (OtherActor :type "Actor Object Reference") (OtherComp :type "PrimitiveComponent Object Reference") (OtherBodyIndex :type Integer) (bFromSweep :type Boolean) (SweepResult :type "HitResult Structure (by ref)"))
  (if (and (== OtherActor (`GameplayStatics.GetPlayerPawn` 0)) (`self.ambushActive`))
    (`|ExecutionSequence`
      (:`then_0`
        (`KismetSystemLibrary.Delay` (`self.ambushDelay`))
        (`KismetSystemLibrary.DelayUntilNextTick`)
        (`/Engine/EditorBlueprintResources/StandardMacros.Gate` true :!label _label_3
          (:`Exit`
            (goto _label))))
      (:`then_1`
        (goto _label_3 :!via `Open`)))))

(event `StopAmbush`
  (goto _label_3 :!via `Close`))

(fn `Despawn`
  (returns (Destroy :type Boolean))
  (locals (NewLocalVar :type "Array of /Game/Blueprints/Characters/Enemy/Zombie/BP_Zombie Object Reference"))
  (bind _returnvalue (== 0 (`self.zombiesToSpawn`)))
  (for _array_element (`self.spawnedZombies`)
    ;[1 1 1] Decrease zombies to spawn in next ambush if killed
    (`/Engine/EditorBlueprintResources/StandardMacros.IsValid` _array_element
      (:`Is Valid`
        (`self.K2_DestroyActor` _array_element))
      (:`Is Not Valid`
        (`/Engine/EditorBlueprintResources/StandardMacros.DecrementInt` (`self.zombiesToSpawn`)))))
  ;[1 1 1] If all zombies were killed, destroy ambush
  (`KismetArrayLibrary.Array_Clear` (`self.spawnedZombies`))
  (if _returnvalue
    _
    (else
      _))
  (return _returnvalue))

(fn `UserConstructionScript`
  (bind (_ambushsize_x _ambushsize_y) (`KismetMathLibrary.BreakVector2D` (`self.ambushSize`)))
  (`self.SetActorScale3D` (1.0 1.0 1.0))
  (`BoxComponent.SetBoxExtent` (`self.Box`) (`KismetMathLibrary.MakeVector` _ambushsize_x _ambushsize_y 50.0) true))