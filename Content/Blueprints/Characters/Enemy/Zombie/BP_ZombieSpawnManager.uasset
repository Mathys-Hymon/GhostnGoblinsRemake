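; Zombie spawn manager that switches its linked spawners and ambushes on and off as the player moves through an area.
; Entering the inner spawn box activates both, optionally triggering ambushes immediately.
; Leaving the outer despawn box deactivates and despawns them, removes finished ambushes and resets the zombie attack state.
; The construction script keeps the despawn box at least spawn-box size; debug mode shows both volumes and prints state.
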(event `self.ReceiveBeginPlay`
  ;[0 0 0] Debug
  (bind _instanceref (message `/Game/Blueprints/BPI/GameInstance/BPI_GameInstance.GetInstanceRef` (`GameplayStatics.GetGameInstance`)))
  (add `/Game/_Manager/InGame/GI_Game.debugModeChange` _instanceref (delegate `Debug mode`)))

(event `Debug mode`
  ;[0 0 0] Debug
  (bind _debugmode (message `/Game/Blueprints/BPI/GameInstance/BPI_GameInstance.GetDebugMode` (`GameplayStatics.GetGameInstance`)))
  (bind _returnvalue (not _debugmode))
  (`SceneComponent.SetHiddenInGame` (`self.Despawn Collider`) _returnvalue false)
  (`SceneComponent.SetHiddenInGame` (`self.Spawn Collider`) _returnvalue false))

(event `self.Spawn Collider.OnComponentBeginOverlap`
  (params (OverlappedComponent :type "PrimitiveComponent Object Reference") (OtherActor :type "Actor Object Reference") (OtherComp :type "PrimitiveComponent Object Reference") (OtherBodyIndex :type Integer) (bFromSweep :type Boolean) (SweepResult :type "HitResult Structure (by ref)"))
  ;[1 1 1] Set Spawners Active
  (if (and (== OtherActor (`GameplayStatics.GetPlayerPawn` 0)) (!= (`self.Active`) true))
    (set `self.Active` true)
    (`|ExecutionSequence`
      (:`then_0`
        (for _array_element (`self.spawns`)
          (`/Game/Blueprints/Characters/Enemy/Zombie/BP_ZombieSpawn.ActivateSpawner` _array_element (`self.Active`)))
        ;[0 0 0] Debug
        (bind _debugmode (message `/Game/Blueprints/BPI/GameInstance/BPI_GameInstance.GetDebugMode` (`GameplayStatics.GetGameInstance`)))
        (`KismetSystemLibrary.PrintString` "Spawns Active" _debugmode _debugmode (struct :`G` 0.66 :`B` 1.0 :`A` 1.0) 1.0))
      (:`then_1`
        (for _array_element_2 (`self.Ambushes`)
          (set `/Game/Blueprints/Characters/Enemy/Zombie/BP_ZombieAmbush.ambushActive` (`self.Active`) _array_element_2)
          (if (`self.TriggerAmbushes on enter`)
            (`/Game/Blueprints/Characters/Enemy/Zombie/BP_ZombieAmbush.TriggerAllAmbushes` _array_element_2)))
        ;[0 0 0] Debug
        (bind _debugmode_2 (message `/Game/Blueprints/BPI/GameInstance/BPI_GameInstance.GetDebugMode` (`GameplayStatics.GetGameInstance`)))
        (`KismetSystemLibrary.PrintString` "Ambushes Active" _debugmode_2 _debugmode_2 (struct :`G` 0.66 :`B` 1.0 :`A` 1.0) 1.0)))))

(event `self.Despawn Collider.OnComponentEndOverlap`
  (params (OverlappedComponent :type "PrimitiveComponent Object Reference") (OtherActor :type "Actor Object Reference") (OtherComp :type "PrimitiveComponent Object Reference") (OtherBodyIndex :type Integer))
  ;[1 1 1] Deactivate Spawners
  (if (== OtherActor (`GameplayStatics.GetPlayerPawn` 0))
    (set `self.Active` false)
    (`|ExecutionSequence`
      (:`then_0`
        (for _array_element (`self.spawns`)
          (`/Game/Blueprints/Characters/Enemy/Zombie/BP_ZombieSpawn.ActivateSpawner` _array_element (`self.Active`))
          (`/Game/Blueprints/Characters/Enemy/Zombie/BP_ZombieSpawn.Despawn` _array_element))
        ;[0 0 0] Debug
        (bind _debugmode (message `/Game/Blueprints/BPI/GameInstance/BPI_GameInstance.GetDebugMode` (`GameplayStatics.GetGameInstance`)))
        (`KismetSystemLibrary.PrintString` "Spawns Inactive" _debugmode _debugmode (struct :`G` 0.66 :`B` 1.0 :`A` 1.0) 1.0))
      (:`then_1`
        (for _array_element_2 (`self.Ambushes`)
          (`/Engine/EditorBlueprintResources/StandardMacros.IsValid` _array_element_2
            (:`Is Valid`
              (`/Game/Blueprints/Characters/Enemy/Zombie/BP_ZombieAmbush.StopAmbush` _array_element_2)
              (set `/Game/Blueprints/Characters/Enemy/Zombie/BP_ZombieAmbush.ambushActive` (`self.Active`) _array_element_2)
              (bind _destroy (`/Game/Blueprints/Characters/Enemy/Zombie/BP_ZombieAmbush.Despawn` _array_element_2))
              (if _destroy
                (`self.K2_DestroyActor` _array_element_2)
                (`KismetArrayLibrary.Array_RemoveItem` (`self.Ambushes`) _array_element_2)))))
        (message `/Game/Blueprints/BPI/GameInstance/BPI_GameInstance.ResetZombieAttackingPlayer` (`GameplayStatics.GetGameInstance`))
        ;[0 0 0] Debug
        (bind _debugmode_2 (message `/Game/Blueprints/BPI/GameInstance/BPI_GameInstance.GetDebugMode` (`GameplayStatics.GetGameInstance`)))
        (`KismetSystemLibrary.PrintString` "Ambushes Inactive" _debugmode_2 _debugmode_2 (struct :`G` 0.66 :`B` 1.0 :`A` 1.0) 1.0)))))

(fn `UserConstructionScript`
  (bind (_spawnsize_x _spawnsize_y _spawnsize_z) (`KismetMathLibrary.BreakVector` (`self.spawnSize`)))
  (bind (_despawnsize_x _despawnsize_y _despawnsize_z) (`KismetMathLibrary.BreakVector` (`self.despawnSize`)))
  (bind (_spawnsize_x_2 _spawnsize_y_2 _spawnsize_z_2) (`KismetMathLibrary.BreakVector` (`self.spawnSize`)))
  (bind (_despawnsize_x_2 _despawnsize_y_2 _despawnsize_z_2) (`KismetMathLibrary.BreakVector` (`self.despawnSize`)))
  (`SceneComponent.K2_SetRelativeLocation` (`self.Spawn Collider`) (`KismetMathLibrary.MakeVector` 0.0 0.0 _spawnsize_z_2) false true)
  (`SceneComponent.K2_SetRelativeLocation` (`self.Despawn Collider`) (`KismetMathLibrary.MakeVector` 0.0 0.0 (`KismetMathLibrary.FClamp` _despawnsize_z_2 _spawnsize_z_2 1000000000000.0)) false true)
  (`self.SetActorScale3D` (1.0 1.0 1.0))
  (set `self.despawnSize` (`KismetMathLibrary.MakeVector` (`KismetMathLibrary.FClamp` _despawnsize_x _spawnsize_x 1000000000000.0) (`KismetMathLibrary.FClamp` _despawnsize_y _spawnsize_y 1000000000000.0) (`KismetMathLibrary.FClamp` _despawnsize_z _spawnsize_z 1000000000000.0)))
  (`BoxComponent.SetBoxExtent` (`self.Spawn Collider`) (`self.spawnSize`) true)
  (`BoxComponent.SetBoxExtent` (`self.Despawn Collider`) (`self.despawnSize`) true))