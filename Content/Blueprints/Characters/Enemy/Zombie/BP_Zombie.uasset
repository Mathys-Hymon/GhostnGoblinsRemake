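; Zombie enemy character that takes its stats, score and animations from a data asset and randomizes its dissolve material and scale on spawn.
; Tick crossfades idle and run sounds by velocity, while non-lethal damage plays gated hit reactions.
; Death runs once, driving a material dissolve, awarding score with floating text, dropping souls (halved for ultimate kills), and notifying its door and AI controller.
; It also destroys attached actors, then itself after the death montage.
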(event `/Game/Blueprints/BPI/Enemies/BPI_Zombie.SetDebugState`
  (params (state :type Integer))
  ;[1 0 0] Debug
  (`TextRenderComponent.K2_SetText` (`self.AttackState_Text`) (`|FormatText` "State : {value}" (select `int` state :`0` "running" :`1` "waiting" :`2` "attacking" :!type "Text"))))

(event `self.ReceiveBeginPlay`
  (bind _returnvalue (`self.K2_GetActorLocation`))
  (bind _charactermovement (`self.CharacterMovement`))
  (bind _sfxdataasset (`self.sfxDataAsset`))
  (bind _dataasset (`self.dataAsset`))
  (`parent.ReceiveBeginPlay`)
  (`GameplayStatics.PlaySoundAtLocation` (`KismetArrayLibrary.Array_Random` (`/Game/_Manager/InGame/DataAsset/BP/SFX/BP_SFX_DA.spawnZombieVoice` _sfxdataasset)) _returnvalue (struct) 1.0 1.0 0.0 "/Game/Imports/SFX/SoundAttenuation.SoundAttenuation" null null null)
  (`GameplayStatics.PlaySoundAtLocation` (`KismetArrayLibrary.Array_Random` (`/Game/_Manager/InGame/DataAsset/BP/SFX/BP_SFX_DA.spawnZombieFX` _sfxdataasset)) _returnvalue (struct) 1.0 1.0 0.0 "/Game/Imports/SFX/SoundAttenuation.SoundAttenuation" null null null)
  (`PrimitiveComponent.SetMaterial` (`self.Mesh`) 0 (`KismetArrayLibrary.Array_Random` (`|MakeArray` "/Game/Imports/VFX/FX_Dissolve/MI_DissolveZombie1.MI_DissolveZombie1" "/Game/Imports/VFX/FX_Dissolve/MI_DissolveZombie2.MI_DissolveZombie2" "/Game/Imports/VFX/FX_Dissolve/MI_DissolveZombie3.MI_DissolveZombie3" "/Game/Imports/VFX/FX_Dissolve/MI_DissolveZombie4.MI_DissolveZombie4" :!type "MaterialInterface Object Reference")))
  (`SceneComponent.SetRelativeScale3D` (`self.Mesh`) (`KismetMathLibrary.Conv_DoubleToVector` (`KismetMathLibrary.RandomFloatInRange` 0.9 1.1)))
  ;[1 1 1] Data Asset
  (set `self.health` (`/Game/_Manager/InGame/DataAsset/BP/BP_ZombieDA.health` (`self.dataAsset`)))
  (set `CharacterMovementComponent.MaxWalkSpeed` (`/Game/_Manager/InGame/DataAsset/BP/BP_ZombieDA.movementSpeed` _dataasset) _charactermovement)
  (set `CharacterMovementComponent.MaxAcceleration` (`/Game/_Manager/InGame/DataAsset/BP/BP_ZombieDA.acceleration` _dataasset) _charactermovement)
  (set `CharacterMovementComponent.GravityScale` (`/Game/_Manager/InGame/DataAsset/BP/BP_ZombieDA.gravityScale` _dataasset) _charactermovement)
  (`self.SetDebugState` 0)
  (`TextRenderComponent.K2_SetText` (`self.EnemyScore`) (`self.BaseText`))
  (`KismetSystemLibrary.Delay` 0.3)
  (bind _returnvalue_2 (`GameplayStatics.SpawnSoundAttached` (`KismetArrayLibrary.Array_Random` (`/Game/_Manager/InGame/DataAsset/BP/SFX/BP_SFX_DA.idleZombie` (`self.sfxDataAsset`))) (`self.CapsuleComponent`) "None" (0.0 0.0 0.0) (struct) "KeepRelativeOffset" false 1.0 1.0 0.0 "/Game/Imports/SFX/SoundAttenuation.SoundAttenuation" null))
  (set `self.zombieNoise` _returnvalue_2))

(event `self.debugMode`
  (`parent.debugMode`)
  (bind _debugmode (message `/Game/Blueprints/BPI/GameInstance/BPI_GameInstance.GetDebugMode` (`GameplayStatics.GetGameInstance`)))
  (`SceneComponent.SetHiddenInGame` (`self.AttackState_Text`) (not _debugmode) false))

(event `self.ReceiveTick`
  (params (DeltaSeconds :type "Float (single-precision)"))
  (bind _zombienoise (`self.zombieNoise`))
  (bind _capsulecomponent (`self.CapsuleComponent`))
  (if (> (`KismetMathLibrary.VSize` (`self.GetVelocity`)) 0.1)
    (`|ExecutionSequence`
      (:`then_0`
        (`/Engine/EditorBlueprintResources/StandardMacros.DoOnce` false :!label _label
          (:`Completed`
            (bind _returnvalue (`GameplayStatics.SpawnSoundAttached` (`KismetArrayLibrary.Array_Random` (`/Game/_Manager/InGame/DataAsset/BP/SFX/BP_SFX_DA.runZombie` (`self.sfxDataAsset`))) _capsulecomponent "None" (0.0 0.0 0.0) (struct) "KeepRelativeOffset" false 1.0 1.0 0.0 "/Game/Imports/SFX/SoundAttenuation.SoundAttenuation" null))
            (`/Engine/EditorBlueprintResources/StandardMacros.IsValid` (stale _returnvalue_2)
              (:`Is Valid`
                (`AudioComponent.FadeOut` (stale _returnvalue_2) 0.3 0.0 "Linear"))
              (:`Is Not Valid`
                _)))))
      (:`then_1`
        (goto _label_2 :!via `Reset`)))
    (else
      (`|ExecutionSequence`
        (:`then_0`
          (goto _label :!via `Reset`))
        (:`then_1`
          (`/Engine/EditorBlueprintResources/StandardMacros.DoOnce` false :!label _label_2
            (:`Completed`
              (bind _returnvalue_2 (`GameplayStatics.SpawnSoundAttached` (`KismetArrayLibrary.Array_Random` (`/Game/_Manager/InGame/DataAsset/BP/SFX/BP_SFX_DA.idleZombie` (`self.sfxDataAsset`))) _capsulecomponent "None" (0.0 0.0 0.0) (struct) "KeepRelativeOffset" false 1.0 1.0 0.0 "/Game/Imports/SFX/SoundAttenuation.SoundAttenuation" null))
              (`/Engine/EditorBlueprintResources/StandardMacros.IsValid` _returnvalue
                (:`Is Valid`
                  (`AudioComponent.FadeOut` _returnvalue 0.3 0.0 "Linear"))
                (:`Is Not Valid`
                  _))))))))
  (`/Engine/EditorBlueprintResources/StandardMacros.IsValid` _zombienoise
    (:`Is Valid`
      (`AudioComponent.FadeOut` _zombienoise 0.3 0.0 "Linear"))))

(event `/Game/Blueprints/BPI/Enemies/BPI_Enemy.setDoorRef`
  (params (doorRef :type "/Game/Blueprints/GPE/BP_SkullDoor Object Reference"))
  (set `self.doorRef` doorRef))

(event `self.ReceiveAnyDamage`
  (params (Damage :type "Float (single-precision)") (DamageType :type "DamageType Object Reference") (InstigatedBy :type "Controller Object Reference") (DamageCauser :type "Actor Object Reference"))
  (bind _out_actors (`self.Out Actors`))
  (bind _zombienoise (`self.zombieNoise`))
  (bind _doorref (`self.doorRef`))
  (bind _soulsdropped (`/Game/_Manager/InGame/DataAsset/BP/BP_ZombieDA.soulsDropped` (`self.dataAsset`)))
  ;[1 1 1] Take Damage
  (bind _output_get (set `self.health` (- (`self.health`) Damage)))
  (if (<= _output_get 0.0)
    (`/Engine/EditorBlueprintResources/StandardMacros.DoOnce` false
      (:`Completed`
        (`|ExecutionSequence`
          (:`then_0`
            (`PrimitiveComponent.SetCollisionEnabled` (`self.CapsuleComponent`) "NoCollision")
            (message `/Game/Blueprints/BPI/GameInstance/BPI_GameInstance.GainScore` (`GameplayStatics.GetGameInstance`) (`/Game/_Manager/InGame/DataAsset/BP/BP_ZombieDA.score` (`self.dataAsset`))))
          (:`then_1`
            (bind (_direction _appear) (`Timeline|Timeline` :!via `PlayFromStart`)
              (:`Update`
                (`MeshComponent.SetScalarParameterValueOnMaterials` (`self.Mesh`) "Alpha" _appear))))
          (:`then_2`
            (`|SpawnActorFromClass` "/Game/Imports/VFX/FX_Ultimate_Charge/BP_DropFx.BP_DropFx_C" (`KismetMathLibrary.MakeTransform` (`self.K2_GetActorLocation`)) "AlwaysSpawn" "MultiplyWithRoot" null (`KismetMathLibrary.SelectInt` _soulsdropped (/ _soulsdropped 2) (!= DamageType "/Game/Blueprints/Characters/Player/BP_UltDamageType.BP_UltDamageType")) null)
            (`/Engine/EditorBlueprintResources/StandardMacros.IsValid` _doorref
              (:`Is Valid`
                (`/Game/Blueprints/GPE/BP_SkullDoor.EnemyDied` _doorref))
              (:`Is Not Valid`
                _))
            (set `self.Out Actors` (`self.GetAttachedActors` false true))
            (message `/Game/Blueprints/BPI/Enemies/BPI_Zombie.ClearPlayerRefInBB` (`AIBlueprintHelperLibrary.GetAIController` self))
            (bind _isattacking (message `/Game/Blueprints/BPI/Enemies/BPI_Zombie.GetIsAttackingPlayer` (`AIBlueprintHelperLibrary.GetAIController` self)))
            (if _isattacking
              (message `/Game/Blueprints/BPI/GameInstance/BPI_GameInstance.UpdateZombiesAttackingPlayer` (`GameplayStatics.GetGameInstance`) -1))
            (for _array_element _out_actors
              (`/Engine/EditorBlueprintResources/StandardMacros.IsValid` _array_element
                (:`Is Valid`
                  (`self.K2_DestroyActor` _array_element))))
            (`KismetArrayLibrary.Array_Clear` _out_actors)
            (`self.DisplayScore`)
            (`|PlayMontage` (`self.Mesh`) (`KismetArrayLibrary.Array_Random` (`/Game/_Manager/InGame/DataAsset/BP/BP_ZombieDA.deadAnim` (`self.dataAsset`)))
              (:`OnCompleted`
                (`self.K2_DestroyActor`)
                (`GameplayStatics.SpawnSoundAttached` (`KismetArrayLibrary.Array_Random` (`/Game/_Manager/InGame/DataAsset/BP/SFX/BP_SFX_DA.deathZombie` (`self.sfxDataAsset`))) (`self.CapsuleComponent`) "None" (0.0 0.0 0.0) (struct) "KeepRelativeOffset" false 1.0 1.0 0.0 "/Game/Imports/SFX/SoundAttenuation.SoundAttenuation" null)
                (`/Engine/EditorBlueprintResources/StandardMacros.IsValid` _zombienoise
                  (:`Is Valid`
                    (`AudioComponent.FadeOut` _zombienoise 0.3 0.0 "Linear")))))))))
    (else
      (`/Engine/EditorBlueprintResources/StandardMacros.DoOnce` false :!label _label_3
        (:`Completed`
          (`|PlayMontage` (`self.Mesh`) (`KismetArrayLibrary.Array_Random` (`/Game/_Manager/InGame/DataAsset/BP/BP_ZombieDA.hitAnim` (`self.dataAsset`)))
            (:`then`
              (`GameplayStatics.PlaySoundAtLocation` (`KismetArrayLibrary.Array_Random` (`/Game/_Manager/InGame/DataAsset/BP/SFX/BP_SFX_DA.hitZombie` (`self.sfxDataAsset`))) (`self.K2_GetActorLocation`) (struct) 1.0 1.0 0.0 "/Game/Imports/SFX/SoundAttenuation.SoundAttenuation" null null null))
            (:`OnCompleted`
              (`self.CanPlayHitAnimAgain`))))))))

(event `CanPlayHitAnimAgain`
  ;[1 1 1] Take Damage
  (goto _label_3 :!via `Reset`))

(event `DisplayScore`
  (bind _enemyscore (`self.EnemyScore`))
  (bind (_relativelocation_x _relativelocation_y _relativelocation_z) (`KismetMathLibrary.BreakVector` (`SceneComponent.RelativeLocation` _enemyscore)))
  ;[1 1 1] Take Damage
  (`TextRenderComponent.K2_SetText` _enemyscore (`KismetTextLibrary.Conv_IntToText` (`/Game/_Manager/InGame/DataAsset/BP/BP_ZombieDA.score` (`self.dataAsset`))))
  (`KismetSystemLibrary.MoveComponentTo` _enemyscore (`KismetMathLibrary.MakeVector` _relativelocation_x _relativelocation_y (+ _relativelocation_z (`self.FinalScoreHeight`))) (`SceneComponent.RelativeRotation` _enemyscore) true false (`self.OverTimeScore`)))

(event `/Game/Blueprints/BPI/Enemies/BPI_Zombie.AttackAnim`
  ;[1 1 1] Take Damage
  (`|PlayMontage` (`self.Mesh`) (`KismetArrayLibrary.Array_Random` (`/Game/_Manager/InGame/DataAsset/BP/BP_ZombieDA.attackAnim` (`self.dataAsset`)))
    (:`then`
      (`GameplayStatics.PlaySoundAtLocation` (`KismetArrayLibrary.Array_Random` (`/Game/_Manager/InGame/DataAsset/BP/SFX/BP_SFX_DA.attackZombie` (`self.sfxDataAsset`))) (`self.K2_GetActorLocation`) (struct) 1.0 1.0 0.0 "/Game/Imports/SFX/SoundAttenuation.SoundAttenuation" null null null))))

(fn `CheckForPlayer`
  (returns (isTouchingPlayer :type Boolean))
  (bind _returnvalue (`self.K2_GetActorLocation`))
  (bind (_outhit _returnvalue_2) (`KismetSystemLibrary.SphereTraceSingleByProfile` _returnvalue (+ _returnvalue (* (`KismetMathLibrary.GetDirectionUnitVector` _returnvalue (`self.K2_GetActorLocation` (`GameplayStatics.GetPlayerPawn` 0))) 100.0)) 40.0 "None" false (`|MakeArray` (`GameplayStatics.GetPlayerCharacter` 0) :!type "Actor Object Reference") "None" true (struct :`R` 1.0 :`A` 1.0) (struct :`G` 1.0 :`A` 1.0) 1.0))
  (return (not _returnvalue_2)))

(fn `GetHealth`
  (returns (health :type "Float (double-precision)") (isDead :type Boolean))
  (bind _health (`self.health`))
  (return _health (<= _health 0.0)))

(fn `getHeight`
  (returns (height :type "Float (double-precision)"))
  (return (/ (`CapsuleComponent.CapsuleHalfHeight` (`self.CapsuleComponent`)) 2.0)))

(fn `GetIsAttackingPlayer`
  (returns (isAttacking :type Boolean))
  (return false))

(fn `UserConstructionScript`
  (`parent.UserConstructionScript`))