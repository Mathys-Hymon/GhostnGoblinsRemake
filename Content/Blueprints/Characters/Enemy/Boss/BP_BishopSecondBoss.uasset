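; Second Bishop boss, which periodically splits into itself and two BP_BishopClone decoys around the arena center.
; After a charge, it hides, picks a random yaw and places itself and both clones 120 degrees apart, then reveals all three after a delay.
; Tick mirrors its attack, dash and look state onto living clones.
; Once both are gone, a cooldown re-arms spawning through two resettable DoOnce gates.
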(event `UpdateClone`
  (params (Clone :type "/Game/Blueprints/Characters/Enemy/Boss/BP_BishopClone Object Reference"))
  (set `/Game/Blueprints/Characters/Enemy/Boss/BP_BishopClone.canAttack` (`self.canAttack`) Clone)
  (set `/Game/Blueprints/Characters/Enemy/Boss/BP_BishopClone.dashing` (`self.dashing`) Clone)
  (set `/Game/Blueprints/Characters/Enemy/Boss/BP_BishopClone.stopLookPlayer` (`self.stopLookPlayer`) Clone)
  (set `/Game/Blueprints/Characters/Enemy/Boss/BP_BishopClone.attacker` (`self.attacker`) Clone))

(event `self.ReceiveTick`
  (params (DeltaSeconds :type "Float (single-precision)"))
  (bind _firstclone (`self.firstClone`))
  (bind _secondclone (`self.SecondClone`))
  (`parent.ReceiveTick` DeltaSeconds)
  (if (`self.canSpawnClone`)
    (set `self.canAttack` false)
    (set `self.stopLookPlayer` true)
    (`SceneComponent.SetHiddenInGame` (`self.Sphere`) false false)
    (`KismetSystemLibrary.Delay` (`self.chargingTime`))
    (set `self.canSpawnClone` false)
    (`/Engine/EditorBlueprintResources/StandardMacros.DoOnce` false :!label _label
      (:`Completed`
        (`self.SpawnClone`)))
    (elif (or (`KismetSystemLibrary.IsValid` (`self.firstClone`)) (`KismetSystemLibrary.IsValid` (`self.SecondClone`)))
      (`/Engine/EditorBlueprintResources/StandardMacros.IsValid` _firstclone
        (:`Is Valid`
          (`self.UpdateClone` _firstclone))
        (:`Is Not Valid`
          _))
      (`/Engine/EditorBlueprintResources/StandardMacros.IsValid` _secondclone
        (:`Is Valid`
          (`self.UpdateClone` _secondclone)))
      (else
        ;[1 1 1] New clones spawning loop
        (`/Engine/EditorBlueprintResources/StandardMacros.DoOnce` false :!label _label_2
          (:`Completed`
            (`KismetSystemLibrary.Delay` (`self.cloneCooldown`))
            (set `self.canSpawnClone` true)
            (`self.CanCloneAgain`)))))))

(event `CanCloneAgain`
  (goto _label :!via `Reset`))

(event `ResetDoOnceCooldown`
  ;[1 1 1] New clones spawning loop
  (goto _label_2 :!via `Reset`))

(event `SpawnClone`
  (bind (_returnvalue_x _returnvalue_y _returnvalue_z) (`KismetMathLibrary.BreakVector` (`self.K2_GetActorLocation`)))
  (bind (_returnvalue_roll _returnvalue_pitch) (`KismetMathLibrary.BreakRotator` (`self.K2_GetActorRotation`)))
  (bind (_returnvalue_roll_2 _returnvalue_pitch_2 _returnvalue_yaw) (`KismetMathLibrary.BreakRotator` (`self.K2_GetActorRotation`)))
  (bind (_returnvalue_roll_3 _returnvalue_pitch_3 _returnvalue_yaw_2) (`KismetMathLibrary.BreakRotator` (`self.K2_GetActorRotation`)))
  (bind (_returnvalue_x_2 _returnvalue_y_2) (`KismetMathLibrary.BreakVector` (`self.K2_GetActorLocation` (`self.centerOfArena`))))
  ;[0.3594 0.03917 0] Random teleport and spawn clones
  (`SceneComponent.SetHiddenInGame` (`self.Mesh`) true true)
  (`self.K2_SetActorLocation` (`KismetMathLibrary.MakeVector` _returnvalue_x_2 _returnvalue_y_2 _returnvalue_z) false true)
  (`self.K2_SetActorRotation` (`KismetMathLibrary.MakeRotator` _returnvalue_roll _returnvalue_pitch (`KismetMathLibrary.RandomFloatInRange` 0.0 360.0)) true)
  ;;[1 1 1] Spawn clones
  (bind _clone (`self.SpawnCloneFonction` (`KismetMathLibrary.MakeRotator` _returnvalue_roll_2 _returnvalue_pitch_2 (+ _returnvalue_yaw 120.0))))
  (set `self.firstClone` _clone)
  (bind _clone_2 (`self.SpawnCloneFonction` (`KismetMathLibrary.MakeRotator` _returnvalue_roll_3 _returnvalue_pitch_3 (+ _returnvalue_yaw_2 240.0))))
  (set `self.SecondClone` _clone_2)
  (`self.K2_SetActorLocation` (+ (`self.K2_GetActorLocation`) (* (`self.GetActorForwardVector`) (`self.rangeFromCenter`))) false true)
  (`self.LookCenter`)
  ;;[1 1 1] Boss and clones reapear
  (`KismetSystemLibrary.Delay` (`self.dissapearTime`))
  (`SceneComponent.SetHiddenInGame` (`self.Mesh`) false true)
  (`/Engine/EditorBlueprintResources/StandardMacros.IsValid` (`self.firstClone`)
    (:`Is Valid`
      (`SceneComponent.SetHiddenInGame` (`Character.Mesh` (`self.firstClone`)) false true))
    (:`Is Not Valid`
      _))
  (`/Engine/EditorBlueprintResources/StandardMacros.IsValid` (`self.SecondClone`)
    (:`Is Valid`
      (`SceneComponent.SetHiddenInGame` (`Character.Mesh` (`self.SecondClone`)) false true))
    (:`Is Not Valid`
      _))
  (set `self.canAttack` true)
  (`self.ResetDoOnceCooldown`))

(event `self.ReceiveAnyDamage`
  (params (Damage :type "Float (single-precision)") (DamageType :type "DamageType Object Reference") (InstigatedBy :type "Controller Object Reference") (DamageCauser :type "Actor Object Reference"))
  ;[1 1 1] Kill clone when hit
)

(fn `SpawnCloneFonction`
  (params (`Spawn Transform Rotation` :type "Rotator Structure"))
  (returns (clone :type "/Game/Blueprints/Characters/Enemy/Boss/BP_BishopClone Object Reference"))
  (bind (_returnvalue_x _returnvalue_y _returnvalue_z) (`KismetMathLibrary.BreakVector` (`self.K2_GetActorLocation`)))
  (bind (_returnvalue_x_2 _returnvalue_y_2) (`KismetMathLibrary.BreakVector` (`self.K2_GetActorLocation` (`self.centerOfArena`))))
  (bind _returnvalue (`|SpawnActorFromClass` "/Game/Blueprints/Characters/Enemy/Boss/BP_BishopClone.BP_BishopClone_C" (`KismetMathLibrary.MakeTransform` (`KismetMathLibrary.MakeVector` _returnvalue_x_2 _returnvalue_y_2 _returnvalue_z) `Spawn Transform Rotation`) "AlwaysSpawn" "MultiplyWithRoot" null null)) ; Spawn First clone
  (`self.K2_SetActorLocation` _returnvalue (+ (`self.K2_GetActorLocation` _returnvalue) (* (`self.GetActorForwardVector` _returnvalue) (`self.rangeFromCenter`))) false false)
  (set `/Game/Blueprints/Characters/Enemy/Boss/BP_BishopClone.encircleDirection` (`self.encircleDirection`) _returnvalue)
  (`SceneComponent.SetHiddenInGame` (`Character.Mesh` _returnvalue) true true)
  (set `/Game/Blueprints/Characters/Enemy/Boss/BP_BishopClone.centerOfArena` (`self.centerOfArena`) _returnvalue)
  (set `/Game/Blueprints/Characters/Enemy/Boss/BP_BishopClone.rangeFromCenter` (`self.rangeFromCenter`) _returnvalue)
  (return _returnvalue))

(fn `UserConstructionScript`
  (`parent.UserConstructionScript`))