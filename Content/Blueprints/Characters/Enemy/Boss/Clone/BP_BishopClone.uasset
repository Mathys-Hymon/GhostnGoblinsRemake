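; Bishop boss clone enemy that faces the player or arena center and fires cone or spray attacks through BPCBossAttacks.
; In routine mode it spawns a center position reference once; otherwise it circles the arena and self-destructs after a data-asset-based delay.
; It dies when damage depletes its HP.
; When the main boss is hit, it drops capsule collision, stops attacking and interpolates into the boss before destroying itself.
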(event `self.ReceiveTick`
  (params (DeltaSeconds :type "Float (single-precision)"))
  ;[0 0.2759 0.3958] Init clone
  (if (`KismetSystemLibrary.IsValid` (`self.centerOfArena`))
    (if (`self.cloneRoutine?`)
      (`self.CloneRoutine`)
      (else
        (`self.LookTheCenter`)
        (`self.AddMovementInput` (* (`self.GetActorRightVector`) (`self.encircleDirection`)) 1000.0)
        (`/Engine/EditorBlueprintResources/StandardMacros.DoOnce` false
          (:`Completed`
            (`KismetSystemLibrary.Delay` (+ (`/Game/_Manager/InGame/DataAsset/BP/Boss/BP_Bishop2DA.cloneAttackChargeTime` (`self.dataAsset`)) 2.0))
            (`self.K2_DestroyActor`)))))))

(event `ActualiseAttack`
  ;[0 0.2759 0.3958] Init clone
  (`/Game/Blueprints/Characters/Enemy/Boss/BPC_BossAttacks.StopAttack` (`self.BPC_BossAttacks`) :!label _label))

(event `self.ReceiveBeginPlay`
  ;[0 0.2759 0.3958] Init clone
  (set `self.cloneHP` (`/Game/_Manager/InGame/DataAsset/BP/Boss/BP_Bishop2DA.cloneHP` (`self.dataAsset`)))
  (goto _label))

(event `LookThePlayer`
  (bind (_returnvalue_roll _returnvalue_pitch _returnvalue_yaw) (`KismetMathLibrary.BreakRotator` (`KismetMathLibrary.FindLookAtRotation` (`self.K2_GetActorLocation`) (`self.K2_GetActorLocation` (`GameplayStatics.GetPlayerPawn` 0)))))
  ;[1 1 1] Clone look to...
  (`self.K2_SetActorRotation` (`KismetMathLibrary.RInterpTo` (`self.K2_GetActorRotation`) (`KismetMathLibrary.MakeRotator` 0.0 0.0 _returnvalue_yaw) (`GameplayStatics.GetWorldDeltaSeconds`) 10.0)))

(event `LookTheCenter`
  (bind (_returnvalue_roll _returnvalue_pitch _returnvalue_yaw) (`KismetMathLibrary.BreakRotator` (`KismetMathLibrary.FindLookAtRotation` (`self.K2_GetActorLocation`) (`self.K2_GetActorLocation` (`self.centerOfArena`)))))
  ;[1 1 1] Clone look to...
  (`self.K2_SetActorRotation` (`KismetMathLibrary.RInterpTo` (`self.K2_GetActorRotation`) (`KismetMathLibrary.MakeRotator` 0.0 0.0 _returnvalue_yaw) (`GameplayStatics.GetWorldDeltaSeconds`) 10.0)))

(event `CloneRoutine`
  ;[1 1 1] Routine
  (`self.StartClone`)
  (if (`self.goBoss`)
    (`self.GoToBoss`))
  (if (`self.LookCenter?`)
    (`self.LookTheCenter`)
    (elif (not (`self.stopLookPlayer`))
      (`self.LookThePlayer`))))

(event `StartClone`
  ;[1 1 1] Start clone and spawn reference pos
  (`/Engine/EditorBlueprintResources/StandardMacros.DoOnce` false
    (:`Completed`
      (bind _returnvalue (`|SpawnActorFromClass` "/Game/Blueprints/Characters/Enemy/Boss/Clone/BP_ClonePosRef.BP_ClonePosRef_C" (`self.GetTransform` (`self.centerOfArena`)) "AlwaysSpawn" "MultiplyWithRoot" null null))
      (set `self.centerPosRef` _returnvalue))))

(event `self.ReceiveAnyDamage`
  (params (Damage :type "Float (single-precision)") (DamageType :type "DamageType Object Reference") (InstigatedBy :type "Controller Object Reference") (DamageCauser :type "Actor Object Reference"))
  ;[0 0 0] Death
  (if (not (and (`SceneComponent.bHiddenInGame` (`self.Sphere`)) (`self.cloneRoutine?`)))
    (bind _output_get (set `self.cloneHP` (- (`self.cloneHP`) Damage)))
    (if (<= _output_get 0.0)
      (`KismetSystemLibrary.DelayUntilNextTick`)
      (`self.K2_DestroyActor`))))

(event `BossHit`
  (params (mainBoss :type "/Game/Blueprints/Characters/Enemy/Boss/BP_BishopUniqueBoss Object Reference"))
  ;[0 0 0] Player hit main boss
  (`PrimitiveComponent.SetCollisionEnabled` (`self.CapsuleComponent`) "NoCollision")
  (bind _output_get (set `self.Main Boss` mainBoss))
  (`/Engine/EditorBlueprintResources/StandardMacros.IsValid` _output_get
    (:`Is Valid`
      (set `self.goBoss` true)
      (set `/Game/Blueprints/Characters/Enemy/Boss/BPC_BossAttacks.canAttack` false (`self.BPC_BossAttacks`)))
    (:`Is Not Valid`
      (`self.K2_DestroyActor`))))

(event `GoToBoss`
  (bind _main_boss (`self.Main Boss`))
  ;[0 0 0] Return to the boss
  (`/Engine/EditorBlueprintResources/StandardMacros.IsValid` _main_boss
    (:`Is Valid`
      (if (>= (`self.GetDistanceTo` _main_boss self) 15.0)
        (`self.K2_SetActorLocation` (`KismetMathLibrary.VInterpTo` (`self.K2_GetActorLocation`) (`self.K2_GetActorLocation` (`self.Main Boss`)) (`GameplayStatics.GetWorldDeltaSeconds`) 15.0))
        (else
          (`self.K2_DestroyActor`))))))

(fn `coneAttack`
  (`/Game/Blueprints/Characters/Enemy/Boss/BPC_BossAttacks.StartConeAttack` (`self.BPC_BossAttacks`) (`self.bossProjectile`) self (`self.dataAsset`)))

(fn `getHeight`
  (returns (height :type "Float (double-precision)"))
  (return 0.0))

(fn `sprayAttack`
  (`/Game/Blueprints/Characters/Enemy/Boss/BPC_BossAttacks.StartSprayAttack` (`self.BPC_BossAttacks`) (`self.bossProjectile`) self (`self.dataAsset`)))

(fn `UserConstructionScript`
  (`parent.UserConstructionScript`))