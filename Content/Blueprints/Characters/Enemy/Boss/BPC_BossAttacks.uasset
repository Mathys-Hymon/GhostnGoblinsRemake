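; Boss attack component that fires cone and spray fireball attacks, with timing and counts read from a data asset.
; After charging, the cone spawns a fan across an angle centred on the launcher's yaw, pitched toward the player, and sets projectile speed.
; The spray loops through delayed shots, re-aiming at the player each time.
; StopAttack toggles the CanAttack gate, and end-of-attack messages go back to the launch actor.
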(event `StopAttack`
  (set `self.canAttack` (not (`self.canAttack`))))

(event `StartConeAttack`
  (params (Projectil :type "Actor Class Reference") (LunchPos :type "Actor Object Reference") (dataAsset :type "/Game/_Manager/InGame/DataAsset/BP/Boss/BP_BishopDA Object Reference"))
  (bind _returnvalue (`Actor.GetTransform` LunchPos))
  (bind _coneprojectilespeed (`/Game/_Manager/InGame/DataAsset/BP/Boss/BP_BishopDA.coneProjectileSpeed` dataAsset))
  (bind _nbconefireball (`/Game/_Manager/InGame/DataAsset/BP/Boss/BP_BishopDA.nbConeFireBall` dataAsset))
  (bind _coneangle (`/Game/_Manager/InGame/DataAsset/BP/Boss/BP_BishopDA.coneAngle` dataAsset))
  (bind (_returnvalue_roll _returnvalue_pitch) (`KismetMathLibrary.BreakRotator` (`KismetMathLibrary.FindLookAtRotation` (.location _returnvalue) (`Actor.K2_GetActorLocation` (`GameplayStatics.GetPlayerCharacter` 0)))))
  ;[0.3375 0.1599 1] Cone attack
  (`KismetSystemLibrary.Delay` (`/Game/_Manager/InGame/DataAsset/BP/Boss/BP_BishopDA.coneChargingTime` dataAsset))
  (if (`self.canAttack`)
    (for _index (range 1 (+ _nbconefireball 1))
      (bind _returnvalue_2 (`|SpawnActorFromClass` Projectil (`KismetMathLibrary.MakeTransform` (.location _returnvalue) (`KismetMathLibrary.MakeRotator` _returnvalue_roll _returnvalue_pitch (+ (* (- _index 1) (/ _coneangle _nbconefireball)) (- (.yaw (.rotation _returnvalue)) (/ _coneangle 2.0)))) (.scale _returnvalue)) "AlwaysSpawn" "MultiplyWithRoot" null null)) ; Spawn Fire Balls
      (bind _asbp_weapon_parent (cast `/Game/Blueprints/Weapons/BP_WeaponParent` _returnvalue_2))
      (bind _projectilemovement (`/Game/Blueprints/Weapons/BP_WeaponParent.ProjectileMovement` _asbp_weapon_parent))
      (set `ProjectileMovementComponent.InitialSpeed` _coneprojectilespeed _projectilemovement)
      (set `ProjectileMovementComponent.MaxSpeed` _coneprojectilespeed _projectilemovement))
    (message `/Game/Blueprints/BPI/Enemies/BPI_Boss.EndConeAttack` LunchPos)))

(event `StartSprayAttack`
  (params (Projectil :type "Actor Class Reference") (LunchPos :type "Actor Object Reference") (dataAsset :type "/Game/_Manager/InGame/DataAsset/BP/Boss/BP_BishopDA Object Reference"))
  (bind (_returnvalue_location _returnvalue_rotation _returnvalue_scale) (`KismetMathLibrary.BreakTransform` (`Actor.GetTransform` LunchPos)))
  ;[0.02594 0.2132 1] Spray attack
  (`KismetSystemLibrary.Delay` (`/Game/_Manager/InGame/DataAsset/BP/Boss/BP_BishopDA.sprayChargingTime` dataAsset))
  (set `self.actualNbFireBalls` (`/Game/_Manager/InGame/DataAsset/BP/Boss/BP_BishopDA.nbSprayFireBall` dataAsset))
  (bind _output_get (set `self.nbLunchingFireBalls` 0))
  (if (and (< _output_get (`self.actualNbFireBalls`)) (`self.canAttack`)) :!label _label
    (`KismetSystemLibrary.Delay` (`/Game/_Manager/InGame/DataAsset/BP/Boss/BP_BishopDA.shootRate` dataAsset))
    (`/Engine/EditorBlueprintResources/StandardMacros.IncrementInt` (`self.nbLunchingFireBalls`)
      (:`  `
        (if (`self.canAttack`)
          (`|SpawnActorFromClass` Projectil (`KismetMathLibrary.MakeTransform` _returnvalue_location (`KismetMathLibrary.FindLookAtRotation` _returnvalue_location (`Actor.K2_GetActorLocation` (`GameplayStatics.GetPlayerCharacter` 0))) _returnvalue_scale) "AlwaysSpawn" "MultiplyWithRoot" null null) ; Spawn Fire Balls
          (goto _label)
          (else
            (goto _label)))))
    (else
      (message `/Game/Blueprints/BPI/Enemies/BPI_Boss.EndSprayAttack` LunchPos))))