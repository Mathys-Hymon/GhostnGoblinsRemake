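; Bishop boss: a floating ghost enemy that circles the arena center and attacks the player in bursts.
; Tick steers it into a ring around CenterOfArena, easing height toward the player while repositioning, then strafes until an attack is ready.
; Each burst repeats a random number of timeline-driven sideways dashes, each followed by a spray or cone attack from BPCBossAttacks, whose end events chain repeats and cooldowns.
; At zero health it scatters souls and destroys itself.
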(event `self.ReceiveBeginPlay`
  ;[0.1928 1 0] Set a direction for the ghost to follow when encircling player
  (set `self.encircleDirection` (`KismetMathLibrary.MapRangeClamped` (`KismetMathLibrary.Conv_BoolToDouble` (`KismetMathLibrary.RandomBool`)) 0.0 1.0 -1.0 1.0))
  (`SceneComponent.SetHiddenInGame` (`self.Sphere`) true false)
  (`KismetSystemLibrary.Delay` 2.0)
  (set `self.attacker` true))

(event `EndAttack`
  ;[1 0.4091 0] Phase after an attack
  (`SceneComponent.SetHiddenInGame` (`self.Sphere`) true false)
  (set `self.dashing` false)
  (set `self.canAttack` true)
  (`KismetSystemLibrary.Delay` (`KismetMathLibrary.RandomFloatInRange` (`self.minDelayBetweenAttacks`) (`self.maxDelayBetweenAttacks`)))
  (set `self.attacker` true))

(event `self.ReceiveTick`
  (params (DeltaSeconds :type "Float (single-precision)"))
  (`/Engine/EditorBlueprintResources/StandardMacros.IsValid` (`self.centerOfArena`)
    (:`Is Valid`
      (`self.EventTickMoveAttack`))))

(event `AttackAgain`
  ;[1 1 1] Attack Pattern - If can attack, they should dash and then shoot.
  (`self.LookCenter`)
  (bind _output_get (set `self.encircleDirection` (`KismetMathLibrary.MapRangeClamped` (`KismetMathLibrary.Conv_BoolToDouble` (`KismetMathLibrary.RandomBool`)) 0.0 1.0 -1.0 1.0) :!label _label))
  (set `self.dashing` true)
  (bind (_direction _dash_curve) (`Timeline|Timeline` :!via `PlayFromStart`)
    (:`Update`
      (`self.Dash` _output_get _dash_curve))
    (:`Finished`
      ;[0 0 0] Attack
      (set `self.stopLookPlayer` false)
      (set `self.encircleSpeed` 0.0)
      (`MovementComponent.StopMovementImmediately` (`self.CharacterMovement`))
      (if (>= (`self.probabilityOfSprayAttack`) (`KismetMathLibrary.RandomFloatInRange` 0.0 1.0))
        (set `self.strayAttack?` true)
        (`/Game/Blueprints/Characters/Enemy/Boss/BPC_BossAttacks.StartSprayAttack` (`self.BPC_BossAttacks`) (`self.bossProjectile`) self)
        (`KismetSystemLibrary.DelayUntilNextTick`)
        (set `self.strayAttack?` false)
        (else
          (set `self.coneAttack?` true)
          (`/Game/Blueprints/Characters/Enemy/Boss/BPC_BossAttacks.StartConeAttack` (`self.BPC_BossAttacks`) (`self.bossProjectile`) self)
          (`KismetSystemLibrary.DelayUntilNextTick`)
          (set `self.coneAttack?` false))))))

(event `self.CapsuleComponent.OnComponentBeginOverlap`
  (params (OverlappedComponent :type "PrimitiveComponent Object Reference") (OtherActor :type "Actor Object Reference") (OtherComp :type "PrimitiveComponent Object Reference") (OtherBodyIndex :type Integer) (bFromSweep :type Boolean) (SweepResult :type "HitResult Structure (by ref)"))
  ;[1 1 1] On overlap with another pawn, move opposite direction
  (`self.AddMovementInput` (* (`KismetMathLibrary.GetDirectionUnitVector` (`self.K2_GetActorLocation` OtherActor) (`self.K2_GetActorLocation` self)) 100.0)))

(event `self.CapsuleComponent.OnComponentHit`
  (params (HitComponent :type "PrimitiveComponent Object Reference") (OtherActor :type "Actor Object Reference") (OtherComp :type "PrimitiveComponent Object Reference") (NormalImpulse :type "Vector Structure") (Hit :type "HitResult Structure (by ref)"))
  ;[1 1 1] On overlap with another pawn, move opposite direction
  (`/Engine/EditorBlueprintResources/StandardMacros.DoOnce` false :!label _label_2
    (:`Completed`
      (`/Engine/EditorBlueprintResources/StandardMacros.NegateFloat` (`self.encircleDirection`)
        (:`  `
          (`KismetSystemLibrary.Delay` 0.05)
          (`self.ResetDoOnce`))))))

(event `ResetDoOnce`
  ;[1 1 1] On overlap with another pawn, move opposite direction
  (goto _label_2 :!via `Reset`))

(event `EventTickMoveAttack`
  (bind (_returnvalue_x _returnvalue_y _returnvalue_z) (`KismetMathLibrary.BreakVector` (`self.K2_GetActorLocation`)))
  (bind _centerofarena (`self.centerOfArena`))
  (bind _rangefromcenter (`self.rangeFromCenter`))
  (bind _returnvalue (`self.GetDistanceTo` _centerofarena self))
  (bind (_returnvalue_x_2 _returnvalue_y_2 _returnvalue_z_2) (`KismetMathLibrary.BreakVector` (`self.K2_GetActorLocation` (`GameplayStatics.GetPlayerPawn` 0))))
  (bind (_returnvalue_roll _returnvalue_pitch _returnvalue_yaw) (`KismetMathLibrary.BreakRotator` (`KismetMathLibrary.FindLookAtRotation` (`self.K2_GetActorLocation`) (`self.K2_GetActorLocation` (`GameplayStatics.GetPlayerPawn` 0)))))
  (bind (_returnvalue_roll_2 _returnvalue_pitch_2 _returnvalue_yaw_2) (`KismetMathLibrary.BreakRotator` (`KismetMathLibrary.FindLookAtRotation` (`self.K2_GetActorLocation`) (`self.K2_GetActorLocation` _centerofarena))))
  (bind _returnvalue_2 (< (- _rangefromcenter 20.0) _returnvalue))
  (bind _returnvalue_3 (`KismetMathLibrary.FClamp` (/ _returnvalue 1000.0) -1.0))
  (bind _returnvalue_4 (`KismetMathLibrary.Conv_RotatorToVector` (`KismetMathLibrary.MakeRotator` 0.0 0.0 _returnvalue_yaw_2)))
  ;[1 1 1] Calculate distance to player
  (if (or (and (> (+ _rangefromcenter 20.0) _returnvalue) _returnvalue_2) (`self.dashing`))
    (if (`self.canAttack`)
      (if (`self.attacker`)
        ;[1 1 1] Attack Pattern - If can attack, they should dash and then shoot.
        (`SceneComponent.SetHiddenInGame` (`self.Sphere`) false false)
        (set `self.nbAttack` (`KismetMathLibrary.RandomIntegerInRange` (`self.minNbAttack`) (`self.maxNbAttack`)))
        (set `self.attacker` false)
        (set `self.canAttack` false)
        (goto _label)
        (else
          (set `self.encircleSpeed` (`self.baseEncircleSpeed`))
          (`self.EncirclingLogic `)
          (`self.LookCenter`)))
      (elif (`self.stopLookPlayer`)
        (set `self.LookCenter?` false)
        (else
          (`self.K2_SetActorRotation` (`KismetMathLibrary.RInterpTo` (`self.K2_GetActorRotation`) (`KismetMathLibrary.MakeRotator` 0.0 0.0 _returnvalue_yaw) (`GameplayStatics.GetWorldDeltaSeconds`) 10.0)) ; Rotate to face player
          (set `self.LookCenter?` false))))
    (else
      (if _returnvalue_2
        ;[1 1 1] Move towards player
        (`self.AddMovementInput` _returnvalue_4 _returnvalue_3)
        ;[1 1 1] Adjust ghost's height based on player position
        (`self.StopMovement`)
        (else
          (`self.AddMovementInput` _returnvalue_4 (* _returnvalue_3 -1.0))
          (set `self.idle` true)))
      (`self.K2_AddActorWorldOffset` (`KismetMathLibrary.MakeVector` 0.0 0.0 (`KismetMathLibrary.FInterpTo` 0.0 (- (+ _returnvalue_z_2 (`self.height`)) _returnvalue_z) (`GameplayStatics.GetWorldDeltaSeconds`) 1.0)))
      ;[1 1 1] Rotate actor to face center of the arena
      (`self.K2_SetActorRotation` (`KismetMathLibrary.RInterpTo` (`self.K2_GetActorRotation`) (`KismetMathLibrary.MakeRotator` 0.0 0.0 _returnvalue_yaw_2) (`GameplayStatics.GetWorldDeltaSeconds`) 10.0) :!label _label_3)
      (set `self.LookCenter?` true))))

(event `LookCenter`
  ;[1 1 1] Rotate actor to face center of the arena
  (goto _label_3))

(event `/Game/Blueprints/BPI/Enemies/BPI_Boss.EndConeAttack`
  ;[0.3375 0.1599 1] Cone attack
  (bind _result (`/Engine/EditorBlueprintResources/StandardMacros.DecrementInt` (`self.nbAttack`))
    (:`  `
      (if (> _result 0)
        (`self.AttackAgain`)
        (else
          (set `self.stopLookPlayer` true)
          (`KismetSystemLibrary.Delay` (`self.coneAttackCooldown`))
          (`self.EndAttack`))))))

(event `/Game/Blueprints/BPI/Enemies/BPI_Boss.EndSprayAttack`
  ;[0.02594 0.2132 1] Spray attack
  (bind _result (`/Engine/EditorBlueprintResources/StandardMacros.DecrementInt` (`self.nbAttack`))
    (:`  `
      (if (> _result 0)
        (`self.AttackAgain`)
        (else
          (set `self.stopLookPlayer` true)
          (`KismetSystemLibrary.Delay` (`self.sprayAttackCooldown`))
          (`self.EndAttack`))))))

(event `self.ReceiveAnyDamage`
  (params (Damage :type "Float (single-precision)") (DamageType :type "DamageType Object Reference") (InstigatedBy :type "Controller Object Reference") (DamageCauser :type "Actor Object Reference"))
  (bind (_returnvalue_location _returnvalue_rotation _returnvalue_scale) (`KismetMathLibrary.BreakTransform` (`self.GetTransform`)))
  ;[0 1 0.5971] Boss life
  (bind _output_get (set `self.bishopHealth` (- (`self.bishopHealth`) Damage)))
  (if (<= _output_get 0.0)
    (for _ (range 1 (+ (`self.soulsDropped`) 1))
      (`|SpawnActorFromClass` "/Game/Blueprints/Characters/Enemy/Bp_Soul.Bp_Soul_C" (`KismetMathLibrary.MakeTransform` (+ _returnvalue_location (`KismetMathLibrary.MakeVector` (`KismetMathLibrary.RandomFloatInRange` -200.0 200.0) (`KismetMathLibrary.RandomFloatInRange` -200.0 200.0) (`KismetMathLibrary.RandomFloatInRange` -200.0 200.0))) _returnvalue_rotation _returnvalue_scale) "AlwaysSpawn" "MultiplyWithRoot" null null) ; Spawn Fire Balls
    )
    (`KismetSystemLibrary.DelayUntilNextTick`)
    (`self.K2_DestroyActor`)))

(fn `Dash`
  (params (encircleDir :type "Float (double-precision)" :default 1.0) (dashTimeline :type "Float (double-precision) (by ref)"))
  (set `self.stopLookPlayer` true)
  (`self.K2_AddActorWorldOffset` (* (* encircleDir (`self.GetActorRightVector`)) (* dashTimeline (`self.dashDistance`)))))

(fn `EncirclingLogic `
  (bind _charactermovement (`self.CharacterMovement`))
  (bind (_velocity_x _velocity_y _velocity_z) (`KismetMathLibrary.BreakVector` (`MovementComponent.Velocity` _charactermovement)))
  ;[1 1 1] Encircling logic - decrease  X-velocity when in attack range and move along right vector in the set random direction
  (bind _result (`/Engine/EditorBlueprintResources/StandardMacros.DecrementFloat` _velocity_x)
    (:`  `
      (set `MovementComponent.Velocity` (`KismetMathLibrary.MakeVector` _result _velocity_y _velocity_z) _charactermovement)
      (`self.AddMovementInput` (* (`self.GetActorRightVector`) (`self.encircleDirection`)) (`self.encircleSpeed`)))))

(fn `getHeight`
  (returns (height :type "Float (double-precision)"))
  (return 0.0))

(fn `UserConstructionScript`
  (set `self.probabilityOfConeAttack` (- 1.0 (`self.probabilityOfSprayAttack`))))