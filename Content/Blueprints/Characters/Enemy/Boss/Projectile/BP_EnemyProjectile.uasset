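; BP_EnemyProjectile is a boss enemy projectile that damages the player on impact.
; On BeginPlay it pulls damage, speed and lifetime from a child data asset, configures its ProjectileMovement and destroys itself when the lifetime expires.
; A static mesh hit applies damage only to actors implementing BPI_Player, then destroys the projectile on the next tick whatever it struck.
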(event `self.ReceiveBeginPlay`
  (bind _dataassetchild (`self.dataAssetChild`))
  (bind _projectilemovement (`self.ProjectileMovement`))
  (bind _projectilespeed (`/Game/_Manager/InGame/DataAsset/BP/Boss/BP_BishopDA.projectileSpeed` _dataassetchild))
  (`parent.ReceiveBeginPlay`)
  (set `self.damages` (`/Game/_Manager/InGame/DataAsset/BP/Boss/BP_BishopDA.projectileDamage` _dataassetchild))
  (set `ProjectileMovementComponent.InitialSpeed` _projectilespeed _projectilemovement)
  (set `ProjectileMovementComponent.MaxSpeed` _projectilespeed _projectilemovement)
  (`KismetSystemLibrary.Delay` (`/Game/_Manager/InGame/DataAsset/BP/Boss/BP_BishopDA.timeBeforeDeleteProjectil` _dataassetchild))
  (`self.K2_DestroyActor`))

(event `self.StaticMesh.OnComponentHit`
  (params (HitComponent :type "PrimitiveComponent Object Reference") (OtherActor :type "Actor Object Reference") (OtherComp :type "PrimitiveComponent Object Reference") (NormalImpulse :type "Vector Structure") (Hit :type "HitResult Structure (by ref)"))
  (if (`KismetSystemLibrary.DoesImplementInterface` OtherActor "/Game/Blueprints/BPI/Player/BPI_Player.BPI_Player_C")
    (`GameplayStatics.ApplyDamage` OtherActor (`/Game/_Manager/InGame/DataAsset/BP/Boss/BP_BishopDA.projectileDamage` (`self.dataAssetChild`)) null self))
  (`KismetSystemLibrary.DelayUntilNextTick`)
  (`self.K2_DestroyActor`))

(fn `UserConstructionScript`
  (`parent.UserConstructionScript`))