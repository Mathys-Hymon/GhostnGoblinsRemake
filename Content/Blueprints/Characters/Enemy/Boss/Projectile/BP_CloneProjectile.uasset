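; Projectile fired by the boss's clone that damages player actors on hit, with damage, speed and lifetime read from a data asset.
; A random flight sound plays from spawn and fades out on impact or timeout.
; On hit it plays an impact sound, removes the skull and swaps the trail for an impact Niagara effect before destruction.
; Tick ignores a custom collision channel while the player dashes, restoring blocking otherwise.
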(event `self.ReceiveBeginPlay`
  (bind _dataassetchild (`self.dataAssetChild`))
  (bind _projectilemovement (`self.ProjectileMovement`))
  (bind _flyingsoundref (`self.FlyingSoundRef`))
  (bind _cloneprojectilespeed (`/Game/_Manager/InGame/DataAsset/BP/Boss/BP_Bishop2DA.cloneProjectileSpeed` _dataassetchild))
  (`parent.ReceiveBeginPlay`)
  (set `self.damages` (`/Game/_Manager/InGame/DataAsset/BP/Boss/BP_Bishop2DA.cloneProjectileDamage` _dataassetchild))
  (set `ProjectileMovementComponent.InitialSpeed` _cloneprojectilespeed _projectilemovement)
  (set `ProjectileMovementComponent.MaxSpeed` _cloneprojectilespeed _projectilemovement)
  (bind _returnvalue (`GameplayStatics.SpawnSound2D` (`KismetArrayLibrary.Array_Random` (`/Game/_Manager/InGame/DataAsset/BP/SFX/BP_SFX_DA.flightEnemyFireball` (`self.sfxDataAsset`))) 1.0 1.0 0.0 null))
  (set `self.FlyingSoundRef` _returnvalue)
  (`KismetSystemLibrary.Delay` (`/Game/_Manager/InGame/DataAsset/BP/Boss/BP_Bishop2DA.cloneTimeBeforeDeleteProjectil` _dataassetchild))
  (`/Engine/EditorBlueprintResources/StandardMacros.IsValid` _flyingsoundref
    (:`Is Valid`
      (`AudioComponent.FadeOut` _flyingsoundref 0.2 0.0 "Linear")
      (`self.K2_DestroyActor`))))

(event `self.StaticMesh.OnComponentHit`
  (params (HitComponent :type "PrimitiveComponent Object Reference") (OtherActor :type "Actor Object Reference") (OtherComp :type "PrimitiveComponent Object Reference") (NormalImpulse :type "Vector Structure") (Hit :type "HitResult Structure (by ref)"))
  (bind _flyingsoundref (`self.FlyingSoundRef`))
  (if (`KismetSystemLibrary.DoesImplementInterface` OtherActor "/Game/Blueprints/BPI/Player/BPI_Player.BPI_Player_C")
    (`GameplayStatics.ApplyDamage` OtherActor (`/Game/_Manager/InGame/DataAsset/BP/Boss/BP_Bishop2DA.cloneProjectileDamage` (`self.dataAssetChild`)) null self))
  (`/Engine/EditorBlueprintResources/StandardMacros.IsValid` _flyingsoundref
    (:`Is Valid`
      (`AudioComponent.FadeOut` _flyingsoundref 0.2 0.0 "Linear"))
    (:`Is Not Valid`
      _))
  (`GameplayStatics.PlaySoundAtLocation` (`KismetArrayLibrary.Array_Random` (`/Game/_Manager/InGame/DataAsset/BP/SFX/BP_SFX_DA.hitEnemyFireball` (`self.sfxDataAsset`))) (`self.K2_GetActorLocation`) (struct) 1.0 1.0 0.0 "/Game/Imports/SFX/SoundAttenuation.SoundAttenuation" null null null)
  (`/Engine/EditorBlueprintResources/StandardMacros.IsValid` (`self.skull1`)
    (:`Is Valid`
      (`ActorComponent.K2_DestroyComponent` (`self.skull1`))
      (`NiagaraComponent.SetAsset` (`self.trail`) "/Game/Imports/VFX/FX_Boss/FireBall/NS_Impact_Boss_Clone.NS_Impact_Boss_Clone" true)
      (`KismetSystemLibrary.Delay` 2.0)
      (`self.K2_DestroyActor`))))

(event `self.ReceiveTick`
  (params (DeltaSeconds :type "Float (single-precision)"))
  (bind _invicibledash (message `/Game/Blueprints/BPI/Player/BPI_Player.GetIsDashing` (`GameplayStatics.GetPlayerCharacter` 0)))
  (if _invicibledash
    (`PrimitiveComponent.SetCollisionResponseToChannel` (`self.StaticMesh`) "ECC_GameTraceChannel1" "ECR_Ignore")
    (else
      (`PrimitiveComponent.SetCollisionResponseToChannel` (`self.StaticMesh`) "ECC_GameTraceChannel1" "ECR_Block"))))

(fn `UserConstructionScript`
  (`parent.UserConstructionScript`))