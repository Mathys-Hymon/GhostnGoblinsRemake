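; Bishop boss child Blueprint that adds a repeating clone attack once health falls below a data-asset threshold.
; An invincible charge shows two decoy clones, then boss and two real clones reappear 120 degrees apart around the arena center.
; Tick makes clones mirror its position, visibility and attacks; hitting the boss notifies and releases them, enabling a delayed recast.
; Damage also drives half-health music blending and death with soul drops, score and dissolve.
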(event `self.ReceiveBeginPlay`
  (`parent.ReceiveBeginPlay`)
  (bind _output_get (set `self.dataAsset` (`self.dataAssetChild`)))
  (set `self.health` (`/Game/_Manager/InGame/DataAsset/BP/Boss/BP_BishopDA.health` _output_get)))

(event `self.ReceiveTick`
  (params (DeltaSeconds :type "Float (single-precision)"))
  (bind (_returnvalue_location _returnvalue_rotation) (`KismetMathLibrary.BreakTransform` (`self.GetTransform`)))
  (bind (_returnvalue_location_2 _returnvalue_rotation_2) (`KismetMathLibrary.BreakTransform` (`self.GetTransform`)))
  (bind _firstclone (`self.firstClone`))
  (bind _secondclone (`self.SecondClone`))
  (bind _dataassetchild (`self.dataAssetChild`))
  (`parent.ReceiveTick` DeltaSeconds)
  ;[0.7146 1 0] Clone if the boss is midlife
  (if (< (`self.health`) (* (`/Game/_Manager/InGame/DataAsset/BP/Boss/BP_BishopDA.health` (`self.dataAsset`)) (/ (`/Game/_Manager/InGame/DataAsset/BP/Boss/BP_Bishop2DA.cloneBeginning%` (`self.dataAssetChild`)) 100.0)))
    ;[0 0.7791 1] Cloning
    (if (`self.canSpawnClone`)
      (set `self.canAttack` false)
      (`self.LookCenter`)
      (`SceneComponent.SetHiddenInGame` (`self.Mesh`) false false)
      (`/Engine/EditorBlueprintResources/StandardMacros.DoOnce` false :!label _label
        (:`Completed`
          (set `self.movementMode` "NewEnumerator4")
          (set `self.invincible` true) ; Stop shooting
          (`KismetSystemLibrary.DelayUntilNextTick`)
          (`/Game/Blueprints/Characters/Enemy/Boss/BPC_BossAttacks.StopAttack` (`self.BPC_BossAttacks`))
          (set `self.canDash?` false)
          (bind _returnvalue (`|SpawnActorFromClass` "/Game/Blueprints/Characters/Enemy/Boss/Clone/BP_BishopClone.BP_BishopClone_C" (`KismetMathLibrary.MakeTransform` _returnvalue_location_2 _returnvalue_rotation_2) "AlwaysSpawn" "MultiplyWithRoot" null null)) ; Spawn First clone
          (`PrimitiveComponent.SetCollisionEnabled` (`Character.CapsuleComponent` _returnvalue) "NoCollision")
          (set `/Game/Blueprints/Characters/Enemy/Boss/Clone/BP_BishopClone.centerOfArena` (`self.centerOfArena`) _returnvalue)
          (set `/Game/Blueprints/Characters/Enemy/Boss/Clone/BP_BishopClone.cloneRoutine?` false _returnvalue)
          (bind _returnvalue_2 (`|SpawnActorFromClass` "/Game/Blueprints/Characters/Enemy/Boss/Clone/BP_BishopClone.BP_BishopClone_C" (`KismetMathLibrary.MakeTransform` _returnvalue_location _returnvalue_rotation) "AlwaysSpawn" "MultiplyWithRoot" null null)) ; Spawn Second clone
          (`PrimitiveComponent.SetCollisionEnabled` (`Character.CapsuleComponent` _returnvalue_2) "NoCollision")
          (set `/Game/Blueprints/Characters/Enemy/Boss/Clone/BP_BishopClone.centerOfArena` (`self.centerOfArena`) _returnvalue_2)
          (set `/Game/Blueprints/Characters/Enemy/Boss/Clone/BP_BishopClone.encircleDirection` -1.0 _returnvalue_2)
          (set `/Game/Blueprints/Characters/Enemy/Boss/Clone/BP_BishopClone.cloneRoutine?` false _returnvalue_2)
          (`KismetSystemLibrary.Delay` (`/Game/_Manager/InGame/DataAsset/BP/Boss/BP_Bishop2DA.cloneAttackChargeTime` (`self.dataAssetChild`)))
          (set `self.canDash?` true)
          (`/Game/Blueprints/Characters/Enemy/Boss/BPC_BossAttacks.StopAttack` (`self.BPC_BossAttacks`))
          (`self.K2_DestroyActor` _returnvalue)
          (`self.K2_DestroyActor` _returnvalue_2)
          (set `self.canSpawnClone` false)
          (`self.SpawnClone`)))
      (elif (or (`KismetSystemLibrary.IsValid` (`self.firstClone`)) (`KismetSystemLibrary.IsValid` (`self.SecondClone`)))
        ;[0.2207 1 0] Update
        (`/Engine/EditorBlueprintResources/StandardMacros.IsValid` _firstclone
          (:`Is Valid`
            (`self.UpdateClone` _firstclone))
          (:`Is Not Valid`
            _))
        (`/Engine/EditorBlueprintResources/StandardMacros.IsValid` _secondclone
          (:`Is Valid`
            (`self.UpdateClone` _secondclone)))
        (else
          ;[1 1 1] New clones spawning loop
          (`/Engine/EditorBlueprintResources/StandardMacros.DoOnce` false :!label _label_2
            (:`Completed`
              (`KismetSystemLibrary.Delay` (`KismetMathLibrary.RandomFloatInRange` (`/Game/_Manager/InGame/DataAsset/BP/Boss/BP_Bishop2DA.delayCloneAttackMin` _dataassetchild) (`/Game/_Manager/InGame/DataAsset/BP/Boss/BP_Bishop2DA.delayCloneAttackMax` _dataassetchild)))
              (set `self.canSpawnClone` true)
              (`self.CanCloneAgain`))))))))

(event `CanCloneAgain`
  ;[0 0.7791 1] Cloning
  (goto _label :!via `Reset`))

(event `ResetDoOnceCooldown`
  ;[1 1 1] New clones spawning loop
  (goto _label_2 :!via `Reset`))

(event `UpdateClone`
  (params (Clone :type "/Game/Blueprints/Characters/Enemy/Boss/Clone/BP_BishopClone Object Reference"))
  (bind (_returnvalue_x _returnvalue_y _returnvalue_z) (`KismetMathLibrary.BreakVector` (`self.K2_GetActorLocation`)))
  (bind _centerposref (`/Game/Blueprints/Characters/Enemy/Boss/Clone/BP_BishopClone.centerPosRef` Clone))
  (bind _centerposref_2 (`/Game/Blueprints/Characters/Enemy/Boss/Clone/BP_BishopClone.centerPosRef` Clone))
  (bind (_returnvalue_roll _returnvalue_pitch _returnvalue_yaw) (`KismetMathLibrary.BreakRotator` (`KismetMathLibrary.FindLookAtRotation` (`self.K2_GetActorLocation` _centerposref_2) (`self.K2_GetActorLocation`))))
  (bind (_returnvalue_x_2 _returnvalue_y_2) (`KismetMathLibrary.BreakVector` (`KismetMathLibrary.VInterpTo` (`self.K2_GetActorLocation` Clone) (+ (`self.K2_GetActorLocation` _centerposref) (* (`self.GetActorForwardVector` _centerposref) (`self.GetDistanceTo` (`self.centerOfArena`) self))) (`GameplayStatics.GetWorldDeltaSeconds`) 10.0)))
  ;[0 0.06563 0.5052] Update all clones
  (if (== Clone (`self.firstClone`))
    (set `self.cloneTeleporteAngle` 120.0)
    (else
      (set `self.cloneTeleporteAngle` 240.0)))
  (`self.K2_SetActorRotation` _centerposref_2 (`KismetMathLibrary.MakeRotator` 0.0 0.0 (+ _returnvalue_yaw (`self.cloneTeleporteAngle`))) false)
  (`self.K2_SetActorLocation` Clone (`KismetMathLibrary.MakeVector` _returnvalue_x_2 _returnvalue_y_2 _returnvalue_z) false false)
  (set `/Game/Blueprints/Characters/Enemy/Boss/Clone/BP_BishopClone.LookCenter?` (`self.LookCenter?`) Clone)
  (set `/Game/Blueprints/Characters/Enemy/Boss/Clone/BP_BishopClone.stopLookPlayer` (`self.stopLookPlayer`) Clone)
  (`SceneComponent.SetHiddenInGame` (`Character.Mesh` Clone) (`SceneComponent.bHiddenInGame` (`self.Mesh`)) false)
  (set `/Game/Blueprints/Characters/Enemy/Boss/Clone/BP_BishopClone.bossAttack?` (`self.bossAttack?`) Clone)
  (if (`self.strayAttack?`)
    (`/Game/Blueprints/Characters/Enemy/Boss/Clone/BP_BishopClone.sprayAttack` Clone)
    (elif (`self.coneAttack?`)
      (`/Game/Blueprints/Characters/Enemy/Boss/Clone/BP_BishopClone.coneAttack` Clone))))

(event `SpawnClone`
  (bind (_returnvalue_x _returnvalue_y _returnvalue_z) (`KismetMathLibrary.BreakVector` (`self.K2_GetActorLocation`)))
  (bind (_returnvalue_roll _returnvalue_pitch _returnvalue_yaw) (`KismetMathLibrary.BreakRotator` (`self.K2_GetActorRotation`)))
  (bind (_returnvalue_x_2 _returnvalue_y_2 _returnvalue_z_2) (`KismetMathLibrary.BreakVector` (`self.K2_GetActorLocation`)))
  (bind (_returnvalue_roll_2 _returnvalue_pitch_2) (`KismetMathLibrary.BreakRotator` (`self.K2_GetActorRotation`)))
  (bind (_returnvalue_roll_3 _returnvalue_pitch_3 _returnvalue_yaw_2) (`KismetMathLibrary.BreakRotator` (`self.K2_GetActorRotation`)))
  (bind _secondclone (`self.SecondClone`))
  (bind _firstclone (`self.firstClone`))
  (bind (_returnvalue_x_3 _returnvalue_y_3) (`KismetMathLibrary.BreakVector` (`self.K2_GetActorLocation` (`self.centerOfArena`))))
  (bind (_returnvalue_x_4 _returnvalue_y_4) (`KismetMathLibrary.BreakVector` (+ (`KismetMathLibrary.MakeVector` _returnvalue_x_2 _returnvalue_y_2) (* (`self.GetActorForwardVector`) (`/Game/_Manager/InGame/DataAsset/BP/Boss/BP_BishopDA.distanceFromCenter` (`self.dataAssetChild`))))))
  ;[0.3594 0.03917 0] Random teleport and spawn clones
  (`SceneComponent.SetHiddenInGame` (`self.Mesh`) true true)
  (set `self.movementMode` "NewEnumerator3")
  (`/Game/Blueprints/Characters/Enemy/Boss/BPC_BossAttacks.StopAttack` (`self.BPC_BossAttacks`))
  (`self.K2_SetActorLocation` (`KismetMathLibrary.MakeVector` _returnvalue_x_3 _returnvalue_y_3 _returnvalue_z) false true)
  (`self.K2_SetActorRotation` (`KismetMathLibrary.MakeRotator` _returnvalue_roll_2 _returnvalue_pitch_2 (`KismetMathLibrary.RandomFloatInRange` 0.0 360.0)) true)
  ;;[1 1 1] Spawn clones
  (bind _clone (`self.SpawnCloneFonction` (`KismetMathLibrary.MakeRotator` _returnvalue_roll_3 _returnvalue_pitch_3 (+ _returnvalue_yaw_2 120.0))))
  (set `self.firstClone` _clone)
  (bind _clone_2 (`self.SpawnCloneFonction` (`KismetMathLibrary.MakeRotator` _returnvalue_roll _returnvalue_pitch (+ _returnvalue_yaw 240.0))))
  (set `self.SecondClone` _clone_2)
  (set `self.invincible` false)
  (`self.K2_SetActorLocation` (`KismetMathLibrary.MakeVector` _returnvalue_x_4 _returnvalue_y_4 _returnvalue_z_2) false true)
  (`self.LookCenter`)
  ;;[1 1 1] Boss and clones reapear
  (`self.EndAttack`)
  (set `self.nbAttack` 0)
  (`KismetSystemLibrary.Delay` (`/Game/_Manager/InGame/DataAsset/BP/Boss/BP_Bishop2DA.invisiblilityTime` (`self.dataAssetChild`)))
  (`SceneComponent.SetHiddenInGame` (`self.Mesh`) false true)
  (if (not (`self.debugOn`))
    (`SceneComponent.SetHiddenInGame` (`self.ActorName`) true true))
  (`/Engine/EditorBlueprintResources/StandardMacros.IsValid` (`self.firstClone`)
    (:`Is Valid`
      (`SceneComponent.SetHiddenInGame` (`Character.Mesh` _firstclone) false true)
      (`SceneComponent.SetHiddenInGame` (`Character.Mesh` _firstclone) (`SceneComponent.bHiddenInGame` (`self.Mesh`)) false)
      (`/Game/Blueprints/Characters/Enemy/Boss/Clone/BP_BishopClone.ActualiseAttack` _firstclone))
    (:`Is Not Valid`
      _))
  (`/Engine/EditorBlueprintResources/StandardMacros.IsValid` (`self.SecondClone`)
    (:`Is Valid`
      (`SceneComponent.SetHiddenInGame` (`Character.Mesh` _secondclone) false true)
      (`SceneComponent.SetHiddenInGame` (`Character.Mesh` _secondclone) (`SceneComponent.bHiddenInGame` (`self.Mesh`)) false)
      (`/Game/Blueprints/Characters/Enemy/Boss/Clone/BP_BishopClone.ActualiseAttack` _secondclone))
    (:`Is Not Valid`
      _))
  (set `self.canAttack` true)
  (`self.ResetDoOnceCooldown`)
  (set `self.movementMode` "NewEnumerator4")
  (`/Game/Blueprints/Characters/Enemy/Boss/BPC_BossAttacks.StopAttack` (`self.BPC_BossAttacks`)))

(event `self.ReceiveAnyDamage`
  (params (Damage :type "Float (single-precision)") (DamageType :type "DamageType Object Reference") (InstigatedBy :type "Controller Object Reference") (DamageCauser :type "Actor Object Reference"))
  (bind _outactors (`self.GetAttachedActors` false true))
  (bind _returnvalue_location (`KismetMathLibrary.BreakTransform` (`self.GetTransform`)))
  (bind _firstclone (`self.firstClone`))
  (bind _firstclone_2 (`self.firstClone`))
  (bind _secondclone (`self.SecondClone`))
  (bind _secondclone_2 (`self.SecondClone`))
  (bind _soulsdropped (`/Game/_Manager/InGame/DataAsset/BP/Boss/BP_BishopDA.soulsDropped` (`self.dataAsset`)))
  ;[0 0 0] Death
  (if (not (or (`SceneComponent.bHiddenInGame` (`self.Mesh`)) (`self.invincible`)))
    ;;[1 1 1] Kill clone when hit
    (`/Engine/EditorBlueprintResources/StandardMacros.IsValid` _firstclone_2
      (:`Is Valid`
        (`/Game/Blueprints/Characters/Enemy/Boss/Clone/BP_BishopClone.BossHit` _firstclone_2 self))
      (:`Is Not Valid`
        _))
    (`/Engine/EditorBlueprintResources/StandardMacros.IsValid` _secondclone
      (:`Is Valid`
        (`/Game/Blueprints/Characters/Enemy/Boss/Clone/BP_BishopClone.BossHit` _secondclone self))
      (:`Is Not Valid`
        _))
    ;[0 1 0.5971] Boss life
    (bind _output_get (set `self.health` (- (`self.health`) Damage)))
    (`|ExecutionSequence`
      (:`then_0`
        (if (<= _output_get (/ (`/Game/_Manager/InGame/DataAsset/BP/Boss/BP_BishopDA.health` (`self.dataAssetChild`)) 2.0))
          (bind (_direction _alpha) (`Timeline|Timeline_0`)
            (:`Update`
              (message `/Game/Blueprints/BPI/GameInstance/BPI_GameInstance.LerpBossMusic` (`GameplayStatics.GetGameInstance`) _alpha)))))
      (:`then_1`
        (if (<= _output_get 0.0)
          (`/Engine/EditorBlueprintResources/StandardMacros.DoOnce` false
            (:`Completed`
              (`GameplayStatics.PlaySoundAtLocation` (`KismetArrayLibrary.Array_Random` (`/Game/_Manager/InGame/DataAsset/BP/SFX/BP_SFX_DA.deathBishop` (`self.sfxDataAsset`))) (`self.K2_GetActorLocation`) (struct) 1.0 1.0 0.0 "/Game/Imports/SFX/SoundAttenuation.SoundAttenuation" null null null)
              (`/Engine/EditorBlueprintResources/StandardMacros.IsValid` _firstclone
                (:`Is Valid`
                  (`self.K2_DestroyActor` _firstclone))
                (:`Is Not Valid`
                  _))
              (`/Engine/EditorBlueprintResources/StandardMacros.IsValid` _secondclone_2
                (:`Is Valid`
                  (`self.K2_DestroyActor` _secondclone_2))
                (:`Is Not Valid`
                  _))
              (`SkeletalMeshComponent.PlayAnimation` (`self.Mesh`) "/Game/Imports/Animations/Bishop/AnimSequence/bishop_spawn_and_death_pose_v02.bishop_spawn_and_death_pose_v02" false)
              (`KismetSystemLibrary.Delay` 0.5)
              (`|SpawnActorFromClass` "/Game/Imports/VFX/FX_Ultimate_Charge/BP_DropFx.BP_DropFx_C" (`KismetMathLibrary.MakeTransform` _returnvalue_location) "AlwaysSpawn" "MultiplyWithRoot" null (`KismetMathLibrary.SelectInt` _soulsdropped (/ _soulsdropped 2) (!= DamageType "/Game/Blueprints/Characters/Player/BP_UltDamageType.BP_UltDamageType")) null) ; Spawn Fire Balls
              (message `/Game/Blueprints/BPI/Player/BPI_HUD.ShowBossHealthBar` (`PlayerController.GetHUD` (`GameplayStatics.GetPlayerController` 0)) false null)
              ;[0 0 0] Bishop disolve
              (message `/Game/Blueprints/BPI/GameInstance/BPI_GameInstance.GainScore` (`GameplayStatics.GetGameInstance`) (`/Game/_Manager/InGame/DataAsset/BP/Boss/BP_Bishop2DA.score` (`self.dataAssetChild`)))
              (for _array_element _outactors
                (`/Engine/EditorBlueprintResources/StandardMacros.IsValid` _array_element
                  (:`Is Valid`
                    (`self.K2_DestroyActor` _array_element))))
              (`KismetArrayLibrary.Array_Clear` _outactors)
              (`MeshComponent.SetOverlayMaterial` (`self.Mesh`) null)
              (`GameplayStatics.PlaySoundAtLocation` (`KismetArrayLibrary.Array_Random` (`/Game/_Manager/InGame/DataAsset/BP/SFX/BP_SFX_DA.dissolveFXBishop` (`self.sfxDataAsset`))) (`self.K2_GetActorLocation`) (struct) 1.0 1.0 0.0 "/Game/Imports/SFX/SoundAttenuation.SoundAttenuation" null null null)
              (bind (_direction_2 _appear) (`Timeline|Timeline_1` :!via `PlayFromStart`)
                (:`Update`
                  (set `self.canAttack` false)
                  (`MeshComponent.SetScalarParameterValueOnMaterials` (`self.Mesh`) "Alpha" _appear)
                  (`MeshComponent.SetVectorParameterValueOnMaterials` (`self.Mesh`) "Edge Color" (`self.deathColor`)))
                (:`Finished`
                  (`self.K2_DestroyActor`)))))
          (else
            (set `self.firstClone` null)
            (set `self.SecondClone` null)
            (`GameplayStatics.PlaySoundAtLocation` (`KismetArrayLibrary.Array_Random` (`/Game/_Manager/InGame/DataAsset/BP/SFX/BP_SFX_DA.hitBishop` (`self.sfxDataAsset`))) (`self.K2_GetActorLocation`) (struct) 1.0 1.0 0.0 "/Game/Imports/SFX/SoundAttenuation.SoundAttenuation" null null null)))))))

(fn `SpawnCloneFonction`
  (params (`Spawn Transform Rotation` :type "Rotator Structure"))
  (returns (clone :type "/Game/Blueprints/Characters/Enemy/Boss/Clone/BP_BishopClone Object Reference"))
  (bind (_returnvalue_x _returnvalue_y _returnvalue_z) (`KismetMathLibrary.BreakVector` (`self.K2_GetActorLocation`)))
  (bind (_returnvalue_x_2 _returnvalue_y_2) (`KismetMathLibrary.BreakVector` (`self.K2_GetActorLocation` (`self.centerOfArena`))))
  (bind _returnvalue (`|SpawnActorFromClass` "/Game/Blueprints/Characters/Enemy/Boss/Clone/BP_BishopClone.BP_BishopClone_C" (`KismetMathLibrary.MakeTransform` (`KismetMathLibrary.MakeVector` _returnvalue_x_2 _returnvalue_y_2 _returnvalue_z) `Spawn Transform Rotation`) "AlwaysSpawn" "MultiplyWithRoot" null null)) ; Spawn First clone
  (`self.K2_SetActorLocation` _returnvalue (+ (`self.K2_GetActorLocation` _returnvalue) (* (`self.GetActorForwardVector` _returnvalue) (`/Game/_Manager/InGame/DataAsset/BP/Boss/BP_BishopDA.distanceFromCenter` (`self.dataAssetChild`)))) false false)
  (`SceneComponent.SetHiddenInGame` (`Character.Mesh` _returnvalue) true true)
  (set `/Game/Blueprints/Characters/Enemy/Boss/Clone/BP_BishopClone.centerOfArena` (`self.centerOfArena`) _returnvalue)
  (return _returnvalue))

(fn `UserConstructionScript`)