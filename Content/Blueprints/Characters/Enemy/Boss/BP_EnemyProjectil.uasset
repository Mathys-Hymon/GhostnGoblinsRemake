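; BP_EnemyProjectil is a boss enemy projectile that sets its damage and speed on spawn and removes itself after a delay.
; BeginPlay calls the parent, then copies the clone damage into Damages and applies one speed value as both initial and max speed of ProjectileMovement.
; These values and the lifetime are marked as data asset values.
; This Blueprint implements no hit logic, as its overlap and tick events are disabled.
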(event `self.ReceiveBeginPlay`
  (bind _projectilemovement (`self.ProjectileMovement`))
  (bind _projectile_speed (`self.Projectile Speed`))
  (`parent.ReceiveBeginPlay`)
  (set `self.damages` (`self.cloneDamage`))
  (set `ProjectileMovementComponent.InitialSpeed` _projectile_speed _projectilemovement)
  (set `ProjectileMovementComponent.MaxSpeed` _projectile_speed _projectilemovement)
  (`KismetSystemLibrary.Delay` (`self.Time Before Delete`))
  (`self.K2_DestroyActor`))

(fn `UserConstructionScript`
  (`parent.UserConstructionScript`))