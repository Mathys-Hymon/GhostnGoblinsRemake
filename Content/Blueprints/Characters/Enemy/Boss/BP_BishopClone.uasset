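; Destructible clone of the Bishop boss that can fire cone and spray projectile attacks through the BPCBossAttacks component.
; Once CenterOfArena is valid, Tick spawns a position reference actor there once and stores it as CenterPosRef.
; Each tick it smoothly yaws toward the arena center or the player, selected by the LookCenter and StopLookPlayer flags.
; Incoming damage drains CloneHP and destroys the clone a tick after it runs out.
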(event `LookThePlayer`
  (bind (_returnvalue_roll _returnvalue_pitch _returnvalue_yaw) (`KismetMathLibrary.BreakRotator` (`KismetMathLibrary.FindLookAtRotation` (`self.K2_GetActorLocation`) (`self.K2_GetActorLocation` (`GameplayStatics.GetPlayerPawn` 0)))))
  (`self.K2_SetActorRotation` (`KismetMathLibrary.RInterpTo` (`self.K2_GetActorRotation`) (`KismetMathLibrary.MakeRotator` 0.0 0.0 _returnvalue_yaw) (`GameplayStatics.GetWorldDeltaSeconds`) 10.0)))

(event `LookTheCenter`
  (bind (_returnvalue_roll _returnvalue_pitch _returnvalue_yaw) (`KismetMathLibrary.BreakRotator` (`KismetMathLibrary.FindLookAtRotation` (`self.K2_GetActorLocation`) (`self.K2_GetActorLocation` (`self.centerOfArena`)))))
  (`self.K2_SetActorRotation` (`KismetMathLibrary.RInterpTo` (`self.K2_GetActorRotation`) (`KismetMathLibrary.MakeRotator` 0.0 0.0 _returnvalue_yaw) (`GameplayStatics.GetWorldDeltaSeconds`) 10.0)))

(event `self.ReceiveTick`
  (params (DeltaSeconds :type "Float (single-precision)"))
  (if (`KismetSystemLibrary.IsValid` (`self.centerOfArena`))
    (`self.StartClone`)
    (if (`self.LookCenter?`)
      (`self.LookTheCenter`)
      (elif (not (`self.stopLookPlayer`))
        (`self.LookThePlayer`)))))

(event `StartClone`
  (`/Engine/EditorBlueprintResources/StandardMacros.DoOnce` false
    (:`Completed`
      (bind _returnvalue (`|SpawnActorFromClass` "/Game/Blueprints/Characters/Enemy/Boss/BP_ClonePosRef.BP_ClonePosRef_C" (`self.GetTransform` (`self.centerOfArena`)) "AlwaysSpawn" "MultiplyWithRoot" null null))
      (set `self.centerPosRef` _returnvalue))))

(event `self.ReceiveAnyDamage`
  (params (Damage :type "Float (single-precision)") (DamageType :type "DamageType Object Reference") (InstigatedBy :type "Controller Object Reference") (DamageCauser :type "Actor Object Reference"))
  (bind _output_get (set `self.cloneHP` (- (`self.cloneHP`) Damage)))
  (if (<= _output_get 0.0)
    (`KismetSystemLibrary.DelayUntilNextTick`)
    (`self.K2_DestroyActor`)))

(fn `coneAttack`
  (`/Game/Blueprints/Characters/Enemy/Boss/BPC_BossAttacks.StartConeAttack` (`self.BPC_BossAttacks`) (`self.bossProjectile`) self))

(fn `getHeight`
  (returns (height :type "Float (double-precision)"))
  (return 0.0))

(fn `sprayAttack`
  (`/Game/Blueprints/Characters/Enemy/Boss/BPC_BossAttacks.StartSprayAttack` (`self.BPC_BossAttacks`) (`self.bossProjectile`) self))

(fn `UserConstructionScript`
  (`parent.UserConstructionScript`))