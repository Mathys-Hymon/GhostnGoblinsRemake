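; Boss arena actor that spawns the Bishop unique boss the first time the player enters its trigger zone.
; The boss spawns offset along the actor's forward vector, receives the arena center (CenterRef or self) and appears on the HUD health bar.
; Tick watches the boss reference and destroys the actor after a delay once the boss is gone.
; A debug-mode event from the game instance toggles trigger zone visibility.
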(event `self.ReceiveBeginPlay`
  (`SceneComponent.SetVisibility` (`self.TriggerZone`) false false)
  (bind _newcenter (`self.GetCenterArea`))
  (set `self.newCenter` _newcenter)
  ;[0.3542 0 0] Debug mode
  (bind _instanceref (message `/Game/Blueprints/BPI/GameInstance/BPI_GameInstance.GetInstanceRef` (`GameplayStatics.GetGameInstance`)))
  (`KismetSystemLibrary.DelayUntilNextTick`)
  (add `/Game/_Manager/InGame/GI_Game.debugModeChange` _instanceref (delegate `DebugMode`)))

(event `self.ReceiveTick`
  (params (DeltaSeconds :type "Float (single-precision)"))
  ;[0.3542 0 0] Debug mode
  (if (`self.debugOn`)
    (`SceneComponent.SetVisibility` (`self.TriggerZone`) true false))
  ;[0.2518 0.006914 1] Destroy cage after Boss die
  (if (`self.bossIsSpawning`)
    (`/Engine/EditorBlueprintResources/StandardMacros.IsValid` (`self.bossRef`)
      (:`Is Not Valid`
        (`KismetSystemLibrary.Delay` (`self.timeBeforeDestroyAfterBossDie`))
        (`self.K2_DestroyActor`)))))

(event `DebugMode`
  ;[0.3542 0 0] Debug mode
  (bind _debugmode (message `/Game/Blueprints/BPI/GameInstance/BPI_GameInstance.GetDebugMode` (`GameplayStatics.GetGameInstance`)))
  (bind _output_get (set `self.debugOn` _debugmode))
  (`SceneComponent.SetVisibility` (`self.TriggerZone`) _output_get false))

(event `self.TriggerZone.OnComponentBeginOverlap`
  (params (OverlappedComponent :type "PrimitiveComponent Object Reference") (OtherActor :type "Actor Object Reference") (OtherComp :type "PrimitiveComponent Object Reference") (OtherBodyIndex :type Integer) (bFromSweep :type Boolean) (SweepResult :type "HitResult Structure (by ref)"))
  ;[0 0 0] Spawn boos when you enter in the trigger box
  (if (== OtherActor (`GameplayStatics.GetPlayerCharacter` 0))
    (`/Engine/EditorBlueprintResources/StandardMacros.DoOnce` false
      (:`Completed`
        (bind _returnvalue (`|SpawnActorFromClass` "/Game/Blueprints/Characters/Enemy/Boss/BP_BishopUniqueBoss.BP_BishopUniqueBoss_C" (`KismetMathLibrary.MakeTransform` (+ (`self.K2_GetActorLocation` self) (* (`self.GetActorForwardVector` self) (/ (`/Game/_Manager/InGame/DataAsset/BP/Boss/BP_BishopDA.distanceFromCenter` (`self.dataAsset`)) 2.0)))) "Undefined" "MultiplyWithRoot" null null))
        (set `self.bossRef` _returnvalue)
        (set `/Game/Blueprints/Characters/Enemy/Boss/Master/BP_BishopBoss.centerOfArena` (`self.newCenter`) _returnvalue)
        (message `/Game/Blueprints/BPI/Player/BPI_HUD.ShowBossHealthBar` (`PlayerController.GetHUD` (`GameplayStatics.GetPlayerController` 0)) true _returnvalue)
        (set `self.bossIsSpawning` true)))))

(fn `GetCenterArea`
  (returns (newCenter :type "Actor Object Reference"))
  (bind _centerref (`self.centerRef`))
  (`/Engine/EditorBlueprintResources/StandardMacros.IsValid` _centerref
    (:`Is Valid`
      (return _centerref))
    (:`Is Not Valid`
      (return self))))

(fn `UserConstructionScript`)