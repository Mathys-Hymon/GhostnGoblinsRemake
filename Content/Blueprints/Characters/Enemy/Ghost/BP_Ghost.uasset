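; Flying ghost enemy that chases and circles the player, tuned by a data asset and awarding score on death.
; Tick drives a hidden idle state with distance-scaled tick interval, approach with height tracking, and de-aggro teleport back to spawn.
; In range, attackers play a timeline dash, a placeholder print-only attack and a cooldown; others strafe in a random direction, flipped on hits.
; Game-instance debug mode shows velocity and spheres.
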(event `self.ReceiveBeginPlay`
  (bind _dataasset (`self.dataAsset`))
  (bind _dataasset_2 (`self.dataAsset`))
  (set `self.spawn` (`self.K2_GetActorLocation`))
  (set `self.health` (`/Game/_Manager/InGame/DataAsset/BP/BP_GhostDA.health` (`self.dataAsset`)))
  ;[1 1 1] Set a random height for the ghost on spawn
  (set `self.setHeight` (`KismetMathLibrary.RandomFloatInRange` (`/Game/_Manager/InGame/DataAsset/BP/BP_GhostDA.minHeight` _dataasset_2) (`/Game/_Manager/InGame/DataAsset/BP/BP_GhostDA.maxHeight` _dataasset_2)))
  (set `self.encircleDistance` (`KismetMathLibrary.RandomFloatInRange` (`/Game/_Manager/InGame/DataAsset/BP/BP_GhostDA.minEncircleDist` _dataasset) (`/Game/_Manager/InGame/DataAsset/BP/BP_GhostDA.maxEncircleDist` _dataasset)))
  ;[1 1 1] Set a direction for the ghost to follow when encircling player
  (set `self.encircleDirection` (`KismetMathLibrary.MapRangeClamped` (`KismetMathLibrary.Conv_BoolToDouble` (`KismetMathLibrary.RandomBool`)) 0.0 1.0 -1.0 1.0))
  (set `CharacterMovementComponent.MaxFlySpeed` (`/Game/_Manager/InGame/DataAsset/BP/BP_GhostDA.movementSpeed` (`self.dataAsset`)) (`self.CharacterMovement`))
  ;[0 0 0] Debug
  (bind _instanceref (message `/Game/Blueprints/BPI/GameInstance/BPI_GameInstance.GetInstanceRef` (`GameplayStatics.GetGameInstance`)))
  (add `/Game/_Manager/InGame/GI_Game.debugModeChange` _instanceref (delegate `Debug Mode`)))

(event `Debug Mode`
  (bind _textobject (`self.TextObject`))
  ;[0 0 0] Debug
  (bind _debugmode (message `/Game/Blueprints/BPI/GameInstance/BPI_GameInstance.GetDebugMode` (`GameplayStatics.GetGameInstance`)))
  (bind _returnvalue (not _debugmode))
  (`SceneComponent.SetHiddenInGame` (`self.VelocityArrow`) _returnvalue false)
  (`SceneComponent.SetHiddenInGame` _textobject _returnvalue false)
  (`TextRenderComponent.K2_SetText` _textobject (`KismetTextLibrary.Conv_StringToText` (`KismetSystemLibrary.GetObjectName` self)))
  (`SceneComponent.SetHiddenInGame` (`self.VelocityText`) _returnvalue false))

(event `self.ReceiveTick`
  (params (DeltaSeconds :type "Float (single-precision)"))
  (bind _returnvalue (`GameplayStatics.GetPlayerPawn` 0))
  (bind _velocitytext (`self.VelocityText`))
  (bind _charactermovement (`self.CharacterMovement`))
  (bind _dataasset (`self.dataAsset`))
  (bind _returnvalue_2 (`self.GetDistanceTo` _returnvalue self))
  (bind (_velocity_x _velocity_y _velocity_z) (`KismetMathLibrary.BreakVector` (`MovementComponent.Velocity` _charactermovement)))
  (bind (_returnvalue_roll _returnvalue_pitch _returnvalue_yaw) (`KismetMathLibrary.BreakRotator` (`KismetMathLibrary.FindLookAtRotation` (`self.K2_GetActorLocation`) (`self.K2_GetActorLocation` _returnvalue))))
  (bind _returnvalue_3 (<= (`/Game/_Manager/InGame/DataAsset/BP/BP_GhostDA.idleDist` (`self.dataAsset`)) (`self.GetDistanceTo` (`GameplayStatics.GetPlayerPawn` 0) self)))
  (`|ExecutionSequence`
    (:`then_0`
      ;[0 0 0] Debug
      (bind _debugmode (message `/Game/Blueprints/BPI/GameInstance/BPI_GameInstance.GetDebugMode` (`GameplayStatics.GetGameInstance`)))
      (if _debugmode
        (`KismetSystemLibrary.DrawDebugSphere` (`self.spawn`) (`self.de-aggro distance`) 12 (struct :`R` 1.0 :`A` 1.0) 1.0)
        (`KismetSystemLibrary.DrawDebugSphere` (`self.spawn`) 10.0 12 (struct :`A` 1.0) 1.0)
        (`KismetSystemLibrary.DrawDebugSphere` (`SceneComponent.K2_GetComponentLocation` (`self.CapsuleComponent`)) 10.0 12 (struct :`R` 1.0 :`B` 0.852288 :`A` 1.0) 0.5)
        (`SceneComponent.K2_SetWorldRotation` (`self.VelocityArrow`) (`KismetMathLibrary.FindLookAtRotation` (0.0 0.0 0.0) (`self.GetVelocity`)) false false)
        (`SceneComponent.K2_SetWorldRotation` _velocitytext (`KismetMathLibrary.FindLookAtRotation` (`SceneComponent.K2_GetComponentLocation` _velocitytext) (`PlayerCameraManager.GetCameraLocation` (`GameplayStatics.GetPlayerCameraManager` 0))) false false)
        (`TextRenderComponent.K2_SetText` _velocitytext (`|FormatText` "Velocity : {value}" (`KismetMathLibrary.VSize` (`self.GetVelocity`))))))
    (:`then_1`
      (if (`self.idle`)
        ;[1 1 1] Idle Phase - invisible and inactive until player in range
        (set `self.idle` _returnvalue_3)
        (if _returnvalue_3
          ;;[1 0 0] !! Temporary solution
          (`self.SetActorHiddenInGame` true)
          (`self.SetActorTickInterval` (`KismetMathLibrary.FClamp` (/ (- (`self.GetDistanceTo` (`GameplayStatics.GetPlayerPawn` 0) self) (`/Game/_Manager/InGame/DataAsset/BP/BP_GhostDA.idleDist` (`self.dataAsset`))) 4000.0) 0.0 6.0))
          (else
            (`KismetSystemLibrary.PrintString` "Aggro")
            (`self.SetActorHiddenInGame` false)
            (`self.SetActorTickInterval` 0.0)))
        (elif (>= (`KismetMathLibrary.Vector_Distance` (`self.spawn`) (`self.K2_GetActorLocation` (`GameplayStatics.GetPlayerPawn` 0))) (`/Game/_Manager/InGame/DataAsset/BP/BP_GhostDA.de-aggro range` (`self.dataAsset`)))
          ;[1 1 1] De-aggro
          (`MovementComponent.StopMovementImmediately` (`self.CharacterMovement`))
          (`KismetSystemLibrary.PrintString` "deaggro")
          (`self.SetActorHiddenInGame` true)
          (`self.K2_SetActorLocation` (`self.spawn`) false true)
          (set `self.idle` true)
          (`TimelineComponent.SetPlaybackPosition` (`self.Timeline`) 0.0 false true)
          (else
            ;[1 1 1] Calculate distance to player
            (if (>= (`self.encircleDistance`) _returnvalue_2)
              (`self.Adjust Height`)
              (if (`self.canAttack`)
                (if (`self.attacker`)
                  ;[1 1 1] Attack Pattern - If the ghost is an attacker, and can attack, they should dash and then shoot. Then there is a "cooldown" for their next attack pattern
                  (set `self.canAttack` false)
                  (bind _output_get (set `self.encircleDirection` (`KismetMathLibrary.MapRangeClamped` (`KismetMathLibrary.Conv_BoolToDouble` (`KismetMathLibrary.RandomBool`)) 0.0 1.0 -1.0 1.0)))
                  (bind (_direction _dash_curve) (`Timeline|Timeline` :!via `PlayFromStart`)
                    (:`Update`
                      (`self.Dash` _output_get _dash_curve))
                    (:`Finished`
                      (`self.Attack`)
                      (`KismetSystemLibrary.Delay` (`/Game/_Manager/InGame/DataAsset/BP/BP_GhostDA.attackCooldown` (`self.dataAsset`)))
                      (set `self.canAttack` true)))
                  (else
                    (set `self.encircleSpeed` (`/Game/_Manager/InGame/DataAsset/BP/BP_GhostDA.movementSpeed` (`self.dataAsset`)))
                    ;[1 1 1] Encircling logic - decrease  X-velocity when in attack range and move along right vector in the set random direction
                    (bind _result (`/Engine/EditorBlueprintResources/StandardMacros.DecrementFloat` _velocity_x :!label _label)
                      (:`  `
                        (set `MovementComponent.Velocity` (`KismetMathLibrary.MakeVector` _result _velocity_y _velocity_z) _charactermovement)
                        (`self.AddMovementInput` (* (`self.GetActorRightVector`) (`self.encircleDirection`)) (`KismetMathLibrary.FClamp` (`self.encircleSpeed`) -1.0))
                        (`self.K2_SetActorRotation` (`KismetMathLibrary.RInterpTo` (`self.K2_GetActorRotation`) (`KismetMathLibrary.MakeRotator` 0.0 0.0 _returnvalue_yaw) (`GameplayStatics.GetWorldDeltaSeconds`)) :!label _label_2) ; Rotate to face player
                      ))))
                (else
                  (set `self.encircleSpeed` (`/Game/_Manager/InGame/DataAsset/BP/BP_GhostDA.attackingMovementSpeed` _dataasset)) ; Attacking ghosts move slower
                  (set `self.encircleDistance` (`KismetMathLibrary.RandomFloatInRange` (`/Game/_Manager/InGame/DataAsset/BP/BP_GhostDA.minAttackEncircleDist` _dataasset) (`/Game/_Manager/InGame/DataAsset/BP/BP_GhostDA.maxAttackEncircleDist` _dataasset)))
                  (goto _label)))
              (else
                ;[1 1 1] Move towards player
                (`self.AddMovementInput` (`KismetMathLibrary.Conv_RotatorToVector` (`KismetMathLibrary.MakeRotator` 0.0 0.0 _returnvalue_yaw)) (`KismetMathLibrary.FClamp` (/ _returnvalue_2 1000.0) -1.0))
                ;[1 1 1] Adjust ghost's height based on player position
                (`self.Adjust Height`)
                (goto _label_2)))))))))

(event `self.CapsuleComponent.OnComponentBeginOverlap`
  (params (OverlappedComponent :type "PrimitiveComponent Object Reference") (OtherActor :type "Actor Object Reference") (OtherComp :type "PrimitiveComponent Object Reference") (OtherBodyIndex :type Integer) (bFromSweep :type Boolean) (SweepResult :type "HitResult Structure (by ref)"))
  ;[1 1 1] On overlap with another pawn, move opposite direction
  (`self.AddMovementInput` (* (`KismetMathLibrary.GetDirectionUnitVector` (`self.K2_GetActorLocation` OtherActor) (`self.K2_GetActorLocation` self)) 100.0)))

(event `self.CapsuleComponent.OnComponentHit`
  (params (HitComponent :type "PrimitiveComponent Object Reference") (OtherActor :type "Actor Object Reference") (OtherComp :type "PrimitiveComponent Object Reference") (NormalImpulse :type "Vector Structure") (Hit :type "HitResult Structure (by ref)"))
  ;[1 1 1] When ghosts hit a wall, change encircle direction
  (`/Engine/EditorBlueprintResources/StandardMacros.DoOnce` false :!label _label_3
    (:`Completed`
      (`/Engine/EditorBlueprintResources/StandardMacros.NegateFloat` (`self.encircleDirection`)
        (:`  `
          (`KismetSystemLibrary.Delay` 0.05)
          (`self.ResetDoOnce`))))))

(event `ResetDoOnce`
  ;[1 1 1] When ghosts hit a wall, change encircle direction
  (goto _label_3 :!via `Reset`))

(event `self.ReceiveAnyDamage`
  (params (Damage :type "Float (single-precision)") (DamageType :type "DamageType Object Reference") (InstigatedBy :type "Controller Object Reference") (DamageCauser :type "Actor Object Reference"))
  (bind _out_actors (`self.Out Actors`))
  ;[1 1 1] Take damage when hit
  (if (not (`self.idle`))
    (set `self.health` (- (`self.health`) Damage))
    (if (<= (`self.health`) 0.0)
      (message `/Game/Blueprints/BPI/GameInstance/BPI_GameInstance.GainScore` (`GameplayStatics.GetGameInstance`) (`/Game/_Manager/InGame/DataAsset/BP/BP_GhostDA.score` (`self.dataAsset`)))
      (set `self.Out Actors` (`self.GetAttachedActors` false true))
      (for _array_element _out_actors
        (`/Engine/EditorBlueprintResources/StandardMacros.IsValid` _array_element
          (:`Is Valid`
            (`self.K2_DestroyActor` _array_element))))
      (`KismetArrayLibrary.Array_Clear` _out_actors)
      (`self.K2_DestroyActor`))))

(fn `Adjust Height`
  (bind (_returnvalue_x _returnvalue_y _returnvalue_z) (`KismetMathLibrary.BreakVector` (`self.K2_GetActorLocation`)))
  (bind (_returnvalue_x_2 _returnvalue_y_2 _returnvalue_z_2) (`KismetMathLibrary.BreakVector` (`self.K2_GetActorLocation` (`GameplayStatics.GetPlayerPawn` 0))))
  (`self.K2_AddActorWorldOffset` (`KismetMathLibrary.MakeVector` 0.0 0.0 (`KismetMathLibrary.FInterpTo` 0.0 (- (+ _returnvalue_z_2 (`self.setHeight`)) _returnvalue_z) (`GameplayStatics.GetWorldDeltaSeconds`) 1.0))))

(fn `Attack`
  (`KismetSystemLibrary.PrintString` "Bang"))

(fn `Dash`
  (params (encircleDir :type "Float (double-precision)" :default 1.0) (dashTimeline :type "Float (double-precision) (by ref)"))
  (`self.K2_AddActorWorldOffset` (* (* encircleDir (`self.GetActorRightVector`)) (* dashTimeline (`/Game/_Manager/InGame/DataAsset/BP/BP_GhostDA.dashDist` (`self.dataAsset`))))))

(fn `getHeight`
  (returns (height :type "Float (double-precision)"))
  (return (`CapsuleComponent.CapsuleHalfHeight` (`self.CapsuleComponent`))))

(fn `UserConstructionScript`)