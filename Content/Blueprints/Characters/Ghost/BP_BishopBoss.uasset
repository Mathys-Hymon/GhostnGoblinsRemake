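; Bishop ghost boss that circles the arena center, attacks the player with projectiles, and spawns souls on death.
; Tick logic flies it toward the center until in range, then alternates encircling with attack sequences gated by Attacker and CanAttack, showing a sphere while attacking.
; Each sequence chains a random number of timeline-driven side dashes, each followed by a probability-picked cone or spray of BP_Dagger projectiles, then a cooldown.
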(event `self.ReceiveTick`
  (params (DeltaSeconds :type "Float (single-precision)"))
  (`self.EventTickMoveAttack`))

(event `self.ReceiveBeginPlay`
  ;[0.1928 1 0] Set a direction for the ghost to follow when encircling player
  (set `self.encircleDirection` (`KismetMathLibrary.MapRangeClamped` (`KismetMathLibrary.Conv_BoolToDouble` (`KismetMathLibrary.RandomBool`)) 0.0 1.0 -1.0 1.0))
  (`KismetSystemLibrary.Delay` 2.0)
  (set `self.attacker` true)
  (`SceneComponent.SetHiddenInGame` (`self.Sphere`) true false))

(event `EndAttack`
  ;[1 0.4091 0] Phase after an attack
  (`SceneComponent.SetHiddenInGame` (`self.Sphere`) true false)
  (set `self.canAttack` true)
  (`KismetSystemLibrary.Delay` (`KismetMathLibrary.RandomFloatInRange` (`self.minDelayBetweenAttacks`) (`self.maxDelayBetweenAttacks`)))
  (set `self.attacker` true))

(event `self.CapsuleComponent.OnComponentBeginOverlap`
  (params (OverlappedComponent :type "PrimitiveComponent Object Reference") (OtherActor :type "Actor Object Reference") (OtherComp :type "PrimitiveComponent Object Reference") (OtherBodyIndex :type Integer) (bFromSweep :type Boolean) (SweepResult :type "HitResult Structure (by ref)"))
  ;[1 1 1] On overlap with another pawn, move opposite direction
  (`self.AddMovementInput` (* (`KismetMathLibrary.GetDirectionUnitVector` (`self.K2_GetActorLocation` OtherActor) (`self.K2_GetActorLocation` self)) 100.0)))

(event `AttackAgain`
  ;[1 1 1] Attack Pattern - If can attack, they should dash and then shoot.
  (bind _output_get (set `self.encircleDirection` (`KismetMathLibrary.MapRangeClamped` (`KismetMathLibrary.Conv_BoolToDouble` (`KismetMathLibrary.RandomBool`)) 0.0 1.0 -1.0 1.0) :!label _label))
  (bind (_direction _dash_curve) (`Timeline|Timeline` :!via `PlayFromStart`)
    (:`Update`
      (`self.Dash` _output_get _dash_curve))
    (:`Finished`
      (`self.Attack`))))

(event `self.CapsuleComponent.OnComponentHit`
  (params (HitComponent :type "PrimitiveComponent Object Reference") (OtherActor :type "Actor Object Reference") (OtherComp :type "PrimitiveComponent Object Reference") (NormalImpulse :type "Vector Structure") (Hit :type "HitResult Structure (by ref)"))
  ;[1 1 1] On overlap with another pawn, move opposite direction
  (`/Engine/EditorBlueprintResources/StandardMacros.DoOnce` false :!label _label_2
    (:`Completed`
      (`/Engine/EditorBlueprintResources/StandardMacros.NegateFloat` (`self.encircleDirection`)
        (:`  `
          (`KismetSystemLibrary.Delay` 0.05)
          (`self.ResetDoOnce`))))))

(event `ResetDoOnce`
  ;[1 1 1] On overlap with another pawn, move opposite direction
  (goto _label_2 :!via `Reset`))

(event `EventTickMoveAttack`
  (bind (_returnvalue_x _returnvalue_y _returnvalue_z) (`KismetMathLibrary.BreakVector` (`self.K2_GetActorLocation`)))
  (bind _centerofarena (`self.centerOfArena`))
  (bind (_returnvalue_x_2 _returnvalue_y_2 _returnvalue_z_2) (`KismetMathLibrary.BreakVector` (`self.K2_GetActorLocation` (`self.centerOfArena`))))
  (bind _returnvalue (`self.GetDistanceTo` _centerofarena self))
  (bind (_returnvalue_roll _returnvalue_pitch _returnvalue_yaw) (`KismetMathLibrary.BreakRotator` (`KismetMathLibrary.FindLookAtRotation` (`self.K2_GetActorLocation`) (`self.K2_GetActorLocation` _centerofarena))))
  ;[1 1 1] Calculate distance to player
  (if (>= (`self.rangeFromCenter`) _returnvalue)
    (if (`self.canAttack`)
      (if (`self.attacker`)
        ;[1 1 1] Attack Pattern - If can attack, they should dash and then shoot.
        (`SceneComponent.SetHiddenInGame` (`self.Sphere`) false false)
        (set `self.nbAttack` (`KismetMathLibrary.RandomIntegerInRange` (`self.minNbAttack`) (`self.maxNbAttack`)))
        (set `self.attacker` false)
        (set `self.canAttack` false)
        (goto _label)
        (else
          (set `self.encircleSpeed` (`self.baseEncircleSpeed`))
          (`self.EncirclingLogic `)
          (`self.K2_SetActorRotation` (`KismetMathLibrary.RInterpTo` (`self.K2_GetActorRotation`) (`KismetMathLibrary.MakeRotator` 0.0 0.0 _returnvalue_yaw) (`GameplayStatics.GetWorldDeltaSeconds`)) :!label _label_3) ; Rotate to face player
        ))
      (elif (not (`self.stopLookPlayer`))
        (`self.RotateToPlayer`)))
    (else
      ;[1 1 1] Move towards player
      (`self.AddMovementInput` (`KismetMathLibrary.Conv_RotatorToVector` (`KismetMathLibrary.MakeRotator` 0.0 0.0 _returnvalue_yaw)) (`KismetMathLibrary.FClamp` (/ _returnvalue 1000.0) -1.0))
      ;[1 1 1] Adjust ghost's height based on player position
      (`self.K2_AddActorWorldOffset` (`KismetMathLibrary.MakeVector` 0.0 0.0 (`KismetMathLibrary.FInterpTo` 0.0 (- (+ _returnvalue_z_2 (`self.height`)) _returnvalue_z) (`GameplayStatics.GetWorldDeltaSeconds`) 1.0)))
      (goto _label_3))))

(event `StartConeAttack`
  (bind _returnvalue (`self.GetTransform`))
  (bind _actualnbfireballs (`self.actualNbFireBalls`))
  ;[0.3375 0.1599 1] Cone attack
  (set `self.encircleSpeed` 0.0)
  (set `MovementComponent.Velocity` (0.0 0.0 0.0) (`self.CharacterMovement`))
  (`KismetSystemLibrary.Delay` (`self.coneChargingTime`))
  (set `self.actualNbFireBalls` (`self.nbConeFireBalls`))
  (for _index (range 1 (+ _actualnbfireballs 1))
    ;;[1 0 0] Change for enemy projectil
    (bind _returnvalue_2 (`|SpawnActorFromClass` "/Game/Blueprints/Weapons/WeaponsBlueprints/BP_Dagger.BP_Dagger_C" (`KismetMathLibrary.MakeTransform` (.location _returnvalue) (`KismetMathLibrary.MakeRotator` (.roll (.rotation _returnvalue)) (.pitch (.rotation _returnvalue)) (+ (* _index (/ (`self.coneFireBallAngle`) _actualnbfireballs)) (- (.yaw (.rotation _returnvalue)) (/ (`self.coneFireBallAngle`) 2.0)))) (.scale _returnvalue)) "AlwaysSpawn" "MultiplyWithRoot" null null)) ; Spawn Fire Balls
    ;;[1 0 0] modifie attack damage
    (set `/Game/Blueprints/Weapons/BP_WeaponParent.damages` (`self.projectileDamage`) _returnvalue_2))
  (`self.ShootAgain?`
    (:`true`
      (`self.AttackAgain`))
    (:`false`
      (set `self.stopLookPlayer` true)
      (`KismetSystemLibrary.Delay` (`self.coneAttackCooldown`))
      (`self.EndAttack`)
      (set `self.stopLookPlayer` false))))

(event `StartSprayAttack`
  ;[0.02594 0.2132 1] Spay attack
  (set `self.encircleSpeed` 0.0)
  (set `MovementComponent.Velocity` (0.0 0.0 0.0) (`self.CharacterMovement`))
  (`KismetSystemLibrary.Delay` (`self.sprayChargingTime`))
  (set `self.actualNbFireBalls` (`self.nbSprayFireBalls`))
  (bind _output_get (set `self.nbLunchingFireBalls` 0))
  (if (< _output_get (`self.actualNbFireBalls`)) :!label _label_4
    (`KismetSystemLibrary.Delay` (`self.shootRate`))
    (`/Engine/EditorBlueprintResources/StandardMacros.IncrementInt` (`self.nbLunchingFireBalls`)
      (:`  `
        ;;[1 0 0] Change for enemy projectil
        (bind _returnvalue (`|SpawnActorFromClass` "/Game/Blueprints/Weapons/WeaponsBlueprints/BP_Dagger.BP_Dagger_C" (`self.GetTransform`) "AlwaysSpawn" "MultiplyWithRoot" null null)) ; Spawn Fire Balls
        ;;[1 0 0] modifie attack damage
        (set `/Game/Blueprints/Weapons/BP_WeaponParent.damages` (`self.projectileDamage`) _returnvalue)
        (goto _label_4)))
    (else
      (`self.ShootAgain?`
        (:`true`
          (`self.AttackAgain`))
        (:`false`
          (set `self.stopLookPlayer` true)
          (`KismetSystemLibrary.Delay` (`self.sprayAttackCooldown`))
          (`self.EndAttack`)
          (set `self.stopLookPlayer` false))))))

(event `self.ReceiveAnyDamage`
  (params (Damage :type "Float (single-precision)") (DamageType :type "DamageType Object Reference") (InstigatedBy :type "Controller Object Reference") (DamageCauser :type "Actor Object Reference"))
  (bind (_returnvalue_location _returnvalue_rotation _returnvalue_scale) (`KismetMathLibrary.BreakTransform` (`self.GetTransform`)))
  ;[0 1 0.5971] Boss life
  (bind _output_get (set `self.bishopHealth` (- (`self.bishopHealth`) Damage)))
  (if (<= _output_get 0.0)
    (for _ (range 1 (+ (`self.soulsDropped`) 1))
      (`|SpawnActorFromClass` "/Game/Blueprints/Bp_Soul.Bp_Soul_C" (`KismetMathLibrary.MakeTransform` (+ _returnvalue_location (`KismetMathLibrary.RandomFloatInRange` -100.0 100.0)) _returnvalue_rotation _returnvalue_scale) "AlwaysSpawn" "MultiplyWithRoot" null null) ; Spawn Fire Balls
      (`KismetSystemLibrary.DelayUntilNextTick`)
      (`self.K2_DestroyActor`))))

(fn `Attack`
  (if (>= (`self.probabilityOfSprayAttack`) (`KismetMathLibrary.RandomFloatInRange` 0.0 1.0))
    (`self.StartSprayAttack`)
    (else
      (`self.StartConeAttack`))))

(fn `Dash`
  (params (encircleDir :type "Float (double-precision)" :default 1.0) (dashTimeline :type "Float (double-precision) (by ref)"))
  (`self.K2_AddActorWorldOffset` (* (* encircleDir (`self.GetActorRightVector`)) (* dashTimeline (`self.dashDistance`)))))

(fn `EncirclingLogic `
  (bind _charactermovement (`self.CharacterMovement`))
  (bind (_velocity_x _velocity_y _velocity_z) (`KismetMathLibrary.BreakVector` (`MovementComponent.Velocity` _charactermovement)))
  ;[1 1 1] Encircling logic - decrease  X-velocity when in attack range and move along right vector in the set random direction
  (bind _result (`/Engine/EditorBlueprintResources/StandardMacros.DecrementFloat` _velocity_x)
    (:`  `
      (set `MovementComponent.Velocity` (`KismetMathLibrary.MakeVector` _result _velocity_y _velocity_z) _charactermovement)
      (`self.AddMovementInput` (* (`self.GetActorRightVector`) (`self.encircleDirection`)) (`self.encircleSpeed`)))))

(fn `RotateToPlayer`
  (bind (_returnvalue_roll _returnvalue_pitch _returnvalue_yaw) (`KismetMathLibrary.BreakRotator` (`KismetMathLibrary.FindLookAtRotation` (`self.K2_GetActorLocation`) (`self.K2_GetActorLocation` (`GameplayStatics.GetPlayerPawn` 0)))))
  (`self.K2_SetActorRotation` (`KismetMathLibrary.RInterpTo` (`self.K2_GetActorRotation`) (`KismetMathLibrary.MakeRotator` 0.0 0.0 _returnvalue_yaw) (`GameplayStatics.GetWorldDeltaSeconds`))) ; Rotate to face player
)

(fn `UserConstructionScript`
  (set `self.probabilityOfConeAttack` (- 1.0 (`self.probabilityOfSprayAttack`))))