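; BP_Ghost is a ghost character that follows the first player until it comes within attack distance.
; Each tick outside that range, it moves along the yaw toward the player, with input scaled by distance.
; An interpolated Z offset eases it toward a hover height above the player, and its rotation is set through RInterpTo.
; The graph contains no attack logic, only this movement.
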(event `self.ReceiveTick`
  (params (DeltaSeconds :type "Float (single-precision)"))
  (bind _returnvalue (`GameplayStatics.GetPlayerPawn` 0))
  (bind (_returnvalue_x _returnvalue_y _returnvalue_z) (`KismetMathLibrary.BreakVector` (`self.K2_GetActorLocation`)))
  (bind _returnvalue_2 (`self.GetDistanceTo` _returnvalue self))
  (bind (_returnvalue_x_2 _returnvalue_y_2 _returnvalue_z_2) (`KismetMathLibrary.BreakVector` (`self.K2_GetActorLocation` (`GameplayStatics.GetPlayerPawn` 0))))
  (bind (_returnvalue_roll _returnvalue_pitch _returnvalue_yaw) (`KismetMathLibrary.BreakRotator` (`KismetMathLibrary.FindLookAtRotation` (`self.K2_GetActorLocation`) (`self.K2_GetActorLocation` _returnvalue))))
  (if (not (>= (`self.attackDistance`) _returnvalue_2))
    (`self.AddMovementInput` (`KismetMathLibrary.Conv_RotatorToVector` (`KismetMathLibrary.MakeRotator` 0.0 0.0 _returnvalue_yaw)) (`KismetMathLibrary.FClamp` (/ _returnvalue_2 1000.0) -1.0))
    (`self.K2_AddActorWorldOffset` (`KismetMathLibrary.MakeVector` 0.0 0.0 (`KismetMathLibrary.FInterpTo` 0.0 (- (+ _returnvalue_z_2 250.0) _returnvalue_z) (`GameplayStatics.GetWorldDeltaSeconds`) 1.0)))
    (`self.K2_SetActorRotation` (`KismetMathLibrary.RInterpTo` (struct) (struct) (`GameplayStatics.GetWorldDeltaSeconds`)))))

(fn `UserConstructionScript`)