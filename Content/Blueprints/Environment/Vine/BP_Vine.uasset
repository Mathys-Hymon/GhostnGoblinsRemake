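; Procedural vine actor that builds branching vines with leaves in its construction script.
; Seeded random streams generate primary splines, secondary splines branching from their points, and leaf positions picked from spline nodes; zero seeds get randomized.
; Optional Project line-traces spline points and leaves along actor down onto surfaces.
; Render replaces splines with collision-free, shadowless spline meshes and leaf meshes; otherwise debug spheres preview leaves.
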(fn `CreateMesh`
  (params (SplineComponent :type "SplineComponent Object Reference"))
  (locals (`Spline to Mesh` :type "SplineComponent Object Reference") (XLength :type "Float (double-precision)" :default 0.0))
  (bind _spline_to_mesh (`local.Spline to Mesh`))
  (bind _spline_to_mesh_2 (`local.Spline to Mesh`))
  (bind (_returnvalue_min _returnvalue_max) (break `Box` (`StaticMesh.GetBoundingBox` (`self.VineMesh`))))
  (bind _returnvalue_x (`KismetMathLibrary.BreakVector` (+ (`KismetMathLibrary.Vector_GetAbs` _returnvalue_min) (`KismetMathLibrary.Vector_GetAbs` _returnvalue_max))))
  (set `local.Spline to Mesh` SplineComponent)
  (bind _output_get (set `local.XLength` _returnvalue_x))
  (for _index (range (+ (`KismetMathLibrary.FTrunc` (/ (`SplineComponent.GetSplineLength` (`local.Spline to Mesh`)) _output_get)) 1))
    (bind _returnvalue (`AddComponent|NODE_AddSplineMeshComponent-1`))
    (`PrimitiveComponent.SetCastShadow` _returnvalue false)
    (`PrimitiveComponent.SetCollisionEnabled` _returnvalue "NoCollision")
    (`SplineMeshComponent.SetForwardAxis` _returnvalue "X" true)
    (`StaticMeshComponent.SetStaticMesh` _returnvalue (`self.VineMesh`))
    (bind _returnvalue_2 (* _index (`local.XLength`)))
    (bind _returnvalue_3 (* (+ _index 1) (`local.XLength`)))
    (`SplineMeshComponent.SetStartAndEnd` _returnvalue (`SplineComponent.GetLocationAtDistanceAlongSpline` _spline_to_mesh_2 _returnvalue_2 "Local") (`KismetMathLibrary.ClampVectorSize` (`SplineComponent.GetTangentAtDistanceAlongSpline` _spline_to_mesh_2 _returnvalue_2 "Local") 0.0 (`local.XLength`)) (`SplineComponent.GetLocationAtDistanceAlongSpline` _spline_to_mesh _returnvalue_3 "Local") (`KismetMathLibrary.ClampVectorSize` (`SplineComponent.GetTangentAtDistanceAlongSpline` _spline_to_mesh _returnvalue_3 "Local") 0.0 (`local.XLength`)) true))
  (for (_array_element _array_index) (`self.LeafPos`)
    (bind _returnvalue_4 (`AddComponent|NODE_AddStaticMeshComponent-0` :`RelativeTransform` (`KismetMathLibrary.MakeTransform` _array_element (`KismetMathLibrary.MakeRotator` 0.0 0.0 (`KismetMathLibrary.RandomFloatInRangeFromStream` (`KismetMathLibrary.MakeRandomStream` _array_index) -20.0 20.0)))))
    (`SceneComponent.K2_SetWorldLocation` _returnvalue_4 _array_element false false)
    (`PrimitiveComponent.SetCastShadow` _returnvalue_4 false)
    (`PrimitiveComponent.SetCollisionEnabled` _returnvalue_4 "NoCollision")
    (`StaticMeshComponent.SetStaticMesh` _returnvalue_4 (`self.LeafMesh`))))

(fn `GenerateLeafLoc`
  (locals (LeafSeed :type "RandomStream Structure"))
  (if (!= (`KismetArrayLibrary.Array_Length` (`self.LeafSeeds`)) 0)
    (for _array_element (`self.LeafSeeds`)
      (bind _output_get (set `local.LeafSeed` (`KismetMathLibrary.MakeRandomStream` _array_element)))
      (`KismetArrayLibrary.Array_Add` (`self.LeafPos`) (`|GetArrayItem` (`self.AllPos`) (`KismetMathLibrary.RandomIntegerFromStream` _output_get (- (`KismetArrayLibrary.Array_Length` (`self.AllPos`)) 1)))))
    (`KismetSystemLibrary.FlushPersistentDebugLines`)
    (if (not (`self.Render`))
      (for _array_element_2 (`self.LeafPos`)
        (`KismetSystemLibrary.DrawDebugSphere` _array_element_2 5.0 12 (struct :`R` 0.01871 :`G` 1.0 :`A` 1.0) 10000000000000.0)))))

(fn `GetNodeLocations`
  (for _array_element (`self.PrimarySplines`)
    (for _index (range 1 (+ (`SplineComponent.GetNumberOfSplinePoints` _array_element) 1))
      (`KismetArrayLibrary.Array_Add` (`self.AllPos`) (`SplineComponent.GetLocationAtSplinePoint` _array_element _index "World"))))
  (for _array_element_2 (`self.SecondarySplines`)
    (for _index_2 (range 1 (+ (`SplineComponent.GetNumberOfSplinePoints` _array_element_2) 1))
      (`KismetArrayLibrary.Array_Add` (`self.AllPos`) (`SplineComponent.GetLocationAtSplinePoint` _array_element_2 _index_2 "World")))))

(fn `MakePrimaryBranches`
  (locals (`Last Location` :type "Vector Structure" :default (0.0 0.0 0.0)) (PBranch :type "SplineComponent Object Reference") (`Primary BSeed` :type "RandomStream Structure" :default (struct :`InitialSeed` 1234)))
  (bind _pbranch (`local.PBranch`))
  (bind _returnvalue (`KismetMathLibrary.RotateAngleAxis` (`self.ForwardVec`) (`KismetMathLibrary.RandomFloatInRangeFromStream` (`local.Primary BSeed`) (`self.Min Degree`) (`self.Max Degree`)) (`self.GetActorUpVector`)))
  ;[1 1 1] Initial step for first node of primary branch
  (for _array_element (`self.PrimarySplineSeeds`)
    (set `local.Primary BSeed` (`KismetMathLibrary.MakeRandomStream` _array_element))
    (set `local.Last Location` (`self.K2_GetActorLocation`))
    (set `self.ForwardVec` (`KismetMathLibrary.GreaterGreater_VectorRotator` (`self.GetActorForwardVector`) (`KismetMathLibrary.MakeRotator` 0.0 0.0 (`KismetMathLibrary.RandomFloatInRangeFromStream` (`local.Primary BSeed`) (`self.Min Origin Offset`) (`self.Max Origin Offset`)))))
    (bind _returnvalue_2 (`AddComponent|NODE_AddSplineComponent-3`))
    (bind _output_get (set `local.PBranch` _returnvalue_2))
    (`SplineComponent.RemoveSplinePoint` _output_get 1 true) ; Splines are initiated with two points, remove the 2nd one
    ;[1 1 1] Create nodes for branch, then add spline to array of primary branch splines
    (for _ (range 2 (+ (`self.Branch Nodes`) 1))
      (set `self.ForwardVec` _returnvalue)
      (bind _output_get_2 (set `local.Last Location` (+ (`local.Last Location`) (* _returnvalue (`KismetMathLibrary.RandomFloatInRangeFromStream` (`local.Primary BSeed`) (`self.Min Dist Between Nodes`) (`self.Max Dist Between Nodes`))))))
      (`SplineComponent.AddSplinePoint` _pbranch _output_get_2 "World" true))
    (`SplineComponent.UpdateSpline` _pbranch)
    (`KismetArrayLibrary.Array_Add` (`self.PrimarySplines`) (`local.PBranch`))))

(fn `MakeSecondaryBranches`
  (locals (`sub-branch` :type "SplineComponent Object Reference") (`Last Location` :type "Vector Structure"))
  (bind _sub_branch (`local.sub-branch`))
  (bind (_returnvalue_location _returnvalue_rotation) (`KismetMathLibrary.BreakTransform` (`SplineComponent.GetTransformAtSplinePoint` _sub_branch (`SplineComponent.GetNumberOfSplinePoints` _sub_branch) "World" false)))
  ;[1 1 1] Create first node thats on top of a random primary branch node
  (for (_array_element _array_index) (`self.PrimarySplines`)
    (for _array_element_2 (`self.SecondarySplineSeeds`)
      (set `self.SubStream` (`KismetMathLibrary.MakeRandomStream` (+ _array_element_2 (`|GetArrayItem` (`self.PrimarySplineSeeds`) _array_index))))
      (bind _returnvalue (`AddComponent|NODE_AddSplineComponent-1`))
      (bind _returnvalue_location_2 (`KismetMathLibrary.BreakTransform` (`SplineComponent.GetTransformAtSplinePoint` _array_element (`KismetMathLibrary.RandomIntegerFromStream` (`self.SubStream`) (`SplineComponent.GetNumberOfSplinePoints` _array_element)) "World" false)))
      (`SplineComponent.SetLocationAtSplinePoint` _returnvalue 0 _returnvalue_location_2 "World" true)
      (bind _output_get (set `local.sub-branch` _returnvalue))
      (`SplineComponent.RemoveSplinePoint` _output_get 1 true)
      ;[1 1 1] Generate nodes in spline, then add to array of secondary splines
      (set `local.Last Location` _returnvalue_location)
      (for _ (range 1 (+ (`self.Secondary Nodes`) 1))
        (bind _output_get_2 (set `local.Last Location` (+ (`local.Last Location`) (* (`KismetMathLibrary.GreaterGreater_VectorRotator` (`KismetMathLibrary.GetForwardVector` _returnvalue_rotation) (`KismetMathLibrary.MakeRotator` 0.0 0.0 (`KismetMathLibrary.RandomFloatInRangeFromStream` (`self.SubStream`) (`self.Min Secondary Degree Offset`) (`self.Max Secondary Degree Offset`)))) (`KismetMathLibrary.RandomFloatInRangeFromStream` (`self.SubStream`) (`self.Min Secondary Dist between Nodes`) (`self.Max Secondary Dist between Nodes`))))))
        (`SplineComponent.AddSplinePoint` (`local.sub-branch`) _output_get_2 "World" true))
      (`SplineComponent.UpdateSpline` (`local.sub-branch`))
      (`KismetArrayLibrary.Array_Add` (`self.SecondarySplines`) (`local.sub-branch`)))))

(fn `ProjectBranches`
  (locals (`Spline to Project` :type "SplineComponent Object Reference"))
  ;[1 1 1] Project Primary and Secondary splines
  (for _array_element (`self.PrimarySplines`)
    (set `local.Spline to Project` _array_element)
    (for _index (range (+ (`SplineComponent.GetNumberOfSplinePoints` (`local.Spline to Project`)) 1)) :!label _label
      (bind _returnvalue_location (`KismetMathLibrary.BreakTransform` (`SplineComponent.GetTransformAtSplinePoint` (`local.Spline to Project`) _index "World" false)))
      (bind (_outhit _returnvalue) (`KismetSystemLibrary.LineTraceSingle` :`Start` _returnvalue_location :`End` (+ _returnvalue_location (* (`self.GetActorUpVector`) -5000.0)) :`TraceChannel` "TraceTypeQuery1" :`DrawTime` 10.0))
      (if _returnvalue
        (`SplineComponent.SetLocationAtSplinePoint` (`local.Spline to Project`) _index (`.ImpactPoint` (`GameplayStatics.BreakHitResult` _outhit)) "World" true) ; Set intersection location as new location for node
        (else
          (`SplineComponent.RemoveSplinePoint` (`local.Spline to Project`) _index true) ; Remove points that dont intersect
        ))))
  (for _array_element_2 (`self.SecondarySplines`)
    (set `local.Spline to Project` _array_element_2)
    (goto _label))
  ;[1 1 1] Project leaves
  (for (_array_element_3 _array_index) (`self.LeafPos`)
    (bind _outhit_2 (`KismetSystemLibrary.LineTraceSingle` :`Start` _array_element_3 :`End` (+ _array_element_3 (* (`self.GetActorUpVector`) -5000.0)) :`TraceChannel` "TraceTypeQuery1" :`DrawTime` 10.0))
    (if true
      (`KismetArrayLibrary.Array_Set` (`self.LeafPos`) _array_index (`.ImpactPoint` (`GameplayStatics.BreakHitResult` _outhit_2)))
      (else
        (`KismetArrayLibrary.Array_Remove` (`self.LeafPos`) _array_index)))))

(fn `UserConstructionScript`
  (locals (ActorRotation :type "Rotator Structure" :default (struct)))
  ;[1 1 1] set actor rotation to 0,0,0 during generation of splines, rotation reset after splines are made
  (set `local.ActorRotation` (`self.K2_GetActorRotation` self))
  (`self.K2_SetActorRotation` (struct))
  ;[1 1 1] If an index in these arrays is equal to 0, give it a random seed
  (for (_array_element _array_index) (`self.PrimarySplineSeeds`)
    (if (== _array_element 0)
      (`KismetArrayLibrary.Array_Set` (`self.PrimarySplineSeeds`) _array_index (`KismetMathLibrary.RandomInteger` 100000))))
  (for (_array_element_2 _array_index_2) (`self.SecondarySplineSeeds`)
    (if (== _array_element_2 0)
      (`KismetArrayLibrary.Array_Set` (`self.SecondarySplineSeeds`) _array_index_2 (`KismetMathLibrary.RandomInteger` 100000))))
  (for (_array_element_3 _array_index_3) (`self.LeafSeeds`)
    (if (== _array_element_3 0)
      (`KismetArrayLibrary.Array_Set` (`self.LeafSeeds`) _array_index_3 (`KismetMathLibrary.RandomInteger` 100000))))
  ;[1 1 1] Generate splines, then rotate actor
  (`self.MakePrimaryBranches`)
  (`self.MakeSecondaryBranches`)
  (`self.K2_SetActorRotation` (`local.ActorRotation`))
  ;[1 1 1] Generate locations for leaves
  (`self.GetNodeLocations`)
  (`self.GenerateLeafLoc`)
  ;[1 1 1] Check if splines should be projected then rendered
  (if (`self.Project`)
    (`self.ProjectBranches`))
  (if (`self.Render`)
    (for _array_element_4 (`self.PrimarySplines`)
      (`self.CreateMesh` _array_element_4)
      (`ActorComponent.K2_DestroyComponent` _array_element_4))
    (for _array_element_5 (`self.SecondarySplines`)
      (`self.CreateMesh` _array_element_5)
      (`ActorComponent.K2_DestroyComponent` _array_element_5))))