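; Chargeable fireball projectile that damages BPI_Enemy actors on impact and can leave a temporary burning area.
; SetVariables derives damage, radii and scale from FireballDA, blended by charge.
; On hit, it applies sphere-trace damage, then traces down for floor, where three chained timelines spread, hold and converge a damage sphere before destroying the actor.
; One DoOnce gates burn damage, so one enemy takes damage per cooldown.
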(event `self.ReceiveBeginPlay`
  (bind _fireballda (`self.fireballDA`))
  (bind _fireballda_2 (`self.fireballDA`))
  (bind _fireballda_3 (`self.fireballDA`))
  (bind _fireballda_4 (`self.fireballDA`))
  (bind _fireballda_5 (`self.fireballDA`))
  (bind _fireballda_6 (`self.fireballDA`))
  (bind _fireballda_7 (`self.fireballDA`))
  (bind _returnvalue (/ (`self.sizeFactor`) 10.0))
  ;[1 1 1] Begin Play
  (`parent.ReceiveBeginPlay`)
  (set `MovementComponent.Velocity` (`self.newVelocity`) (`self.ProjectileMovement`))
  (set `ProjectileMovementComponent.ProjectileGravityScale` (`self.newProjectileGravityScale`) (`self.ProjectileMovement`))
  (if (`self.isCharged`)
    (set `self.firstAoeRadius` (`/Game/_Manager/InGame/DataAsset/BP/BP_Fireball_DA.chargedFirstAoeRadius` (`self.fireballDA`)))
    (set `self.secondAoeRadius` (`/Game/_Manager/InGame/DataAsset/BP/BP_Fireball_DA.chargedSecondAoeRadius` (`self.fireballDA`)))
    (set `self.detectFloorDistance` (`/Game/_Manager/InGame/DataAsset/BP/BP_Fireball_DA.chargedDetectFloorDistance` (`self.fireballDA`)))
    (set `self.damages` (`/Game/_Manager/InGame/DataAsset/BP/BP_Fireball_DA.chargedDamages` (`self.fireballDA`)))
    (set `self.sizeFactor` (`/Game/_Manager/InGame/DataAsset/BP/BP_Fireball_DA.chargedSphereSize` (`self.fireballDA`)))
    (set `self.secondAoeDamages` (`/Game/_Manager/InGame/DataAsset/BP/BP_Fireball_DA.chargedSecondAoeDamages` (`self.fireballDA`)))
    (set `self.cooldownSecondAoe` (`/Game/_Manager/InGame/DataAsset/BP/BP_Fireball_DA.chargedSecondAoeCooldown` (`self.fireballDA`)))
    (else
      (set `self.firstAoeRadius` (`KismetMathLibrary.Lerp` (`/Game/_Manager/InGame/DataAsset/BP/BP_Fireball_DA.normalFirstAoeRadius` _fireballda) (`/Game/_Manager/InGame/DataAsset/BP/BP_Fireball_DA.chargedFirstAoeRadius` _fireballda) (`self.chargeAlpha`)))
      (set `self.secondAoeRadius` (`KismetMathLibrary.Lerp` (`/Game/_Manager/InGame/DataAsset/BP/BP_Fireball_DA.normalSecondAoeRadius` _fireballda_2) (`/Game/_Manager/InGame/DataAsset/BP/BP_Fireball_DA.chargedSecondAoeRadius` _fireballda_2) (`self.chargeAlpha`)))
      (set `self.detectFloorDistance` (`KismetMathLibrary.Lerp` (`/Game/_Manager/InGame/DataAsset/BP/BP_Fireball_DA.normalDetectFloorDistance` _fireballda_3) (`/Game/_Manager/InGame/DataAsset/BP/BP_Fireball_DA.chargedDetectFloorDistance` _fireballda_3) (`self.chargeAlpha`)))
      (set `self.damages` (`KismetMathLibrary.Lerp` (`/Game/_Manager/InGame/DataAsset/BP/BP_Fireball_DA.normalDamages` _fireballda_4) (`/Game/_Manager/InGame/DataAsset/BP/BP_Fireball_DA.chargedDamages` _fireballda_4) (`self.chargeAlpha`)))
      (set `self.sizeFactor` (`KismetMathLibrary.Lerp` (`/Game/_Manager/InGame/DataAsset/BP/BP_Fireball_DA.normalSphereSize` _fireballda_5) (`/Game/_Manager/InGame/DataAsset/BP/BP_Fireball_DA.chargedSphereSize` _fireballda_5) (`self.chargeAlpha`)))
      (set `self.secondAoeDamages` (`KismetMathLibrary.Lerp` (`/Game/_Manager/InGame/DataAsset/BP/BP_Fireball_DA.normalSecondAoeDamages` _fireballda_6) (`/Game/_Manager/InGame/DataAsset/BP/BP_Fireball_DA.chargedSecondAoeDamages` _fireballda_6) (`self.chargeAlpha`)))
      (set `self.cooldownSecondAoe` (`KismetMathLibrary.Lerp` (`/Game/_Manager/InGame/DataAsset/BP/BP_Fireball_DA.normalSecondAoeCooldown` _fireballda_7) (`/Game/_Manager/InGame/DataAsset/BP/BP_Fireball_DA.chargedSecondAoeCooldown` _fireballda_7) (`self.chargeAlpha`)))))
  (`self.SetActorScale3D` (`KismetMathLibrary.MakeVector` _returnvalue _returnvalue _returnvalue))
  (`TimelineComponent.SetPlayRate` (`self.FireBeginning`) (/ 1.0 (`/Game/_Manager/InGame/DataAsset/BP/BP_Fireball_DA.fireSpreadDuration` (`self.fireballDA`))))
  (`TimelineComponent.SetPlayRate` (`self.FireMiddle`) (/ 1.0 (`/Game/_Manager/InGame/DataAsset/BP/BP_Fireball_DA.fireStayDuration` (`self.fireballDA`))))
  (`TimelineComponent.SetPlayRate` (`self.FIreEnd`) (/ 1.0 (`/Game/_Manager/InGame/DataAsset/BP/BP_Fireball_DA.fireConvergeDuration` (`self.fireballDA`)))))

(event `SecondDamagesSphere`
  (params (Start :type "Vector Structure") (End :type "Vector Structure") (Radius :type "Float (single-precision)"))
  ;[1 1 1] Make damages
  (bind _outhits (`KismetSystemLibrary.SphereTraceMulti` :`Start` Start :`End` End :`Radius` Radius :`TraceChannel` "TraceTypeQuery3" :`DrawDebugType` "ForOneFrame"))
  (for _array_element _outhits
    (bind (_bblockinghit _binitialoverlap _time _distance _location _impactpoint _normal _impactnormal _physmat _hitactor) (`GameplayStatics.BreakHitResult` _array_element))
    (if (`KismetSystemLibrary.DoesImplementInterface` _hitactor "/Game/Blueprints/BPI/Enemies/BPI_Enemy.BPI_Enemy_C")
      (`/Engine/EditorBlueprintResources/StandardMacros.DoOnce` false :!label _label
        (:`Completed`
          (`GameplayStatics.ApplyDamage` _hitactor (`self.secondAoeDamages`))
          (`KismetSystemLibrary.Delay` (`self.cooldownSecondAoe`))
          (`self.ResetApplyDamages`))))))

(event `self.StaticMesh.OnComponentHit`
  (params (HitComponent :type "PrimitiveComponent Object Reference") (OtherActor :type "Actor Object Reference") (OtherComp :type "PrimitiveComponent Object Reference") (NormalImpulse :type "Vector Structure") (Hit :type "HitResult Structure (by ref)"))
  (bind (_bblockinghit _binitialoverlap _time _distance _location) (`GameplayStatics.BreakHitResult` Hit))
  (bind _staticmesh (`self.StaticMesh`))
  ;[1 1 1] Make damages
  (`SceneComponent.SetHiddenInGame` _staticmesh true false)
  (`PrimitiveComponent.SetCollisionEnabled` _staticmesh "NoCollision")
  (bind _outhits (`KismetSystemLibrary.SphereTraceMulti` :`Start` _location :`End` _location :`Radius` (`self.firstAoeRadius`) :`TraceChannel` "TraceTypeQuery3" :`DrawDebugType` "ForDuration"))
  (for _array_element _outhits
    (bind (_bblockinghit_2 _binitialoverlap_2 _time_2 _distance_2 _location_2 _impactpoint _normal _impactnormal _physmat _hitactor) (`GameplayStatics.BreakHitResult` _array_element))
    (if (`KismetSystemLibrary.DoesImplementInterface` _hitactor "/Game/Blueprints/BPI/Enemies/BPI_Enemy.BPI_Enemy_C")
      (`GameplayStatics.ApplyDamage` _hitactor (`self.damages`))))
  (bind (_outhit _returnvalue) (`KismetSystemLibrary.LineTraceSingle` :`Start` _location :`End` (+ _location (* (`KismetMathLibrary.Vector_Down`) (`self.detectFloorDistance`))) :`TraceChannel` "TraceTypeQuery1" :`DrawDebugType` "Persistent"))
  (if _returnvalue
    (bind (_direction _alpha) (`Timeline|FireBeginning`)
      (:`Update`
        (bind (_bblockinghit_3 _binitialoverlap_3 _time_3 _distance_3 _location_3 _impactpoint_2) (`GameplayStatics.BreakHitResult` _outhit))
        (`self.SecondDamagesSphere` _impactpoint_2 _impactpoint_2 (`KismetMathLibrary.Lerp` 0.0 (`self.secondAoeRadius`) _alpha)))
      (:`Finished`
        (`Timeline|FireMiddle`
          (:`Update`
            (`self.SecondDamagesSphere` _impactpoint_2 _impactpoint_2 (`self.secondAoeRadius`)))
          (:`Finished`
            (bind (_direction_2 _alpha_2) (`Timeline|FIreEnd`)
              (:`Update`
                (`self.SecondDamagesSphere` _impactpoint_2 _impactpoint_2 (`KismetMathLibrary.Lerp` 0.0 (`self.secondAoeRadius`) _alpha_2)))
              (:`Finished`
                (`KismetSystemLibrary.DelayUntilNextTick`)
                (`self.K2_DestroyActor`)))))))))

(event `ResetApplyDamages`
  ;[1 1 1] Make damages
  (goto _label :!via `Reset`))

(fn `UserConstructionScript`
  (`parent.UserConstructionScript`))