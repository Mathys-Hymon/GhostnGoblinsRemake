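; BP_Dagger is a thrown dagger projectile that flies at a configurable speed and sticks into whatever it hits.
; On hit it removes its projectile movement, attaches to the struck actor in world space and turns off mesh collision.
; Damage is applied only to actors implementing BPI_Enemy.
; A delay started at BeginPlay destroys the dagger after a set lifetime, whether or not it has hit.
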(event `self.ReceiveBeginPlay`
  (bind _projectilemovement (`self.ProjectileMovement`))
  (bind _speed (`self.speed`))
  (`parent.ReceiveBeginPlay`)
  (set `ProjectileMovementComponent.InitialSpeed` _speed _projectilemovement)
  (set `ProjectileMovementComponent.MaxSpeed` _speed _projectilemovement)
  (`KismetSystemLibrary.Delay` (`self.timeBeforeDelete`))
  (`self.K2_DestroyActor`))

(event `self.StaticMesh.OnComponentHit`
  (params (HitComponent :type "PrimitiveComponent Object Reference") (OtherActor :type "Actor Object Reference") (OtherComp :type "PrimitiveComponent Object Reference") (NormalImpulse :type "Vector Structure") (Hit :type "HitResult Structure (by ref)"))
  (bind (_bblockinghit _binitialoverlap _time _distance _location _impactpoint _normal _impactnormal _physmat _hitactor) (`GameplayStatics.BreakHitResult` Hit))
  (`ActorComponent.K2_DestroyComponent` (`self.ProjectileMovement`))
  (`self.K2_AttachToActor` OtherActor "None" "KeepWorld" "KeepWorld" "KeepWorld")
  (`PrimitiveComponent.SetCollisionEnabled` (`self.StaticMesh`) "NoCollision")
  (if (`KismetSystemLibrary.DoesImplementInterface` _hitactor "/Game/Blueprints/BPI/Enemies/BPI_Enemy.BPI_Enemy_C")
    (`GameplayStatics.ApplyDamage` _hitactor (`self.damages`))))

(fn `UserConstructionScript`
  (`parent.UserConstructionScript`))