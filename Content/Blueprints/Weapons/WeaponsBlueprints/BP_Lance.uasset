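; Lance projectile that damages enemies, can pierce a set number of targets, then embeds in what it hits.
; LanceDA supplies speed, damages, range and lifetime, while a non-zero LancePierce enables charged FX on spawn.
; Box overlaps spend pierces or attach the lance to the target, while mesh hits on non-enemies stop it and nudge it inward.
; Tick destroys it beyond range using squared distance until stuck, and a timed delay also removes it.
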(event `self.ReceiveBeginPlay`
  (bind _projectilemovement (`self.ProjectileMovement`))
  (bind _projectilespeed (`/Game/_Manager/InGame/DataAsset/BP/Weapons/BP_Lance_DA.projectileSpeed` (`self.lanceDA`)))
  ;[1 1 1] Begin play
  (`parent.ReceiveBeginPlay`)
  (if (> (`self.lancePierce`) 0.0)
    (`NiagaraComponent.SetAsset` (`self.Niagara`) (`self.chargedFX`) true))
  (set `ProjectileMovementComponent.InitialSpeed` _projectilespeed _projectilemovement)
  (set `ProjectileMovementComponent.MaxSpeed` _projectilespeed _projectilemovement)
  (set `self.spawnPosition` (`self.K2_GetActorLocation`))
  (`KismetSystemLibrary.Delay` (`/Game/_Manager/InGame/DataAsset/BP/Weapons/BP_Lance_DA.timeBeforeDelete` (`self.lanceDA`)))
  (`self.K2_DestroyActor`))

(event `self.Box.OnComponentBeginOverlap`
  (params (OverlappedComponent :type "PrimitiveComponent Object Reference") (OtherActor :type "Actor Object Reference") (OtherComp :type "PrimitiveComponent Object Reference") (OtherBodyIndex :type Integer) (bFromSweep :type Boolean) (SweepResult :type "HitResult Structure (by ref)"))
  (bind _staticmesh (`self.StaticMesh`))
  (`KismetSystemLibrary.PrintString` "Hit")
  ;[1 1 1] Can still pierce more enemies
  (if (!= 0.0 (`self.lancePierce`))
    (set `self.lancePierce` (- (`self.lancePierce`) 1.0))
    (if (`KismetSystemLibrary.DoesImplementInterface` OtherActor "/Game/Blueprints/BPI/Enemies/BPI_Enemy.BPI_Enemy_C")
      (`GameplayStatics.ApplyDamage` OtherActor (`/Game/_Manager/InGame/DataAsset/BP/Weapons/BP_Lance_DA.pierceDamages` (`self.lanceDA`))))
    (else
      ;[1 1 1] Can No longer pierce
      (`/Engine/EditorBlueprintResources/StandardMacros.IsValid` (`self.Box`)
        (:`Is Valid`
          (`/Engine/EditorBlueprintResources/StandardMacros.IsValid` (`self.ProjectileMovement`)
            (:`Is Valid`
              (`ActorComponent.K2_DestroyComponent` (`self.Niagara`))
              (`ActorComponent.K2_DestroyComponent` (`self.Box`))
              (`ActorComponent.K2_DestroyComponent` (`self.ProjectileMovement`))
              (`self.K2_AttachToActor` OtherActor "None" "KeepWorld" "KeepWorld" "KeepWorld")
              (set `self.shouldCheckDistance` false)
              (if (`KismetSystemLibrary.DoesImplementInterface` OtherActor "/Game/Blueprints/BPI/Enemies/BPI_Enemy.BPI_Enemy_C")
                (`GameplayStatics.ApplyDamage` OtherActor (`/Game/_Manager/InGame/DataAsset/BP/Weapons/BP_Lance_DA.damages` (`self.lanceDA`)))
                (`/Engine/EditorBlueprintResources/StandardMacros.IsValid` _staticmesh
                  (:`Is Valid`
                    (`PrimitiveComponent.SetCollisionEnabled` _staticmesh "NoCollision"))))
              (`self.K2_SetActorLocation` (+ (`self.K2_GetActorLocation` self) (* (`self.GetActorForwardVector` self) 20.0))))))))))

(event `self.StaticMesh.OnComponentHit`
  (params (HitComponent :type "PrimitiveComponent Object Reference") (OtherActor :type "Actor Object Reference") (OtherComp :type "PrimitiveComponent Object Reference") (NormalImpulse :type "Vector Structure") (Hit :type "HitResult Structure (by ref)"))
  ;[1 1 1] Collide with static mesh
  (if (not (`KismetSystemLibrary.DoesImplementInterface` OtherActor "/Game/Blueprints/BPI/Enemies/BPI_Enemy.BPI_Enemy_C"))
    (`/Engine/EditorBlueprintResources/StandardMacros.IsValid` (`self.Box`)
      (:`Is Valid`
        (`/Engine/EditorBlueprintResources/StandardMacros.IsValid` (`self.ProjectileMovement`)
          (:`Is Valid`
            (`ActorComponent.K2_DestroyComponent` (`self.Niagara`))
            (`ActorComponent.K2_DestroyComponent` (`self.Box`))
            (`ActorComponent.K2_DestroyComponent` (`self.ProjectileMovement`))
            (`PrimitiveComponent.SetCollisionEnabled` (`self.StaticMesh`) "NoCollision")
            (set `self.shouldCheckDistance` false)
            (`self.K2_SetActorLocation` (+ (`self.K2_GetActorLocation` self) (* (`self.GetActorForwardVector` self) 50.0)))))))))

(event `self.ReceiveTick`
  (params (DeltaSeconds :type "Float (single-precision)"))
  ;[1 1 1] Distance Check
  (`/Engine/EditorBlueprintResources/StandardMacros.IsValid` self
    (:`Is Valid`
      (if (`self.shouldCheckDistance`)
        (if (>= (`KismetMathLibrary.Vector_DistanceSquared` (`self.spawnPosition`) (`self.K2_GetActorLocation`)) (`KismetMathLibrary.Square` (`/Game/_Manager/InGame/DataAsset/BP/Weapons/BP_Lance_DA.range` (`self.lanceDA`))))
          (`self.K2_DestroyActor`))))))

(fn `UserConstructionScript`
  (`parent.UserConstructionScript`))