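; Player weapon component that fires lance, fireball or dagger-fan attacks, either instantly or as aimed, held shots with cooldowns.
; Hold time scales lance pierce, fireball charge and dagger count and spread, with crosshair, rumble and sound feedback.
; Camera traces set the aim and fireball arc velocity.
; While aiming, the fireball previews its predicted path with spline meshes and an impact marker.
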(event `FirstShoot`
  (bind _returnvalue (`GameplayStatics.GetPlayerCharacter` 0))
  (bind _endprevisualizationref (`self.endPrevisualizationRef`))
  (bind _daggersda (`self.daggersDA`))
  (bind _daggersda_2 (`self.daggersDA`))
  (bind _returnvalue_2 (`PlayerController.GetHUD` (`GameplayStatics.GetPlayerController` 0)))
  (bind _returnvalue_3 (+ (`Actor.K2_GetActorLocation` (`GameplayStatics.GetPlayerPawn` 0)) (0.0 0.0 60.0)))
  (bind _rot (`self.FindTargetRot` _returnvalue_3))
  (bind _returnvalue_4 (`SceneComponent.K2_GetComponentLocation` (`SceneComponent.GetChildComponent` (`Character.Mesh` (`GameplayStatics.GetPlayerCharacter` 0)) 1)))
  ;[0 0 0] New shoot system
  (`/Engine/EditorBlueprintResources/StandardMacros.DoOnce` false :!label _label
    (:`Completed`
      (message `/Game/Blueprints/BPI/PlayerController/BPI_PlayerController.PlayGamepadRumble` (`GameplayStatics.GetPlayerController` 0) (select `/Game/Blueprints/Enums/Enum_WeaponType` (`self.currentWeapon`) :`NewEnumerator0` "/Game/Haptics/FFE_LanceThrow.FFE_LanceThrow" :`NewEnumerator1` "/Game/Haptics/FFE_LanceThrow.FFE_LanceThrow" :`NewEnumerator2` "/Game/Haptics/FFE_DaggersThrow.FFE_DaggersThrow" :!type "ForceFeedbackEffect Object Reference") false)
      ;;[0.2067 1 0.6933] Keep hold attack
      (set `self.shootWithoutAiming?` true)
      (set `self.holdTime` 0.0)
      ;[1 1 1] Spawn weapon
      (`|ExecutionSequence` :!label _label_2
        (:`then_0`
          (`GameplayStatics.PlaySound2D` (`KismetArrayLibrary.Array_Random` (`/Game/_Manager/InGame/DataAsset/BP/SFX/BP_SFX_DA.throw` (`self.sfxDataAsset`))) 1.0 1.0 0.0 null null)
          (set `self.aiming?` false)
          (set `self.canShoot` false)
          (`|ExecutionSequence`
            (:`then_0`
              (`self.ShootEvent`)
              (switch `/Game/Blueprints/Enums/Enum_WeaponType` (`self.currentWeapon`) ; Which weapon to spawn ?
                (:`NewEnumerator0`
                  ;[1 1 1] Shoot Lance - The more you charge your shot the more enemies you can pierce through
                  (if (>= (`self.holdTime`) (`/Game/_Manager/InGame/DataAsset/BP/Weapons/BP_Lance_DA.chargeTime` (`self.lanceDA`)))
                    (set `self.lancePierce` (`/Game/_Manager/InGame/DataAsset/BP/Weapons/BP_Lance_DA.maxPierce` (`self.lanceDA`)))
                    (else
                      (set `self.lancePierce` (`KismetMathLibrary.Conv_IntToDouble` (`KismetMathLibrary.FTrunc` (`KismetMathLibrary.Lerp` 0.0 (`/Game/_Manager/InGame/DataAsset/BP/Weapons/BP_Lance_DA.maxPierce` (`self.lanceDA`)) (/ (`self.holdTime`) (`/Game/_Manager/InGame/DataAsset/BP/Weapons/BP_Lance_DA.chargeTime` (`self.lanceDA`)))))))))
                  (`|SpawnActorFromClass` "/Game/Blueprints/Weapons/WeaponsBlueprints/BP_Lance.BP_Lance_C" (`KismetMathLibrary.MakeTransform` _returnvalue_4 (`self.FindTargetRot` _returnvalue_4)) "AlwaysSpawn" "MultiplyWithRoot" null (`self.lancePierce`) null))
                (:`NewEnumerator1`
                  (`|SpawnActorFromClass` "/Game/Blueprints/Weapons/WeaponsBlueprints/BP_Fireball.BP_Fireball_C" (`KismetMathLibrary.MakeTransform` (`SceneComponent.K2_GetComponentLocation` (`SceneComponent.GetChildComponent` (`Character.Mesh` _returnvalue) 1)) (`Actor.K2_GetActorRotation` _returnvalue)) "AlwaysSpawn" "MultiplyWithRoot" null (`self.weaponVelocity`) (`/Game/_Manager/InGame/DataAsset/BP/Weapons/BP_Fireball_DA.gravityScale` (`self.fireballDA`)) (>= (`self.holdTime`) (`/Game/_Manager/InGame/DataAsset/BP/Weapons/BP_Fireball_DA.chargeTime` (`self.fireballDA`))) (/ (`self.holdTime`) (`/Game/_Manager/InGame/DataAsset/BP/Weapons/BP_Fireball_DA.chargeTime` (`self.fireballDA`))) null)
                  ;[1 1 1] Clear previsualization spline
                  (set `self.previsualization?` false)
                  (`/Game/Blueprints/Weapons/Previsualization/BP_Previsualize.ClearSpline` (`self.previsuaizationRef`))
                  (`/Engine/EditorBlueprintResources/StandardMacros.IsValid` _endprevisualizationref
                    (:`Is Valid`
                      (`Actor.K2_DestroyActor` _endprevisualizationref)
                      (`self.ResetSpawnPrevis`))))
                (:`NewEnumerator2`
                  ;[1 1 1] Daggers logic
                  (if (>= (`self.holdTime`) (`/Game/_Manager/InGame/DataAsset/BP/Weapons/BP_Daggers_DA.chargeTime` (`self.daggersDA`)))
                    (set `self.actualNbDagger` (- (`/Game/_Manager/InGame/DataAsset/BP/Weapons/BP_Daggers_DA.maxDaggerAmount` (`self.daggersDA`)) 1))
                    (set `self.DaggerAngle` (`/Game/_Manager/InGame/DataAsset/BP/Weapons/BP_Daggers_DA.maxDaggerConeAngle` (`self.daggersDA`)))
                    (else
                      (set `self.actualNbDagger` (- (`KismetMathLibrary.FTrunc` (`KismetMathLibrary.Lerp` (`KismetMathLibrary.Conv_IntToDouble` (`/Game/_Manager/InGame/DataAsset/BP/Weapons/BP_Daggers_DA.minDaggerAmount` _daggersda)) (`KismetMathLibrary.Conv_IntToDouble` (`/Game/_Manager/InGame/DataAsset/BP/Weapons/BP_Daggers_DA.maxDaggerAmount` _daggersda)) (/ (`self.holdTime`) (`/Game/_Manager/InGame/DataAsset/BP/Weapons/BP_Daggers_DA.chargeTime` (`self.daggersDA`))))) 1))
                      (set `self.DaggerAngle` (`KismetMathLibrary.Lerp` (`/Game/_Manager/InGame/DataAsset/BP/Weapons/BP_Daggers_DA.minDaggerConeAngle` _daggersda_2) (`/Game/_Manager/InGame/DataAsset/BP/Weapons/BP_Daggers_DA.maxDaggerConeAngle` _daggersda_2) (/ (`self.holdTime`) (`/Game/_Manager/InGame/DataAsset/BP/Weapons/BP_Daggers_DA.chargeTime` (`self.daggersDA`)))))))
                  (for _index (range (+ (`self.actualNbDagger`) 1))
                    (`|SpawnActorFromClass` "/Game/Blueprints/Weapons/WeaponsBlueprints/BP_Dagger.BP_Dagger_C" (`KismetMathLibrary.MakeTransform` _returnvalue_3 (`KismetMathLibrary.MakeRotator` (.roll _rot) (.pitch _rot) (+ (* _index (/ (`self.DaggerAngle`) (`self.actualNbDagger`))) (- (.yaw _rot) (/ (`self.DaggerAngle`) 2.0))))) "AlwaysSpawn" "MultiplyWithRoot" null (> (`self.actualNbDagger`) (`self.minNbDagger`)) null)))))
            (:`then_1`
              (`KismetSystemLibrary.Delay` (select `/Game/Blueprints/Enums/Enum_WeaponType` (`self.currentWeapon`) :`NewEnumerator0` (`/Game/_Manager/InGame/DataAsset/BP/Weapons/BP_Lance_DA.cooldown` (`self.lanceDA`)) :`NewEnumerator1` (`/Game/_Manager/InGame/DataAsset/BP/Weapons/BP_Fireball_DA.cooldown` (`self.fireballDA`)) :`NewEnumerator2` (`/Game/_Manager/InGame/DataAsset/BP/Weapons/BP_Daggers_DA.cooldown` (`self.daggersDA`)) :!type "Float (single-precision)"))
              (set `self.canShoot` true))))
        (:`then_1`
          (if (> (`self.holdTime`) 0.1)
            (message `/Game/Blueprints/BPI/Player/BPI_HUD.ResetCrosshairAnimation` _returnvalue_2 (`self.currentWeapon`) 1.0)
            (else
              (message `/Game/Blueprints/BPI/Player/BPI_HUD.ResetCrosshairPosition` _returnvalue_2)))
          (`self.ResetPlayAnimationDO`))))))

(event `ShootAgain`
  ;[0 0 0] New shoot system
  (goto _label :!via `Reset`))

(event `/Game/Blueprints/BPI/Weapon/BPI_Weapons.Shoot`
  (params (holdTime :type "Float (double-precision)"))
  (bind _returnvalue (`GameplayStatics.GetPlayerController` 0))
  ;[1 1 1] Spawn weapon
  (`self.resetSFX`)
  (`self.ShootAgain`)
  (set `self.holdTime` holdTime)
  ;;[0 0 0] New shoot system
  (if (and (`self.canShoot`) (`self.aiming?`))
    (message `/Game/Blueprints/BPI/PlayerController/BPI_PlayerController.StopGamepadRumble` _returnvalue (select `/Game/Blueprints/Enums/Enum_WeaponType` (`self.currentWeapon`) :`NewEnumerator0` "/Game/Haptics/FFE_LanceCharge.FFE_LanceCharge" :`NewEnumerator1` "/Game/Haptics/FFE_FireballCharge.FFE_FireballCharge" :`NewEnumerator2` "/Game/Haptics/FFE_DaggersCharge.FFE_DaggersCharge" :!type "ForceFeedbackEffect Object Reference"))
    (message `/Game/Blueprints/BPI/PlayerController/BPI_PlayerController.StopGamepadRumble` _returnvalue "/Game/Haptics/FFE_WeaponsFullyChargedLoops.FFE_WeaponsFullyChargedLoops")
    (message `/Game/Blueprints/BPI/PlayerController/BPI_PlayerController.PlayGamepadRumble` _returnvalue (select `/Game/Blueprints/Enums/Enum_WeaponType` (`self.currentWeapon`) :`NewEnumerator0` "/Game/Haptics/FFE_LanceChargedThrow.FFE_LanceChargedThrow" :`NewEnumerator1` "/Game/Haptics/FFE_FireballChargedThrow.FFE_FireballChargedThrow" :`NewEnumerator2` "/Game/Haptics/FFE_DaggersChargedThrow.FFE_DaggersChargedThrow" :!type "ForceFeedbackEffect Object Reference") false)
    (goto _label_2)))

(event `self.ReceiveBeginPlay`
  ;[1 1 1] Begin Play
  (bind _returnvalue (`|SpawnActorFromClass` "/Game/Blueprints/Weapons/Previsualization/BP_Previsualize.BP_Previsualize_C" (`Actor.GetTransform` (`GameplayStatics.GetPlayerCharacter` 0)) "Undefined" "MultiplyWithRoot" null null))
  (set `self.previsuaizationRef` _returnvalue)
  (message `/Game/Blueprints/BPI/Player/BPI_HUD.ShowHideRegularCrosshair` (`PlayerController.GetHUD` (`GameplayStatics.GetPlayerController` 0)) false))

(event `ResetPlayAnimationDO`
  (bind _currentweapon (`self.currentWeapon`))
  (bind _returnvalue (`PlayerController.GetHUD` (`GameplayStatics.GetPlayerController` 0)))
  ;[1 1 1] Start shoot event
  (`|ExecutionSequence`
    (:`then_0`
      (goto _label_4 :!via `Reset`))
    (:`then_1`
      (goto _label_8 :!via `Reset`))))

(event `resetSFX`
  (bind _sfxdataasset (`self.sfxDataAsset`))
  ;[1 1 1] Start shoot event
  (goto _label_3 :!via `Reset`))

(event `/Game/Blueprints/BPI/Weapon/BPI_Weapons.StartShoot`
  (params (holdTime :type "Float (double-precision)") (aiming :type Boolean))
  (bind _sfxdataasset (`self.sfxDataAsset`))
  (bind _currentweapon (`self.currentWeapon`))
  (bind _returnvalue (`PlayerController.GetHUD` (`GameplayStatics.GetPlayerController` 0)))
  ;[1 1 1] Start shoot event
  (`|ExecutionSequence`
    (:`then_0`
      (`/Engine/EditorBlueprintResources/StandardMacros.DoOnce` false :!label _label_3
        (:`Completed`
          (`GameplayStatics.PlaySound2D` (`KismetArrayLibrary.Array_Random` (select `/Game/Blueprints/Enums/Enum_WeaponType` (`self.currentWeapon`) :`NewEnumerator0` (`/Game/_Manager/InGame/DataAsset/BP/SFX/BP_SFX_DA.chargingLance` _sfxdataasset) :`NewEnumerator1` (`/Game/_Manager/InGame/DataAsset/BP/SFX/BP_SFX_DA.chargingFireball` _sfxdataasset) :`NewEnumerator2` (`/Game/_Manager/InGame/DataAsset/BP/SFX/BP_SFX_DA.chargingDaggers` _sfxdataasset) :!type "Array of SoundBase Object Reference")) 1.0 1.0 0.0 null null))))
    (:`then_1`
      (set `self.aiming?` aiming)
      (if (`self.canShoot`)
        (set `self.stopAnimation?` (>= holdTime (select `/Game/Blueprints/Enums/Enum_WeaponType` (`self.currentWeapon`) :`NewEnumerator0` (- (`/Game/_Manager/InGame/DataAsset/BP/Weapons/BP_Lance_DA.chargeTime` (`self.lanceDA`)) 0.01) :`NewEnumerator2` (- (`/Game/_Manager/InGame/DataAsset/BP/Weapons/BP_Daggers_DA.chargeTime` (`self.daggersDA`)) 0.01))))
        (`|ExecutionSequence`
          (:`then_0`
            (if (`self.aiming?`)
              (`|ExecutionSequence`
                (:`then_0`
                  (`/Engine/EditorBlueprintResources/StandardMacros.DoOnce` false :!label _label_4
                    (:`Completed`
                      ;;[0.2067 1 0.6933] Keep hold attack
                      (set `self.shootWithoutAiming?` false)
                      (message `/Game/Blueprints/BPI/Player/BPI_HUD.ResetCrosshairPosition` _returnvalue)
                      (message `/Game/Blueprints/BPI/Player/BPI_HUD.PlayCrosshairAnimation` _returnvalue _currentweapon (select `/Game/Blueprints/Enums/Enum_WeaponType` _currentweapon :`NewEnumerator0` (`/Game/_Manager/InGame/DataAsset/BP/Weapons/BP_Lance_DA.chargeTime` (`self.lanceDA`)) :`NewEnumerator2` (`/Game/_Manager/InGame/DataAsset/BP/Weapons/BP_Daggers_DA.chargeTime` (`self.daggersDA`))))
                      (message `/Game/Blueprints/BPI/PlayerController/BPI_PlayerController.PlayGamepadRumble` (`GameplayStatics.GetPlayerController` 0) (select `/Game/Blueprints/Enums/Enum_WeaponType` (`self.currentWeapon`) :`NewEnumerator0` "/Game/Haptics/FFE_LanceCharge.FFE_LanceCharge" :`NewEnumerator1` "/Game/Haptics/FFE_FireballCharge.FFE_FireballCharge" :`NewEnumerator2` "/Game/Haptics/FFE_DaggersCharge.FFE_DaggersCharge" :!type "ForceFeedbackEffect Object Reference") false)
                      (if (`self.stopAnimation?`)
                        (message `/Game/Blueprints/BPI/Player/BPI_HUD.StopCrosshairAnimation` (`PlayerController.GetHUD` (`GameplayStatics.GetPlayerController` 0)) (`self.currentWeapon`))))))
                (:`then_1`
                  (switch `/Game/Blueprints/Enums/Enum_WeaponType` (`self.currentWeapon`) :!label _label_5
                    (:`NewEnumerator1`
                      ;;[0 0 0] Fireball preview only aiming
                      (if (`self.aiming?`)
                        (`|ExecutionSequence`
                          (:`then_0`
                            (`/Engine/EditorBlueprintResources/StandardMacros.DoOnce` false :!label _label_6
                              (:`Completed`
                                (bind _returnvalue_2 (`|SpawnActorFromClass` "/Game/Blueprints/Weapons/Previsualization/BP_EndOfPreVisualization.BP_EndOfPreVisualization_C" (`KismetMathLibrary.MakeTransform` (0.0 0.0 0.0)) "Undefined" "MultiplyWithRoot" null null))
                                (set `self.endPrevisualizationRef` _returnvalue_2))))
                          (:`then_1`
                            (`self.StartPrevisualization`)
                            (set `self.weaponVelocity` (`self.CalculBombeVelocity`) :!label _label_7)))
                        (else
                          (goto _label_7)))))))
              (else
                (set `self.weaponVelocity` (`self.CalculBombeVelocity`))
                (`self.FirstShoot`)
                (goto _label_5))))
          (:`then_1`
            (if (> holdTime (+ (select `/Game/Blueprints/Enums/Enum_WeaponType` (`self.currentWeapon`) :`NewEnumerator0` (`/Game/_Manager/InGame/DataAsset/BP/Weapons/BP_Lance_DA.chargeTime` (`self.lanceDA`)) :`NewEnumerator1` (`/Game/_Manager/InGame/DataAsset/BP/Weapons/BP_Fireball_DA.chargeTime` (`self.fireballDA`)) :`NewEnumerator2` (`/Game/_Manager/InGame/DataAsset/BP/Weapons/BP_Daggers_DA.chargeTime` (`self.daggersDA`))) 0.1))
              (`/Engine/EditorBlueprintResources/StandardMacros.DoOnce` false :!label _label_8
                (:`Completed`
                  (message `/Game/Blueprints/BPI/PlayerController/BPI_PlayerController.PlayGamepadRumble` (`GameplayStatics.GetPlayerController` 0) "/Game/Haptics/FFE_WeaponsFullyChargedLoops.FFE_WeaponsFullyChargedLoops" true))))))))))

(event `ResetSpawnPrevis`
  ;[1 1 1] Start shoot event
  (goto _label_6 :!via `Reset`))

(event `StartPrevisualization`
  (bind _previsuaizationref (`self.previsuaizationRef`))
  (bind _spline (`/Game/Blueprints/Weapons/Previsualization/BP_Previsualize.Spline` (`self.previsuaizationRef`)))
  (bind _spline_2 (`/Game/Blueprints/Weapons/Previsualization/BP_Previsualize.Spline` _previsuaizationref))
  ;[0 0.778 1] Previsualization
  (set `self.previsualization?` true)
  (`self.CalculPos`)
  (`self.GetSpawnLocAndRot`)
  (`/Game/Blueprints/Weapons/Previsualization/BP_Previsualize.ClearSpline` (`self.previsuaizationRef`))
  (bind _predictresult (`GameplayStatics.Blueprint_PredictProjectilePath_Advanced` (make `PredictProjectilePathParams` (`self.spawnLocation`) (`self.CalculBombeVelocity`) true 5.0 2.0 true "ECC_Visibility" _ (`|MakeArray` (`GameplayStatics.GetPlayerCharacter` 0) :!type "Actor Object Reference") 20.0 (* (* (`self.fireballGravityScale`) 980.0) -1.0))))
  (for _array_element (break `PredictProjectilePathResult` _predictresult)
    (`SplineComponent.AddSplinePoint` _spline (break `PredictProjectilePathPointData` _array_element) "Local" true))
  (`SplineComponent.SetSplinePointType` _spline (`KismetArrayLibrary.Array_LastIndex` (break `PredictProjectilePathResult` _predictresult)) "CurveClamped" true)
  (for _index (range (`SplineComponent.GetNumberOfSplinePoints` _spline))
    (bind _splinemeshcomponent (`/Game/Blueprints/Weapons/Previsualization/BP_Previsualize.Add Spline Mesh Component Fonction` _previsuaizationref))
    (bind (_location _tangent) (`SplineComponent.GetLocationAndTangentAtSplinePoint` _spline_2 _index "Local"))
    (bind (_location_2 _tangent_2) (`SplineComponent.GetLocationAndTangentAtSplinePoint` _spline_2 (+ _index 1) "Local"))
    (`SplineMeshComponent.SetStartAndEnd` _splinemeshcomponent _location _tangent _location_2 _tangent_2 true))
  (bind (_bblockinghit _binitialoverlap _time _distance _location_3 _impactpoint _normal) (`GameplayStatics.BreakHitResult` (`.HitResult` (break `PredictProjectilePathResult` _predictresult))))
  (bind (_returnvalue_roll _returnvalue_pitch _returnvalue_yaw) (`KismetMathLibrary.BreakRotator` (`KismetMathLibrary.FindLookAtRotation` (`KismetMathLibrary.Vector_Zero`) _normal)))
  (`Actor.K2_SetActorLocationAndRotation` (`self.endPrevisualizationRef`) _impactpoint (`KismetMathLibrary.MakeRotator` _returnvalue_roll (+ _returnvalue_pitch 90.0) _returnvalue_yaw) false false))

(fn `CalculBombeVelocity`
  (returns (ReturnValue :type "Vector Structure"))
  (bind _fireballda (`self.fireballDA`))
  (bind _projectilespeed (`/Game/_Manager/InGame/DataAsset/BP/Weapons/BP_Fireball_DA.projectileSpeed` (`self.fireballDA`)))
  (bind (_rot _distance) (`self.FindTargetRot` (`SceneComponent.K2_GetComponentLocation` (`SceneComponent.GetChildComponent` (`Character.Mesh` (`GameplayStatics.GetPlayerCharacter` 0)) 1))))
  (return (* (+ (`KismetMathLibrary.GetForwardVector` (`KismetMathLibrary.MakeRotator` (.roll _rot) (`KismetMathLibrary.FClamp` (.pitch _rot) (`/Game/_Manager/InGame/DataAsset/BP/Weapons/BP_Fireball_DA.minThrowAngle` _fireballda) (`/Game/_Manager/InGame/DataAsset/BP/Weapons/BP_Fireball_DA.maxThrowAngle` _fireballda)) (.yaw _rot))) (`KismetMathLibrary.MakeVector` 0.0 0.0 (`/Game/_Manager/InGame/DataAsset/BP/Weapons/BP_Fireball_DA.archFactor` (`self.fireballDA`)))) (`KismetMathLibrary.SelectFloat` _projectilespeed (`KismetMathLibrary.SelectFloat` (`KismetMathLibrary.FClamp` (* _distance 1.5) 0.0 _projectilespeed) _projectilespeed (> _distance 0.0)) (`self.aiming?`)))))

(fn `CalculPos`
  (bind _returnvalue (`GameplayStatics.GetPlayerCameraManager` 0))
  (bind _returnvalue_2 (`Actor.K2_GetActorLocation` _returnvalue))
  (set `self.crossAir` _returnvalue_2)
  (set `self.inpactPoint` (+ _returnvalue_2 (* (`Actor.GetActorForwardVector` _returnvalue) (`self.fireballSpeed`)))))

(fn `FindTargetRot`
  (params (startPos :type "Vector Structure"))
  (returns (rot :type "Rotator Structure") (Distance :type "Float (single-precision)"))
  (bind _returnvalue (`GameplayStatics.GetPlayerCameraManager` 0))
  (bind _returnvalue_2 (`GameplayStatics.GetPlayerCameraManager` 0))
  (bind _returnvalue_3 (`PlayerCameraManager.GetCameraLocation` _returnvalue_2))
  (bind _debugmode (message `/Game/Blueprints/BPI/GameInstance/BPI_GameInstance.GetDebugMode` (`GameplayStatics.GetGameInstance`)))
  (bind _targetarmlength (message `/Game/Blueprints/BPI/Player/BPI_Player.GetCameraArmLength` (`GameplayStatics.GetPlayerCharacter` 0)))
  (bind (_outhit _returnvalue_4) (`KismetSystemLibrary.LineTraceSingle` :`Start` (+ (* _targetarmlength (`Actor.GetActorForwardVector` _returnvalue_2)) _returnvalue_3) :`End` (+ _returnvalue_3 (* (`Actor.GetActorForwardVector` _returnvalue_2) (select `/Game/Blueprints/Enums/Enum_WeaponType` (`self.currentWeapon`) :`NewEnumerator0` (`/Game/_Manager/InGame/DataAsset/BP/Weapons/BP_Lance_DA.range` (`self.lanceDA`)) :`NewEnumerator1` 3000.0 :`NewEnumerator2` (`/Game/_Manager/InGame/DataAsset/BP/Weapons/BP_Daggers_DA.range` (`self.daggersDA`))))) :`TraceChannel` "TraceTypeQuery1" :`DrawDebugType` (select `bool` _debugmode :`true` "ForDuration" :!type "EDrawDebugTrace Enum")))
  (if _returnvalue_4
    (bind (_bblockinghit _binitialoverlap _time _distance _location _impactpoint) (`GameplayStatics.BreakHitResult` _outhit))
    (return (`KismetMathLibrary.FindLookAtRotation` (`local.startPos`) _impactpoint) (`KismetMathLibrary.Vector_Distance` _impactpoint (`PlayerCameraManager.GetCameraLocation` (`GameplayStatics.GetPlayerCameraManager` 0))))
    (else
      (return (`KismetMathLibrary.FindLookAtRotation` (`local.startPos`) (+ (`PlayerCameraManager.GetCameraLocation` _returnvalue) (* (`Actor.GetActorForwardVector` _returnvalue) (select `/Game/Blueprints/Enums/Enum_WeaponType` (`self.currentWeapon`) :`NewEnumerator0` (`/Game/_Manager/InGame/DataAsset/BP/Weapons/BP_Lance_DA.range` (`self.lanceDA`)) :`NewEnumerator1` 3000.0 :`NewEnumerator2` (`/Game/_Manager/InGame/DataAsset/BP/Weapons/BP_Daggers_DA.range` (`self.daggersDA`)))))) 0.0))))

(fn `GetSpawnLocAndRot`
  (bind _outhit (`KismetSystemLibrary.LineTraceSingle` (`self.crossAir`) (`self.inpactPoint`) "TraceTypeQuery1" false (`|MakeArray` (`GameplayStatics.GetPlayerCharacter` 0) :!type "Actor Object Reference")))
  (if (`GameplayStatics.BreakHitResult` _outhit)
    (set `self.inpactPoint` (`.ImpactPoint` (`GameplayStatics.BreakHitResult` _outhit))))
  (set `self.spawnLocation` (`SceneComponent.K2_GetComponentLocation` (`SceneComponent.GetChildComponent` (`Character.Mesh` (`GameplayStatics.GetPlayerCharacter` 0)) 1)))
  (set `self.spawnRotation` (`KismetMathLibrary.MakeRotFromX` (- (`self.inpactPoint`) (`self.spawnLocation`)))))