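; Previsualization Blueprint in the weapons folder that provides the spline and spline meshes for a visual preview.
; On BeginPlay it spawns a separate SplineMeshActor at its own transform and adds the Spline component to it.
; A helper creates manually attached spline mesh components on itself with the previsualization material and tracks them in an array.
; ClearSpline destroys those meshes and clears the spline points; nothing here sets points or shapes meshes.
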(event `self.ReceiveBeginPlay`
  (bind _returnvalue (`|SpawnActorFromClass` "/Script/Engine.SplineMeshActor" (`self.GetTransform`) "Undefined" "MultiplyWithRoot" null null))
  (set `self.PrevisualizationSpline` _returnvalue)
  (bind _returnvalue_2 (`AddComponent|NODE_AddSplineComponent-0` :`self` (`self.PrevisualizationSpline`)))
  (set `self.Spline` _returnvalue_2))

(fn `Add Spline Mesh Component Fonction`
  (returns (splineMeshComponent :type "SplineMeshComponent Object Reference"))
  (bind _returnvalue (`AddComponent|NODE_AddSplineMeshComponent-0` :`bManualAttachment` true))
  (`KismetArrayLibrary.Array_Add` (`self.SplineMesh`) _returnvalue)
  (`PrimitiveComponent.SetMaterial` _returnvalue 0 "/Game/Blueprints/Weapons/Previsualization/MI_Previsualization.MI_Previsualization")
  (return _returnvalue))

(fn `ClearSpline`
  (bind _splinemesh (`self.SplineMesh`))
  (`ActorComponent.K2_DestroyComponent` _splinemesh)
  (`KismetArrayLibrary.Array_Clear` _splinemesh)
  (`SplineComponent.ClearSplinePoints` (`self.Spline`) true))

(fn `UserConstructionScript`)