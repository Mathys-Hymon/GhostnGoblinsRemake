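; Soul orb pickup that drops, bobs in place, then homes in on the player to be absorbed.
; Tick runs three phases: physics fall until a downward trace finds the floor, sine-wave bobbing until the player enters AbsorbRadius, then damped velocity attraction that produces an orbiting effect.
; Each player overlap on the sphere decrements Life; at zero the orb destroys itself and prints "XP", with ultimate charging still a TODO.
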(event `self.ReceiveTick`
  (params (DeltaSeconds :type "Float (single-precision)"))
  (bind _returnvalue (`self.K2_GetActorLocation`))
  (bind _sphere (`self.Sphere`))
  (bind _returnvalue_2 (`SceneComponent.GetRelativeTransform` (`self.Sphere`)))
  (if (`self.initialSpawn`)
    ;[1 1 1] Initial Spawn  Phase - Actor has physics and affected by gravity till near floor
    (bind (_outhit _returnvalue_3) (`KismetSystemLibrary.LineTraceSingle` :`Start` _returnvalue :`End` (+ _returnvalue (* (0.0 0.0 -1.0) 30.0)) :`TraceChannel` "TraceTypeQuery1" :`DrawDebugType` "ForOneFrame"))
    (if _returnvalue_3
      (`PrimitiveComponent.SetEnableGravity` _sphere false)
      ;[1 1 1] Set Up for Idle phase
      (`PrimitiveComponent.SetSimulatePhysics` _sphere false)
      (set `self.initialSpawn` false)
      (set `self.relativeZTransform` (.z (.location (`SceneComponent.GetRelativeTransform` (`self.Sphere`))))))
    (elif (`self.idle`)
      ;[1 1 1] Bobbing phase - When orb is idle on floor
      (`self.K2_SetActorRelativeLocation` (`KismetMathLibrary.MakeVector` (.x (.location _returnvalue_2)) (.y (.location _returnvalue_2)) (+ (`self.relativeZTransform`) (* (`KismetMathLibrary.DegSin` (* (`self.GetGameTimeSinceCreation`) (`self.bobSpeed`))) (`self.bobdistance`)))))
      ;[1 1 1] Set boolean for next phase
      (set `self.idle` (>= (`KismetMathLibrary.Vector_Distance` (`self.K2_GetActorLocation`) (`self.K2_GetActorLocation` (`GameplayStatics.GetPlayerPawn` 0))) (`self.absorbRadius`)))
      (else
        ;[1 1 1] Absorb phase - attracted towards player at an offset for orbiting effect
        (bind _output_get (set `self.Velocity` (* (+ (`self.velocity`) (/ (- (`self.K2_GetActorLocation` (`GameplayStatics.GetPlayerPawn` 0)) (`self.K2_GetActorLocation`)) 100.0)) 0.95)))
        (`self.K2_AddActorWorldOffset` _output_get)))))

(event `self.Sphere.OnComponentBeginOverlap`
  (params (OverlappedComponent :type "PrimitiveComponent Object Reference") (OtherActor :type "Actor Object Reference") (OtherComp :type "PrimitiveComponent Object Reference") (OtherBodyIndex :type Integer) (bFromSweep :type Boolean) (SweepResult :type "HitResult Structure (by ref)"))
  (bind _life (`self.life`))
  ;[1 1 1] Let orbs rotate a few times before being consumed
  (if (== OtherActor (`GameplayStatics.GetPlayerPawn` 0))
    (if (== 0 _life)
      ;[1 0 0] !! Consume and charge ultimate
      (`self.K2_DestroyActor`)
      (`KismetSystemLibrary.PrintString` "XP")
      (else
        (set `self.life` (- _life 1))))))

(fn `UserConstructionScript`)