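; Modular plank platform that builds itself along an editable, optionally looping spline in the construction script.
; Mesh bounds set the segment length for three spline-mesh layers: beams, randomly picked planks with collision, and bottom planks.
; Open splines can get random end-cap meshes at either end.
; A set number of non-colliding supports is spaced evenly along the spline, with configurable offset and random tilt.
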(fn `setStaticMeshAlongSpline`
  (params (index :type Integer) (staticMesh :type "StaticMesh Object Reference") (Length :type "Float (double-precision)") (endOffset :type "Vector Structure") (startOffset :type "Vector Structure") (collision :type "ECollisionEnabled Enum" :default "NoCollision"))
  (bind _returnvalue (* index Length))
  (bind _spline (`self.Spline`))
  (bind _spline_2 (`self.Spline`))
  (bind _spline_3 (`self.Spline`))
  (bind _returnvalue_2 (`SplineComponent.GetRotationAtDistanceAlongSpline` _spline_2 _returnvalue "Local"))
  (bind _returnvalue_3 (* (+ index 1) Length))
  (bind _returnvalue_4 (`SplineComponent.GetRotationAtDistanceAlongSpline` _spline _returnvalue_3 "Local"))
  (bind _returnvalue_5 (`AddComponent|NODE_AddSplineMeshComponent-0`))
  (`PrimitiveComponent.SetCollisionEnabled` _returnvalue_5 collision)
  (`SplineMeshComponent.SetForwardAxis` _returnvalue_5 "X" true)
  (`SplineMeshComponent.SetForwardAxis` _returnvalue_5 "X" true)
  (`StaticMeshComponent.SetStaticMesh` _returnvalue_5 staticMesh)
  (`SplineMeshComponent.SetStartAndEnd` _returnvalue_5 (+ (`SplineComponent.GetLocationAtDistanceAlongSpline` _spline_2 _returnvalue "Local") (* (`KismetMathLibrary.GetForwardVector` _returnvalue_2) (.x (`local.startOffset`))) (* (`KismetMathLibrary.GetRightVector` _returnvalue_2) (.y (`local.startOffset`))) (* (`KismetMathLibrary.GetUpVector` _returnvalue_2) (.z (`local.startOffset`)))) (`KismetMathLibrary.ClampVectorSize` (`SplineComponent.GetTangentAtDistanceAlongSpline` _spline_3 _returnvalue "Local") 0.0 Length) (+ (`SplineComponent.GetLocationAtDistanceAlongSpline` _spline_3 _returnvalue_3 "Local") (* (`KismetMathLibrary.GetForwardVector` _returnvalue_4) (.x (`local.endOffset`))) (* (`KismetMathLibrary.GetRightVector` _returnvalue_4) (.y (`local.endOffset`))) (* (`KismetMathLibrary.GetUpVector` _returnvalue_4) (.z (`local.endOffset`)))) (`KismetMathLibrary.ClampVectorSize` (`SplineComponent.GetTangentAtDistanceAlongSpline` _spline _returnvalue_3 "Local") 0.0 (`local.Length`)) true))

(fn `UserConstructionScript`
  (bind _spline (`self.Spline`))
  (bind _spline_2 (`self.Spline`))
  (bind (_propoffset_x _propoffset_y _propoffset_z) (`KismetMathLibrary.BreakVector` (`self.propOffset`)))
  (bind (_randomtilt_x _randomtilt_y) (`KismetMathLibrary.BreakVector2D` (`self.randomTilt`)))
  (bind _supportamount (`self.supportAmount`))
  (bind _spline_3 (`self.Spline`))
  (bind (_returnvalue_min _returnvalue_max) (break `Box` (`StaticMesh.GetBoundingBox` (`self.bottomPlankMesh`))))
  (bind (_returnvalue_min_2 _returnvalue_max_2) (break `Box` (`StaticMesh.GetBoundingBox` (`self.beamMesh`))))
  (bind _returnvalue (`SplineComponent.GetNumberOfSplinePoints` (`self.Spline`)))
  (bind _returnvalue_2 (`SplineComponent.GetRotationAtSplinePoint` _spline 0 "Local"))
  (bind (_returnvalue_min_3 _returnvalue_max_3) (break `Box` (`StaticMesh.GetBoundingBox` (`|GetArrayItem` (`self.planksMesh`)))))
  (bind _returnvalue_3 (`SplineComponent.GetRotationAtSplinePoint` _spline_2 _returnvalue "Local"))
  (bind _returnvalue_x (`KismetMathLibrary.BreakVector` (+ (`KismetMathLibrary.Vector_GetAbs` _returnvalue_min) (`KismetMathLibrary.Vector_GetAbs` _returnvalue_max))))
  (bind _returnvalue_x_2 (`KismetMathLibrary.BreakVector` (+ (`KismetMathLibrary.Vector_GetAbs` _returnvalue_min_2) (`KismetMathLibrary.Vector_GetAbs` _returnvalue_max_2))))
  (bind _returnvalue_x_3 (`KismetMathLibrary.BreakVector` (+ (`KismetMathLibrary.Vector_GetAbs` _returnvalue_min_3) (`KismetMathLibrary.Vector_GetAbs` _returnvalue_max_3))))
  (`KismetSystemLibrary.FlushPersistentDebugLines`)
  (`SplineComponent.SetClosedLoop` (`self.Spline`) (`self.loop`) true)
  (for _array_element (`self.supports`)
    (`ActorComponent.K2_DestroyComponent` _array_element))
  (`KismetArrayLibrary.Array_Clear` (`self.supports`))
  (`|ExecutionSequence`
    (:`then_0`
      (set `self.xLengthBottomPlank` _returnvalue_x)
      (set `self.xLengthBeam` _returnvalue_x_2)
      (bind _output_get (set `self.xLengthPlanks` _returnvalue_x_3))
      (`|ExecutionSequence`
        (:`then_0`
          (for _index (range (+ (`KismetMathLibrary.FTrunc` (/ (`SplineComponent.GetSplineLength` (`self.Spline`)) (`self.xLengthBeam`))) 1))
            (`self.setStaticMeshAlongSpline` _index (`self.beamMesh`) (`self.xLengthBeam`) (25.0 0.0 -27.0) (0.0 0.0 -27.0))))
        (:`then_1`
          (for _index_2 (range (`KismetMathLibrary.FTrunc` (/ (`SplineComponent.GetSplineLength` (`self.Spline`)) _output_get)))
            (`self.setStaticMeshAlongSpline` _index_2 (`KismetArrayLibrary.Array_Random` (`self.planksMesh`)) (`self.xLengthPlanks`) (0.0 0.0 0.0) (0.0 0.0 0.0) "QueryAndPhysics"))
          (if (not (`self.loop`))
            (`|ExecutionSequence`
              (:`then_0`
                (if (`self.leftEnd`)
                  (bind _returnvalue_4 (`AddComponent|NODE_AddStaticMeshComponent-2` :`RelativeTransform` (`KismetMathLibrary.MakeTransform` (- (`SplineComponent.GetLocationAtSplinePoint` _spline_2 _returnvalue "Local") (* (`KismetMathLibrary.GetForwardVector` _returnvalue_3) 4.0) (0.0 0.0 27.0)) _returnvalue_3 (-1.0 1.0 1.0))))
                  (`StaticMeshComponent.SetStaticMesh` _returnvalue_4 (`KismetArrayLibrary.Array_Random` (`self.endMesh`)))))
              (:`then_1`
                (if (`self.rightEnd`)
                  (bind _returnvalue_5 (`AddComponent|NODE_AddStaticMeshComponent-3` :`RelativeTransform` (`KismetMathLibrary.MakeTransform` (- (`SplineComponent.GetLocationAtSplinePoint` _spline 0 "Local") (* (`KismetMathLibrary.GetForwardVector` _returnvalue_2) 4.0) (0.0 0.0 27.0)) _returnvalue_2)))
                  (`StaticMeshComponent.SetStaticMesh` _returnvalue_5 (`KismetArrayLibrary.Array_Random` (`self.endMesh`))))))))
        (:`then_2`
          (for _index_3 (range (+ (`KismetMathLibrary.FTrunc` (/ (`SplineComponent.GetSplineLength` (`self.Spline`)) (`self.xLengthBottomPlank`))) 1))
            (`self.setStaticMeshAlongSpline` _index_3 (`self.bottomPlankMesh`) (`self.xLengthBottomPlank`) (25.0 0.0 -20.0) (0.0 0.0 -20.0))))))
    (:`then_1`
      (for _index_4 (range (+ _supportamount 1))
        (bind _returnvalue_6 (`SplineComponent.GetRotationAtDistanceAlongSpline` (`self.Spline`) (/ (* _index_4 (`SplineComponent.GetSplineLength` (`self.Spline`))) _supportamount) "Local"))
        (bind _returnvalue_7 (`AddComponent|NODE_AddStaticMeshComponent-1` :`RelativeTransform` (`KismetMathLibrary.MakeTransform` (+ (* (`KismetMathLibrary.GetForwardVector` _returnvalue_6) _propoffset_x) (* (`KismetMathLibrary.GetRightVector` _returnvalue_6) _propoffset_y) (`KismetMathLibrary.MakeVector` 0.0 0.0 _propoffset_z) (- (`SplineComponent.GetLocationAtDistanceAlongSpline` _spline_3 (/ (* _index_4 (`SplineComponent.GetSplineLength` _spline_3)) (`self.supportAmount`)) "Local") (0.0 0.0 65.0))) (`KismetMathLibrary.MakeRotator` (+ (+ (`self.propTiltRot`) 180.0) (`KismetMathLibrary.RandomFloatInRange` _randomtilt_x (* _randomtilt_x -1.0)) (.roll _returnvalue_6)) (+ (.pitch _returnvalue_6) (`KismetMathLibrary.RandomFloatInRange` _randomtilt_y (* _randomtilt_y -1.0))) (.yaw _returnvalue_6)) (-1.0 -1.0 -1.0))))
        (`StaticMeshComponent.SetStaticMesh` _returnvalue_7 (`self.supportMesh`))
        (`KismetArrayLibrary.Array_Add` (`self.supports`) _returnvalue_7)
        (`PrimitiveComponent.SetCollisionEnabled` _returnvalue_7 "NoCollision")))))