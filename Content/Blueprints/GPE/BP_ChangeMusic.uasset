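; BP_ChangeMusic is a trigger volume that switches the game's music when the player enters it.
; Its box takes its extent from the Size variable, applied in the construction script and again on BeginPlay.
; On overlap with an actor implementing BPI_Player, it maps MusicIndex (Cemetery, Village or Boss) to a track number and passes it to the Game Instance through PlayMusicMessage.
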(event `self.ReceiveBeginPlay`
  (`BoxComponent.SetBoxExtent` (`self.Box`) (`self.size`) true))

(event `self.Box.OnComponentBeginOverlap`
  (params (OverlappedComponent :type "PrimitiveComponent Object Reference") (OtherActor :type "Actor Object Reference") (OtherComp :type "PrimitiveComponent Object Reference") (OtherBodyIndex :type Integer) (bFromSweep :type Boolean) (SweepResult :type "HitResult Structure (by ref)"))
  (bind _returnvalue (`GameplayStatics.GetGameInstance`))
  (if (`KismetSystemLibrary.DoesImplementInterface` OtherActor "/Game/Blueprints/BPI/Player/BPI_Player.BPI_Player_C")
    (switch `/Game/Blueprints/Enums/Enum_Music` (`self.musicIndex`)
      (:`NewEnumerator0`
        (message `/Game/Blueprints/BPI/GameInstance/BPI_GameInstance.PlayMusic` _returnvalue 0))
      (:`NewEnumerator1`
        (message `/Game/Blueprints/BPI/GameInstance/BPI_GameInstance.PlayMusic` _returnvalue 1))
      (:`NewEnumerator2`
        (message `/Game/Blueprints/BPI/GameInstance/BPI_GameInstance.PlayMusic` _returnvalue 2)))))

(fn `UserConstructionScript`
  (`BoxComponent.SetBoxExtent` (`self.Box`) (`self.size`) true))