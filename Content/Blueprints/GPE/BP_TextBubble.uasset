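; BP_TextBubble is a proximity text bubble with a bobbing Soul component, showing configurable text when a BPI_Player actor enters its detection sphere.
; Entering plays a random talk sound and reverses the FadeOut timeline to reveal the text, while a looping frame-delta timer turns the actor toward the camera.
; Leaving fades out voice and text through a dynamic material's Opacity, then hides the text and pauses the timer.
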(event `RotateBubbleTimer`
  (bind _returnvalue (`KismetSystemLibrary.K2_SetTimerDelegate` (delegate `RotateBubble`) (`GameplayStatics.GetWorldDeltaSeconds`) true true))
  (set `self.timerByEventRef` _returnvalue))

(event `RotateBubble`
  (`self.K2_SetActorRotation` (`KismetMathLibrary.FindLookAtRotation` (`self.K2_GetActorLocation`) (`self.K2_GetActorLocation` (`GameplayStatics.GetPlayerCameraManager` 0)))))

(event `self.ReceiveBeginPlay`
  (`SceneComponent.SetHiddenInGame` (`self.TextRender`) true false)
  (`MaterialInstanceDynamic.SetScalarParameterValue` (`self.materialRef`) "Opacity" 0.0)
  (bind (_direction _alpha) (`Timeline|soulMovement`)
    (:`Update`
      (`SceneComponent.K2_SetRelativeLocation` (`self.Soul`) (`KismetMathLibrary.MakeVector` 0.0 0.0 (`KismetMathLibrary.Lerp` 80.0 20.0 _alpha)) false false))))

(event `self.Sphere.OnComponentEndOverlap`
  (params (OverlappedComponent :type "PrimitiveComponent Object Reference") (OtherActor :type "Actor Object Reference") (OtherComp :type "PrimitiveComponent Object Reference") (OtherBodyIndex :type Integer))
  (bind _voicesound (`self.voiceSound`))
  (if (`KismetSystemLibrary.DoesImplementInterface` OtherActor "/Game/Blueprints/BPI/Player/BPI_Player.BPI_Player_C")
    (`/Engine/EditorBlueprintResources/StandardMacros.IsValid` _voicesound
      (:`Is Valid`
        (`AudioComponent.FadeOut` _voicesound 0.3 0.0 "Linear")
        (bind (_direction _opacity) (`Timeline|FadeOut` :!label _label)
          (:`Update`
            (`MaterialInstanceDynamic.SetScalarParameterValue` (`self.materialRef`) "Opacity" _opacity))
          (:`Finished`
            (if (== _opacity 0.0)
              (`SceneComponent.SetHiddenInGame` (`self.TextRender`) true false)
              (`KismetSystemLibrary.K2_PauseTimerHandle` (`self.timerByEventRef`))))))
      (:`Is Not Valid`
        (goto _label)))))

(event `self.Sphere.OnComponentBeginOverlap`
  (params (OverlappedComponent :type "PrimitiveComponent Object Reference") (OtherActor :type "Actor Object Reference") (OtherComp :type "PrimitiveComponent Object Reference") (OtherBodyIndex :type Integer) (bFromSweep :type Boolean) (SweepResult :type "HitResult Structure (by ref)"))
  (if (`KismetSystemLibrary.DoesImplementInterface` OtherActor "/Game/Blueprints/BPI/Player/BPI_Player.BPI_Player_C")
    (`SceneComponent.SetHiddenInGame` (`self.TextRender`) false false)
    (`self.RotateBubbleTimer`)
    (bind _returnvalue (`GameplayStatics.SpawnSoundAtLocation` (`KismetArrayLibrary.Array_Random` (`/Game/_Manager/InGame/DataAsset/BP/SFX/BP_SFX_DA.talk` (`self.sfxDataAsset`))) (`self.K2_GetActorLocation`) (struct) 1.0 1.0 0.0 "/Game/Imports/SFX/SoundAttenuation.SoundAttenuation" null))
    (set `self.voiceSound` _returnvalue)
    (goto _label :!via `Reverse`)))

(fn `UserConstructionScript`
  (bind _returnvalue (`PrimitiveComponent.CreateDynamicMaterialInstance` (`self.TextRender`) 0 (`TextRenderComponent.TextMaterial` (`self.TextRender`)) "None"))
  (set `self.materialRef` _returnvalue)
  (`TextRenderComponent.K2_SetText` (`self.TextRender`) (`self.textToShow`))
  (`self.SetActorHiddenInGame` false)
  (`SphereComponent.SetSphereRadius` (`self.Sphere`) (`self.detectionRadius`) true)
  (`MaterialInstanceDynamic.SetScalarParameterValue` (`self.materialRef`) "Opacity" 1.0))