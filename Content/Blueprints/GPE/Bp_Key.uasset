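; Key pickup actor that passes its KeyID to the player pawn on overlap, then destroys itself a tick later.
; On Tick it falls under physics until a short downward trace hits, then disables physics and records a resting height.
; It then idles, spinning via a timeline and bobbing on a sine of its lifetime.
; The construction script applies an optional custom mesh and material, with a fallback mesh.
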(event `self.ReceiveTick`
  (params (DeltaSeconds :type "Float (single-precision)"))
  (`self.ItemMovement`))

(event `ItemMovement`
  (bind _returnvalue (`self.K2_GetActorLocation`))
  (bind _key (`self.Key`))
  (bind _key_2 (`self.Key`))
  (bind _returnvalue_2 (`SceneComponent.GetRelativeTransform` (`self.Key`)))
  (bind (_returnvalue_roll _returnvalue_pitch) (`KismetMathLibrary.BreakRotator` (`SceneComponent.K2_GetComponentRotation` _key)))
  (if (`self.initialSpawn`)
    ;[1 0.8712 0] Initial Spawn  Phase - Actor has physics and affected by gravity till near floor
    (bind (_outhit _returnvalue_3) (`KismetSystemLibrary.LineTraceSingle` :`Start` _returnvalue :`End` (+ _returnvalue (* (0.0 0.0 -1.0) 50.0)) :`TraceChannel` "TraceTypeQuery1" :`DrawDebugType` "ForOneFrame"))
    (if _returnvalue_3
      (`PrimitiveComponent.SetEnableGravity` _key_2 false)
      ;;[1 1 1] Set Up for Idle phase
      (`PrimitiveComponent.SetSimulatePhysics` _key_2 false)
      (set `self.initialSpawn` false)
      (set `self.relativeZTransform` (+ (.z (.location (`SceneComponent.GetRelativeTransform` (`self.Key`)))) 10.0)))
    (else
      ;[0 1 0.2866] Bobbing phase - When orb is idle on floor
      (`TimelineComponent.SetPlayRate` (`self.ActorRotateTimeline`) (`self.rotationSpeed`))
      (bind (_direction _newtrack_0) (`Timeline|ActorRotateTimeline`)
        (:`Update`
          (`SceneComponent.K2_SetWorldRotation` _key (`KismetMathLibrary.MakeRotator` _returnvalue_roll _returnvalue_pitch _newtrack_0) false false)
          (`self.K2_SetActorRelativeLocation` (`KismetMathLibrary.MakeVector` (.x (.location _returnvalue_2)) (.y (.location _returnvalue_2)) (+ (`self.relativeZTransform`) (* (`KismetMathLibrary.DegSin` (* (`self.GetGameTimeSinceCreation`) (`self.bobSpeed`))) (`self.bobDistance`))))))))))

(event `self.Key.OnComponentBeginOverlap`
  (params (OverlappedComponent :type "PrimitiveComponent Object Reference") (OtherActor :type "Actor Object Reference") (OtherComp :type "PrimitiveComponent Object Reference") (OtherBodyIndex :type Integer) (bFromSweep :type Boolean) (SweepResult :type "HitResult Structure (by ref)"))
  (bind _returnvalue (`GameplayStatics.GetPlayerPawn` 0))
  ;[0 1 0.9961] Stack key on the plyaer and destroy actor
  (if (== OtherActor _returnvalue)
    (message `/Game/Blueprints/BPI/Player/BPI_LootKey.GetKeyId` _returnvalue (`self.keyID`))
    (`KismetSystemLibrary.DelayUntilNextTick`)
    (`self.K2_DestroyActor`)))

(fn `UserConstructionScript`
  (bind _custommaterial (`self.customMaterial`))
  (bind _newmesh (`self.newMesh`))
  (`/Engine/EditorBlueprintResources/StandardMacros.IsValid` _newmesh
    (:`Is Valid`
      (`StaticMeshComponent.SetStaticMesh` (`self.Key`) _newmesh))
    (:`Is Not Valid`
      (`StaticMeshComponent.SetStaticMesh` (`self.Key`) "/Engine/VREditor/TransformGizmo/StartRotationHandleIndicator.StartRotationHandleIndicator")))
  (`/Engine/EditorBlueprintResources/StandardMacros.IsValid` _custommaterial
    (:`Is Valid`
      (`PrimitiveComponent.SetMaterial` (`self.Key`) 0 _custommaterial))))