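; BP_WeaponJar is a breakable jar that drops a weapon-change actor when destroyed.
; It plays a random aura sound from the SFX data asset at its location on BeginPlay.
; The first Chaos break event of its Geometry Collection, gated by a DoOnce, plays a random break sound, spawns BP_ChangeWeapon slightly above the jar with its WeaponType, and fades out the aura.
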(event `self.ReceiveBeginPlay`
  (bind _returnvalue (`GameplayStatics.SpawnSoundAtLocation` (`KismetArrayLibrary.Array_Random` (`/Game/_Manager/InGame/DataAsset/BP/SFX/BP_SFX_DA.weaponJarAura` (`self.sfxDataAsset`))) (`self.K2_GetActorLocation`) (struct) 1.0 1.0 0.0 "/Game/Imports/SFX/SoundAttenuation.SoundAttenuation" null))
  (set `self.auraSound` _returnvalue))

(event `self.GeometryCollection.OnChaosBreakEvent`
  (params (BreakEvent :type "ChaosBreakEvent Structure (by ref)"))
  (bind (_returnvalue_x _returnvalue_y _returnvalue_z) (`KismetMathLibrary.BreakVector` (`self.K2_GetActorLocation`)))
  (`/Engine/EditorBlueprintResources/StandardMacros.DoOnce` false
    (:`Completed`
      (`GameplayStatics.PlaySoundAtLocation` (`KismetArrayLibrary.Array_Random` (`/Game/_Manager/InGame/DataAsset/BP/SFX/BP_SFX_DA.weaponJarBreak` (`self.sfxDataAsset`))) (`self.K2_GetActorLocation`) (struct) 1.0 1.0 0.0 "/Game/Imports/SFX/SoundAttenuation.SoundAttenuation" null null null)
      (`|SpawnActorFromClass` "/Game/Blueprints/GPE/BP_ChangeWeapon.BP_ChangeWeapon_C" (`KismetMathLibrary.MakeTransform` (`KismetMathLibrary.MakeVector` _returnvalue_x _returnvalue_y (+ _returnvalue_z 50.0))) "AdjustIfPossibleButAlwaysSpawn" "MultiplyWithRoot" null (`self.Weapon Type`) null)
      (`AudioComponent.FadeOut` (`self.auraSound`) 0.5 0.0 "Linear"))))

(fn `UserConstructionScript`)