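; BP_ChangeWeapon is a weapon pickup that swaps the player's current weapon for its own WeaponType on overlap.
; It queries and sets weapons through BPI_Player, spawns a replacement pickup holding the old weapon at the player's location, then destroys itself.
; A JustSpawned flag, cleared shortly after overlap ends, and a DoOnce prevent immediate re-pickup and duplicate spawns.
; The construction script sets the sphere radius from a data asset and the mesh by weapon type.
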(event `self.DetectionSphere.OnComponentBeginOverlap`
  (params (OverlappedComponent :type "PrimitiveComponent Object Reference") (OtherActor :type "Actor Object Reference") (OtherComp :type "PrimitiveComponent Object Reference") (OtherBodyIndex :type Integer) (bFromSweep :type Boolean) (SweepResult :type "HitResult Structure (by ref)"))
  ;[1 1 1] Detect if player is picking up the new weapon
  (if (`KismetSystemLibrary.DoesImplementInterface` OtherActor "/Game/Blueprints/BPI/Player/BPI_Player.BPI_Player_C")
    (if (not (`self.justSpawned`))
      (bind _canpickupweapon (message `/Game/Blueprints/BPI/Player/BPI_Player.GetCanPickUpWeapon` OtherActor))
      (if _canpickupweapon
        (`/Engine/EditorBlueprintResources/StandardMacros.DoOnce` false :!label _label ; spawn only one weapon
          (:`Completed`
            (bind _currentweapon (message `/Game/Blueprints/BPI/Player/BPI_Player.GetCurrentWeapon` OtherActor))
            (bind _output_get (set `self.lastWeapon` _currentweapon))
            (bind _returnvalue (`|SpawnActorFromClass` "BP_ChangeWeapon_C" (`KismetMathLibrary.MakeTransform` (`self.K2_GetActorLocation` OtherActor)) "AlwaysSpawn" "MultiplyWithRoot" null _output_get true null))
            (set `/Game/Blueprints/GPE/BP_ChangeWeapon.justSpawned` true _returnvalue)
            (message `/Game/Blueprints/BPI/Player/BPI_Player.SetWeapon` OtherActor (`self.weaponType`)) ; Set the new weapon
            (`self.K2_DestroyActor`)))))))

(event `ResetPickUp`
  ;[1 1 1] Detect if player is picking up the new weapon
  (goto _label :!via `Reset`))

(event `self.DetectionSphere.OnComponentEndOverlap`
  (params (OverlappedComponent :type "PrimitiveComponent Object Reference") (OtherActor :type "Actor Object Reference") (OtherComp :type "PrimitiveComponent Object Reference") (OtherBodyIndex :type Integer))
  ;[1 1 1] Detect if player is picking up the new weapon
  (`KismetSystemLibrary.Delay` 0.2)
  (if (`KismetSystemLibrary.DoesImplementInterface` OtherActor "/Game/Blueprints/BPI/Player/BPI_Player.BPI_Player_C")
    (set `self.justSpawned` false)
    (`self.ResetPickUp`) ; can pick up again a new weapon
  ))

(fn `UserConstructionScript`
  (`SphereComponent.SetSphereRadius` (`self.DetectionSphere`) (`/Game/_Manager/InGame/DataAsset/BP/BP_GPE_DA.WeaponPickUpRadius` (`self.dataAsset`)) true)
  (switch `/Game/Blueprints/Enums/Enum_WeaponType` (`self.weaponType`)
    (:`NewEnumerator0`
      (`StaticMeshComponent.SetStaticMesh` (`self.WeaponMesh`) (`|GetArrayItem` (`self.allMeshes`))))
    (:`NewEnumerator1`
      (`StaticMeshComponent.SetStaticMesh` (`self.WeaponMesh`) (`|GetArrayItem` (`self.allMeshes`) 1)))
    (:`NewEnumerator2`
      (`StaticMeshComponent.SetStaticMesh` (`self.WeaponMesh`) (`|GetArrayItem` (`self.allMeshes`) 2)))))