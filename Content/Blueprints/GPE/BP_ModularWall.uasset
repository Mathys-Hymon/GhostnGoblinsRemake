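; Spline-driven modular wall actor that builds a wall topped with spears, side supports and end pillars in its construction script.
; Spline mesh segments sized from the wall mesh bounds follow the optionally looped spline, with optional pillars at open ends.
; Supports and spears are spaced by per-1000-unit densities, with supports optional on each side, mirrored by negative scale.
; Spears cycle through small, medium and big random mesh pools with random yaw and no collision.
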(fn `getSpearMesh`
  (returns (mesh :type "StaticMesh Object Reference"))
  (locals (actualSpear :type Integer))
  (bind _outitem (`KismetArrayLibrary.Array_Random` (`self.spearsMediumMesh`)))
  (set `local.actualSpear` (`self.spearIndex`))
  (bind _result (`/Engine/EditorBlueprintResources/StandardMacros.IncrementInt` (`self.spearIndex`))
    (:`  `
      (if (> _result 3)
        (set `self.spearIndex` 0))
      (return (select `int` (`local.actualSpear`) :`0` (`KismetArrayLibrary.Array_Random` (`self.spearsSmallMesh`)) :`1` _outitem :`2` (`KismetArrayLibrary.Array_Random` (`self.spearsBigMesh`)) :`3` _outitem)))))

(fn `UserConstructionScript`
  (bind _spline (`self.Spline`))
  (bind _spline_2 (`self.Spline`))
  (bind _spline_3 (`self.Spline`))
  (bind _spline_4 (`self.Spline`))
  (bind (_supportoffset_x _supportoffset_y _supportoffset_z) (`KismetMathLibrary.BreakVector` (`self.supportOffset`)))
  (bind _spline_5 (`self.Spline`))
  (bind (_supportoffset_x_2 _supportoffset_y_2 _supportoffset_z_2) (`KismetMathLibrary.BreakVector` (`self.supportOffset`)))
  (bind _spline_6 (`self.Spline`))
  (bind _returnvalue (`SplineComponent.GetNumberOfSplinePoints` (`self.Spline`)))
  (bind _returnvalue_2 (`SplineComponent.GetRotationAtSplinePoint` _spline 0 "Local"))
  (bind (_returnvalue_min _returnvalue_max) (break `Box` (`StaticMesh.GetBoundingBox` (`self.wallMesh`))))
  (bind _returnvalue_3 (`SplineComponent.GetRotationAtSplinePoint` _spline_2 _returnvalue "Local"))
  (bind (_returnvalue_min_2 _returnvalue_max_2) (break `Box` (`StaticMesh.GetBoundingBox` (`|GetArrayItem` (`self.spearsSmallMesh`)))))
  (bind _returnvalue_x (`KismetMathLibrary.BreakVector` (+ (`KismetMathLibrary.Vector_GetAbs` _returnvalue_min) (`KismetMathLibrary.Vector_GetAbs` _returnvalue_max))))
  (bind _returnvalue_x_2 (`KismetMathLibrary.BreakVector` (+ (`KismetMathLibrary.Vector_GetAbs` _returnvalue_min_2) (`KismetMathLibrary.Vector_GetAbs` _returnvalue_max_2))))
  (bind _returnvalue_4 (- (`KismetMathLibrary.FTrunc` (- (* (/ (`self.spearsAmount`) 1000) (`SplineComponent.GetSplineLength` (`self.Spline`))) 1.0)) 2))
  (`KismetSystemLibrary.FlushPersistentDebugLines`)
  (`SplineComponent.SetClosedLoop` (`self.Spline`) (`self.loop`) true)
  (set `self.xFenceLength` _returnvalue_x_2)
  (set `self.xLength` _returnvalue_x)
  (`|ExecutionSequence`
    (:`then_0`
      (for _index (range 1 (+ (`KismetMathLibrary.FTrunc` (- (* (/ (`self.supportAmount`) 1000) (`SplineComponent.GetSplineLength` (`self.Spline`))) 1.0)) 1))
        (`KismetSystemLibrary.PrintString` "Hello")
        (`|ExecutionSequence`
          (:`then_0`
            (if (`self.supportSide2`)
              (bind _returnvalue_5 (`SplineComponent.GetRotationAtDistanceAlongSpline` (`self.Spline`) (/ (* _index (`SplineComponent.GetSplineLength` (`self.Spline`))) (* (/ (`self.supportAmount`) 1000) (`SplineComponent.GetSplineLength` (`self.Spline`)))) "Local"))
              (bind _returnvalue_6 (`AddComponent|NODE_AddStaticMeshComponent-5` :`RelativeTransform` (`KismetMathLibrary.MakeTransform` (+ (* (`KismetMathLibrary.GetForwardVector` _returnvalue_5) _supportoffset_x) (* (`KismetMathLibrary.GetRightVector` _returnvalue_5) _supportoffset_y) (`KismetMathLibrary.MakeVector` 0.0 0.0 _supportoffset_z) (`SplineComponent.GetLocationAtDistanceAlongSpline` _spline_6 (/ (* _index (`SplineComponent.GetSplineLength` _spline_6)) (* (/ (`self.supportAmount`) 1000) (`SplineComponent.GetSplineLength` (`self.Spline`)))) "Local")) (`KismetMathLibrary.ComposeRotators` _returnvalue_5 (struct :`Yaw` 90.0)) (-1.0 -1.0 1.0))))
              (`StaticMeshComponent.SetStaticMesh` _returnvalue_6 (`self.supportMesh`))
              (`PrimitiveComponent.SetCollisionEnabled` _returnvalue_6 "QueryAndPhysics")))
          (:`then_1`
            (if (`self.supportSide1`)
              (bind _returnvalue_7 (`SplineComponent.GetRotationAtDistanceAlongSpline` (`self.Spline`) (/ (* _index (`SplineComponent.GetSplineLength` (`self.Spline`))) (* (/ (`self.supportAmount`) 1000) (`SplineComponent.GetSplineLength` (`self.Spline`)))) "Local"))
              (bind _returnvalue_8 (`AddComponent|NODE_AddStaticMeshComponent-4` :`RelativeTransform` (`KismetMathLibrary.MakeTransform` (+ (* (`KismetMathLibrary.GetForwardVector` _returnvalue_7) _supportoffset_x_2) (* (`KismetMathLibrary.GetRightVector` _returnvalue_7) _supportoffset_y_2) (`KismetMathLibrary.MakeVector` 0.0 0.0 _supportoffset_z_2) (`SplineComponent.GetLocationAtDistanceAlongSpline` _spline_5 (/ (* _index (`SplineComponent.GetSplineLength` _spline_5)) (* (/ (`self.supportAmount`) 1000) (`SplineComponent.GetSplineLength` (`self.Spline`)))) "Local")) (`KismetMathLibrary.ComposeRotators` _returnvalue_7 (struct :`Yaw` 90.0)))))
              (`StaticMeshComponent.SetStaticMesh` _returnvalue_8 (`self.supportMesh`))
              (`PrimitiveComponent.SetCollisionEnabled` _returnvalue_8 "QueryAndPhysics"))))))
    (:`then_1`
      (for _index_2 (range 1 (+ _returnvalue_4 1))
        (bind _returnvalue_9 (`AddComponent|NODE_AddStaticMeshComponent-6` :`RelativeTransform` (`KismetMathLibrary.MakeTransform` (+ (`SplineComponent.GetLocationAtDistanceAlongSpline` _spline_3 (/ (* _index_2 (`SplineComponent.GetSplineLength` _spline_3)) (`KismetMathLibrary.FTrunc` (- (* (/ (`self.spearsAmount`) 1000) (`SplineComponent.GetSplineLength` (`self.Spline`))) 1.0))) "Local") (`KismetMathLibrary.MakeVector` 0.0 0.0 (* (.z (`.BoxExtent` (`KismetMathLibrary.BreakBoxSphereBounds` (`StaticMesh.GetBounds` (`self.wallMesh`))))) 1.9))) (`KismetMathLibrary.ComposeRotators` (`SplineComponent.GetRotationAtDistanceAlongSpline` (`self.Spline`) (/ (* _index_2 (`SplineComponent.GetSplineLength` (`self.Spline`))) _returnvalue_4) "Local") (`KismetMathLibrary.MakeRotator` 0.0 0.0 (`KismetMathLibrary.RandomFloatInRange` 0.0 359.0))))))
        (bind _mesh (`self.getSpearMesh`))
        (`StaticMeshComponent.SetStaticMesh` _returnvalue_9 _mesh)
        (`PrimitiveComponent.SetCollisionEnabled` _returnvalue_9 "NoCollision")))
    (:`then_2`
      (for _index_3 (range (+ (`KismetMathLibrary.FTrunc` (/ (`SplineComponent.GetSplineLength` (`self.Spline`)) (`self.xLength`))) 1))
        (bind _returnvalue_10 (`AddComponent|NODE_AddSplineMeshComponent-2`))
        (`PrimitiveComponent.SetCollisionEnabled` _returnvalue_10 "QueryAndPhysics")
        (`SplineMeshComponent.SetForwardAxis` _returnvalue_10 "X" true)
        (`SplineMeshComponent.SetForwardAxis` _returnvalue_10 "X" true)
        (`StaticMeshComponent.SetStaticMesh` _returnvalue_10 (`self.wallMesh`))
        (bind _returnvalue_11 (* _index_3 (`self.xLength`)))
        (bind _returnvalue_12 (* (+ _index_3 1) (`self.xLength`)))
        (`SplineMeshComponent.SetStartAndEnd` _returnvalue_10 (- (`SplineComponent.GetLocationAtDistanceAlongSpline` _spline_4 _returnvalue_11 "Local") (* (`KismetMathLibrary.GetForwardVector` (`SplineComponent.GetRotationAtDistanceAlongSpline` _spline_4 _returnvalue_11 "Local")) 0.25)) (`KismetMathLibrary.ClampVectorSize` (`SplineComponent.GetTangentAtDistanceAlongSpline` _spline_4 _returnvalue_11 "Local") 0.0 (`self.xLength`)) (`SplineComponent.GetLocationAtDistanceAlongSpline` _spline_4 _returnvalue_12 "Local") (`KismetMathLibrary.ClampVectorSize` (`SplineComponent.GetTangentAtDistanceAlongSpline` _spline_4 _returnvalue_12 "Local") 0.0 (`self.xLength`)) true))
      (if (not (`self.loop`))
        (`|ExecutionSequence`
          (:`then_0`
            (if (`self.pillarLeft`)
              (bind _returnvalue_13 (`AddComponent|NODE_AddStaticMeshComponent-2` :`RelativeTransform` (`KismetMathLibrary.MakeTransform` (- (`SplineComponent.GetLocationAtSplinePoint` _spline_2 _returnvalue "Local") (* (`KismetMathLibrary.GetForwardVector` _returnvalue_3) 4.0)) _returnvalue_3)))
              (`StaticMeshComponent.SetStaticMesh` _returnvalue_13 (`self.pillarMesh`))))
          (:`then_1`
            (if (`self.pillarRight`)
              (bind _returnvalue_14 (`AddComponent|NODE_AddStaticMeshComponent-3` :`RelativeTransform` (`KismetMathLibrary.MakeTransform` (- (`SplineComponent.GetLocationAtSplinePoint` _spline 0 "Local") (* (`KismetMathLibrary.GetForwardVector` _returnvalue_2) 20.0)) _returnvalue_2)))
              (`StaticMeshComponent.SetStaticMesh` _returnvalue_14 (`self.pillarMesh`)))))))))