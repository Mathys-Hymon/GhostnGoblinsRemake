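; BP_Checkpoint is a checkpoint trigger that registers itself as the active checkpoint and can grant the player a life.
; Both begin and end overlap of its box collider by the player pawn send the actor and its index to the Game Instance via interface messages.
; If GiveHealth is set, a DoOnce limits the life gain to one time.
; The Construction Script resets actor scale and sizes and raises the collider from the Size variable.
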(event `self.CheckpointCollider.OnComponentEndOverlap`
  (params (OverlappedComponent :type "PrimitiveComponent Object Reference") (OtherActor :type "Actor Object Reference") (OtherComp :type "PrimitiveComponent Object Reference") (OtherBodyIndex :type Integer))
  (bind _returnvalue (`GameplayStatics.GetGameInstance`))
  (if (or (== OtherActor (`GameplayStatics.GetPlayerPawn` 0)) (== (stale `self.CheckpointCollider.OnComponentBeginOverlap` OtherActor) (`GameplayStatics.GetPlayerPawn` 0))) :!label _label
    (message `/Game/Blueprints/BPI/GameInstance/BPI_GameInstance.SetCheckpoint` _returnvalue self)
    (message `/Game/Blueprints/BPI/GameInstance/BPI_GameInstance.SetCurrentCheckpointID` _returnvalue (`self.checkPointIndex`))
    (if (`self.giveHealth`)
      (`/Engine/EditorBlueprintResources/StandardMacros.DoOnce` false
        (:`Completed`
          (message `/Game/Blueprints/BPI/Player/BPI_Player.GainLife` (`GameplayStatics.GetPlayerPawn` 0)))))))

(event `self.CheckpointCollider.OnComponentBeginOverlap`
  (params (OverlappedComponent :type "PrimitiveComponent Object Reference") (OtherActor :type "Actor Object Reference") (OtherComp :type "PrimitiveComponent Object Reference") (OtherBodyIndex :type Integer) (bFromSweep :type Boolean) (SweepResult :type "HitResult Structure (by ref)"))
  (goto _label))

(fn `UserConstructionScript`
  (bind (_size_x _size_y _size_z) (`KismetMathLibrary.BreakVector` (`self.size`)))
  (`self.SetActorScale3D` (1.0 1.0 1.0))
  (`SceneComponent.K2_SetRelativeLocation` (`self.CheckpointCollider`) (`KismetMathLibrary.MakeVector` 0.0 0.0 _size_z) false true)
  (`BoxComponent.SetBoxExtent` (`self.CheckpointCollider`) (`self.size`) true))