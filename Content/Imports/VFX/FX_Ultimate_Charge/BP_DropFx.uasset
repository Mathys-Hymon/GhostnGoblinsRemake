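; BP_DropFx is a short-lived Niagara effect actor from the ultimate charge VFX set.
; On BeginPlay it passes a particle count and the player pawn to the Niagara system and activates it.
; Each tick it feeds the system a point above the player character's mesh as ActorLocation.
; After a fixed delay it deactivates the system and destroys itself a tick later.
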(event `self.ReceiveBeginPlay`
  (bind _niagara (`self.Niagara`))
  (`NiagaraComponent.SetVariableInt` _niagara "particleAmount" (`self.particleAmount`))
  (`NiagaraComponent.SetVariableObject` _niagara "PlayerRef" (`GameplayStatics.GetPlayerPawn` 0))
  (`ActorComponent.SetActive` (`self.Niagara`) true true)
  (`KismetSystemLibrary.Delay` 25.0)
  (`ActorComponent.SetActive` (`self.Niagara`) false true)
  (`KismetSystemLibrary.DelayUntilNextTick`)
  (`self.K2_DestroyActor`))

(event `self.ReceiveTick`
  (params (DeltaSeconds :type "Float (single-precision)"))
  (`NiagaraComponent.SetVariableVec3` (`self.Niagara`) "ActorLocation" (+ (`SceneComponent.K2_GetComponentLocation` (`Character.Mesh` (`GameplayStatics.GetPlayerCharacter` 0))) (0.0 0.0 100.0))))

(fn `UserConstructionScript`)