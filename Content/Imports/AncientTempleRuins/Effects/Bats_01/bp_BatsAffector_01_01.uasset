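; Actor Blueprint that feeds a target position to a set of bat particle emitters, apparently so the bats react to that point.
; Each tick and on construction, it writes a "Position" vector parameter to every particle system in its Particles array.
; The position is the affector's own location in Debug mode, otherwise the Location of the first bp_FireGuide_01_01 found by a tag search.
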(event `self.ReceiveTick`
  (params (DeltaSeconds :type "Float (single-precision)"))
  (`self.SetPosition`))

(fn `SetPosition`
  (if (`self.Debug`)
    (for _array_element (`self.Particles`)
      (`FXSystemComponent.SetVectorParameter` (`Emitter.ParticleSystemComponent` _array_element) "Position" (`self.K2_GetActorLocation`)))
    (else
      (bind _outactors (`GameplayStatics.GetAllActorsWithTag` (`self.ActorToTraceTag`)))
      (if (> (`KismetArrayLibrary.Array_Length` _outactors) 0)
        (if (> (`KismetArrayLibrary.Array_Length` (`self.Particles`)) 0)
          (bind _asbp_fire_guide_01_01 (cast `/Game/Imports/AncientTempleRuins/Effects/FireGuide_01/bp_FireGuide_01_01` (`|GetArrayItem` _outactors)))
          (for _array_element_2 (`self.Particles`)
            (`FXSystemComponent.SetVectorParameter` (`Emitter.ParticleSystemComponent` _array_element_2) "Position" (`/Game/Imports/AncientTempleRuins/Effects/FireGuide_01/bp_FireGuide_01_01.Location` _asbp_fire_guide_01_01))))))))

(fn `UserConstructionScript`
  (`self.SetPosition`))