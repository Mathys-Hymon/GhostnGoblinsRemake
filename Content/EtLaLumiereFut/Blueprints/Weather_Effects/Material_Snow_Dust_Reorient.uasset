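; Scene component that keeps the snow/dust material's up vector aligned to world up as the component rotates, via the "SWE Snow Up Vector" parameter on dynamic material instances.
; Startup runs a tick after BeginPlay, sets the initial vector in local space and starts a looping timer checking angular drift against a threshold.
; Past it, ReorientSnow re-arms its own timer, stepping toward the target at limited angular speed until within one degree.
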(event `self.ReceiveBeginPlay`
  (`KismetSystemLibrary.K2_SetTimerForNextTick` null "Startup"))

(fn `Check for Snow Reorient`
  (if (not (`self.Reorienting Snow`))
    (if (> (`KismetMathLibrary.DegAcos` (`KismetMathLibrary.Dot_VectorVector` (`self.Snow Up Vector`) (`KismetMathLibrary.LessLess_VectorRotator` (0.0 0.0 1.0) (`self.K2_GetComponentRotation`)))) (`self.Reorientation Needed Threshold`))
      (`self.Reorient Snow`))))

(fn `Reorient Snow`
  (bind _snow_up_vector (`self.Snow Up Vector`))
  (bind _returnvalue (`KismetMathLibrary.LessLess_VectorRotator` (0.0 0.0 1.0) (`self.K2_GetComponentRotation`)))
  (set `self.Snow Up Vector` (`KismetMathLibrary.GetUpVector` (`KismetMathLibrary.RLerp` (`KismetMathLibrary.MakeRotFromZ` _snow_up_vector) (`KismetMathLibrary.MakeRotFromZ` _returnvalue) (`KismetMathLibrary.FClamp` (`KismetMathLibrary.SafeDivide` (* (`KismetMathLibrary.FMax` (`GameplayStatics.GetWorldDeltaSeconds`) (`self.Snow/Dust Reorient Update Period`)) (`self.Snow/Dust Reorient Speed`)) (`KismetMathLibrary.DegAcos` (`KismetMathLibrary.Dot_VectorVector` _snow_up_vector _returnvalue)))) true)))
  (`MaterialInstanceDynamic.SetVectorParameterValue` (`self.Dynamic Material Instances`) "SWE Snow Up Vector" (`KismetMathLibrary.Conv_VectorToLinearColor` (`KismetMathLibrary.Normal` (`self.Snow Up Vector`))))
  (if (> (`KismetMathLibrary.DegAcos` (`KismetMathLibrary.Dot_VectorVector` (`self.Snow Up Vector`) (`KismetMathLibrary.LessLess_VectorRotator` (0.0 0.0 1.0) (`self.K2_GetComponentRotation`)))) 1.0)
    (`KismetSystemLibrary.K2_SetTimer` null "Reorient Snow" (`self.Snow/Dust Reorient Update Period`))
    (set `self.Reorienting Snow` true)
    (else
      (set `self.Reorienting Snow` false))))

(fn `Startup`
  (set `self.Snow Up Vector` (`KismetMathLibrary.LessLess_VectorRotator` (0.0 0.0 1.0) (`self.K2_GetComponentRotation`)))
  (`MaterialInstanceDynamic.SetVectorParameterValue` (`self.Dynamic Material Instances`) "SWE Snow Up Vector" (`KismetMathLibrary.Conv_VectorToLinearColor` (`KismetMathLibrary.Normal` (`self.Snow Up Vector`))))
  (`KismetSystemLibrary.K2_SetTimer` null "Check for Snow Reorient" (`self.Snow/Dust Reorient Check Period`) true))