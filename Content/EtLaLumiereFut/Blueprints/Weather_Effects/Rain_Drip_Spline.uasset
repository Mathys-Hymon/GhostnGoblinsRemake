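; Spline actor for Ultra Dynamic Weather that emits Niagara rain drips and splashes along a placed path.
; On construction and once at startup, it rebuilds one emitter per segment, converting tangents to Bézier handles.
; Segment length scales spawning and collision point count, while sampled fixed bounds extend downward for falling drips.
; Length-based spawn rate feeds either rain and wetness channels or a constant one when ignoring weather.
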(event `/Game/EtLaLumiereFut/Blueprints/System/UDW_Startup_Interface.UDW Starting Up`
  (params (UDW :type "/Game/EtLaLumiereFut/Blueprints/Ultra_Dynamic_Weather Object Reference"))
  (`/Engine/EditorBlueprintResources/StandardMacros.DoOnce` false :!label _label
    (:`Completed`
      (`self.Create Curve Data`)
      (`self.Update Static Niagara Parameters`))))

(event `self.ReceiveBeginPlay`
  (goto _label))

(fn `Create Curve Data`
  (locals (`Number of Segments` :type Integer :default 0) (`Current Emitter` :type "NiagaraComponent Object Reference") (`Segment Index` :type Integer) (`Segment Bounds Min` :type "Vector Structure") (`Segment Bounds Max` :type "Vector Structure"))
  (bind _drip_emitters (`self.Drip Emitters`))
  (bind _spline (`self.Spline`))
  (bind _segment_index (`local.Segment Index`))
  (bind _spline_2 (`self.Spline`))
  (bind _segment_index_2 (`local.Segment Index`))
  (bind _returnvalue (`KismetMathLibrary.SelectFloat` 0.0 (`self.Spawn Rate`) (`self.Ignore Weather State`)))
  (bind _returnvalue_2 (`SplineComponent.GetLocationAtSplinePoint` (`self.Spline`) (`local.Segment Index`) "Local"))
  (bind _returnvalue_3 (`SplineComponent.GetLocationAtSplinePoint` (`self.Spline`) (+ (`local.Segment Index`) 1) "Local"))
  (bind _returnvalue_4 (- (`SplineComponent.GetDistanceAlongSplineAtSplinePoint` _spline_2 (+ _segment_index_2 1)) (`SplineComponent.GetDistanceAlongSplineAtSplinePoint` _spline_2 _segment_index_2)))
  (`SplineComponent.SetClosedLoop` (`self.Spline`) (`self.Closed Spline Loop`) true)
  (`ActorComponent.K2_DestroyComponent` _drip_emitters)
  (`KismetArrayLibrary.Array_Clear` _drip_emitters)
  (set `local.Number of Segments` (`SplineComponent.GetNumberOfSplineSegments` (`self.Spline`)))
  (for _index (range (`local.Number of Segments`))
    (set `local.Segment Index` _index)
    (bind _returnvalue_5 (`AddComponent|NODE_AddNiagaraComponent-3`))
    (bind _output_get (set `local.Current Emitter` _returnvalue_5))
    (`KismetArrayLibrary.Array_Add` (`self.Drip Emitters`) _output_get)
    (`FXSystemComponent.SetVectorParameter` (`local.Current Emitter`) "Curve Position A" _returnvalue_2)
    (`FXSystemComponent.SetVectorParameter` (`local.Current Emitter`) "Curve Handle A" (+ _returnvalue_2 (/ (`SplineComponent.GetLeaveTangentAtSplinePoint` (`self.Spline`) (`local.Segment Index`) "Local") 3.0)))
    (`FXSystemComponent.SetVectorParameter` (`local.Current Emitter`) "Curve Position B" _returnvalue_3)
    (`FXSystemComponent.SetVectorParameter` (`local.Current Emitter`) "Curve Handle B" (+ _returnvalue_3 (* (/ (`SplineComponent.GetArriveTangentAtSplinePoint` (`self.Spline`) (+ (`local.Segment Index`) 1) "Local") 3.0) -1.0)))
    (`FXSystemComponent.SetFloatParameter` (`local.Current Emitter`) "Spawn Distance Scale" (/ _returnvalue_4 (`SplineComponent.GetSplineLength` _spline_2)))
    (`FXSystemComponent.SetIntParameter` (`local.Current Emitter`) "Collision Point Count" (`KismetMathLibrary.FCeil` (`KismetMathLibrary.FClamp` _returnvalue_4 10.0 1000.0)))
    (set `local.Segment Bounds Min` (0.0 0.0 0.0))
    (set `local.Segment Bounds Max` (0.0 0.0 0.0))
    (for _index_2 (range 5)
      (bind _returnvalue_6 (`SplineComponent.GetLocationAtDistanceAlongSpline` (`self.Spline`) (`KismetMathLibrary.Lerp` (`SplineComponent.GetDistanceAlongSplineAtSplinePoint` _spline _segment_index) (`SplineComponent.GetDistanceAlongSplineAtSplinePoint` _spline (+ _segment_index 1)) (/ (`KismetMathLibrary.Conv_IntToDouble` _index_2) 4.0)) "Local"))
      (set `local.Segment Bounds Min` (`KismetMathLibrary.Vector_ComponentMin` _returnvalue_6 (`local.Segment Bounds Min`)))
      (set `local.Segment Bounds Max` (`KismetMathLibrary.Vector_ComponentMax` _returnvalue_6 (`local.Segment Bounds Max`))))
    (`FXSystemComponent.SetFloatParameter` (`local.Current Emitter`) "Spline Radius" (`KismetMathLibrary.Vector_Distance` (`local.Segment Bounds Min`) (`local.Segment Bounds Max`)))
    (set `local.Segment Bounds Min` (- (`local.Segment Bounds Min`) (0.0 0.0 5000.0)))
    (`NiagaraComponent.SetSystemFixedBounds` (`local.Current Emitter`) (`KismetMathLibrary.MakeBox` (`local.Segment Bounds Min`) (`local.Segment Bounds Max`))))
  (`FXSystemComponent.SetFloatParameter` (`self.Drip Emitters`) "Raining Spawn Count" _returnvalue)
  (`FXSystemComponent.SetFloatParameter` (`self.Drip Emitters`) "Wet Spawn Count" (* _returnvalue (`self.Drip with Material Wetness`)))
  (`FXSystemComponent.SetFloatParameter` (`self.Drip Emitters`) "Constant Spawn Count" (`KismetMathLibrary.SelectFloat` (`self.Spawn Rate`) 0.0 (`self.Ignore Weather State`)))
  (`FXSystemComponent.SetFloatParameter` (`self.Drip Emitters`) "Curl Noise Force" (`self.Curl Noise Force`))
  (bind _returnvalue_7 (`GameplayStatics.GetActorOfClass` "/Game/EtLaLumiereFut/Blueprints/Ultra_Dynamic_Sky.Ultra_Dynamic_Sky_C"))
  (`/Engine/EditorBlueprintResources/StandardMacros.IsValid` _returnvalue_7
    (:`Is Valid`
      (`NiagaraComponent.SetVariableMaterial` (`self.Drip Emitters`) "Splash Material" (select `/Game/EtLaLumiereFut/Blueprints/Enum/UDS_RenderingFeatureLevel` (`/Game/EtLaLumiereFut/Blueprints/Ultra_Dynamic_Sky.Feature Level` _returnvalue_7) :`NewEnumerator0` "/Game/EtLaLumiereFut/Materials/Weather/Splash_ParticleMat.Splash_ParticleMat" :`NewEnumerator1` "/Game/EtLaLumiereFut/Materials/Weather/Splash_ParticleMat_Translucent.Splash_ParticleMat_Translucent" :`NewEnumerator2` "/Game/EtLaLumiereFut/Materials/Weather/Splash_ParticleMat_Translucent.Splash_ParticleMat_Translucent" :!type "MaterialInterface Object Reference")))))

(fn `Spawn Rate`
  (returns (Out :type "Float (double-precision)"))
  (return (+ (* (`self.Spawn Rate Per Meter`) (/ (`SplineComponent.GetSplineLength` (`self.Spline`)) 100.0)) (`self.Extra Spawn Rate`))))

(fn `Update Static Niagara Parameters`
  (`FXSystemComponent.SetFloatParameter` (`self.Drip Emitters`) "Splash Percentage" (`self.Splash Frequency`))
  (`FXSystemComponent.SetFloatParameter` (`self.Drip Emitters`) "Collision Head Start" (`self.Collision Line Trace Head Start`)))

(fn `UserConstructionScript`
  (set `self.Refresh` false)
  (`self.Create Curve Data`)
  (`self.Update Static Niagara Parameters`))

(fn `📘 Rain Drip Spline`
  (bind _returnvalue (`GameplayStatics.GetActorOfClass` "/Game/EtLaLumiereFut/Blueprints/Ultra_Dynamic_Weather.Ultra_Dynamic_Weather_C"))
  (`/Engine/EditorBlueprintResources/StandardMacros.IsValid` _returnvalue
    (:`Is Valid`
      (`/Game/EtLaLumiereFut/Blueprints/Ultra_Dynamic_Weather.Open Editor Readme Entry` _returnvalue "RainDripSpline"))))