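; Radial Storm is a localized weather actor for Ultra Dynamic Sky and Weather, with Niagara fog, lightning, shadow and thunder audio.
; It registers with both managers, supplying radius, alpha and weather state for cloud coverage, weather and material effects.
; Timed fades and moves enable interval ticking, refreshing manager render targets only past distance or alpha thresholds.
; The authority drives movement and sends alpha to clients; fade-out destroys the actor.
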(event `self.ReceiveBeginPlay`
  ;[0.365 0.4815 1] Begin Play
  (`self.Get UDS and UDW`)
  (`|ExecutionSequence`
    (:`then_0`
      (`/Engine/EditorBlueprintResources/StandardMacros.IsValid` (`self.UDS`)
        (:`Is Valid`
          (`KismetArrayLibrary.Array_AddUnique` (`/Game/EtLaLumiereFut/Blueprints/Ultra_Dynamic_Sky.Radial Storms` (`self.UDS`)) self))))
    (:`then_1`
      (`SceneComponent.SetVisibility` (`self.Niagara System`) false false)
      (`self.Check Sky Mode for Visibility`)
      (`KismetSystemLibrary.K2_SetTimerForNextTick` null "Second Frame Startup"))))

(event `self.ReceiveEndPlay`
  (params (EndPlayReason :type "EEndPlayReason Enum" :default "Destroyed"))
  ;[0.2148 0.5 0.1797 1 35] End Play
  (`|ExecutionSequence`
    (:`then_0`
      (bind _returnvalue (`GameplayStatics.GetActorOfClass` "/Game/EtLaLumiereFut/Blueprints/Ultra_Dynamic_Sky.Ultra_Dynamic_Sky_C"))
      (`/Engine/EditorBlueprintResources/StandardMacros.IsValid` _returnvalue
        (:`Is Valid`
          (`KismetArrayLibrary.Array_RemoveItem` (`/Game/EtLaLumiereFut/Blueprints/Ultra_Dynamic_Sky.Radial Storms` (`self.UDS`)) self)
          (`KismetSystemLibrary.K2_SetTimerForNextTick` (`self.UDS`) "Update Painted Cloud Coverage Target"))))
    (:`then_1`
      (bind _returnvalue_2 (`GameplayStatics.GetActorOfClass` "/Game/EtLaLumiereFut/Blueprints/Ultra_Dynamic_Weather.Ultra_Dynamic_Weather_C"))
      (`/Engine/EditorBlueprintResources/StandardMacros.IsValid` _returnvalue_2
        (:`Is Valid`
          (message `/Game/EtLaLumiereFut/Blueprints/Weather_Effects/System/Ultra_Dynamic_Weather_Interface.Report Removed Radial Storm` _returnvalue_2 self))))))

(event `self.ReceiveTick`
  (params (DeltaSeconds :type "Float (single-precision)"))
  (`|ExecutionSequence` :!label _label
    (:`then_0`
      (`|ExecutionSequence`
        (:`then_0`
          ;[0.2842 0.2266 1] Fade in/out Alpha
          (if (or (`self.Fading In`) (`self.Fading Out`))
            (bind _output_get (set `self.Storm Alpha` (`KismetMathLibrary.FClamp` (+ (`self.Storm Alpha`) (* (- (`KismetSystemLibrary.GetGameTimeInSeconds`) (`self.Last Tick Time`)) (`self.Fade Speed`) (`KismetMathLibrary.SelectFloat` 1.0 -1.0 (`self.Fading In`)))))))
            (if (== _output_get (`KismetMathLibrary.SelectFloat` 1.0 0.0 (`self.Fading In`)))
              (set `self.Fading In` false)
              (if (`self.Fading Out`)
                (`KismetSystemLibrary.K2_SetTimerForNextTick` null "Destroy")
                (elif (not (`self.Moving`))
                  (`self.SetActorTickEnabled` false))))))
        (:`then_1`
          ;[1 0.5036 0.3015] Move Location
          (if (`self.Moving`)
            (`/Engine/EditorBlueprintResources/ActorMacros.Switch Has Authority`
              (:`Authority`
                (`self.K2_SetActorLocation` (`KismetMathLibrary.VLerp` (`self.Starting Location`) (`self.Movement Target`) (`KismetMathLibrary.FClamp` (/ (`KismetSystemLibrary.K2_GetTimerElapsedTimeHandle` (`self.Movement Timer`)) (`self.Move Duration`)))))))))))
    (:`then_1`
      (`self.Check to Apply Animation Changes`)
      (set `self.Last Tick Time` (`KismetSystemLibrary.GetGameTimeInSeconds`)))))

(event `Force Tick`
  (goto _label))

(event `Client Storm Update`
  (params (Alpha :type "Float (double-precision)"))
  (`/Engine/EditorBlueprintResources/ActorMacros.Switch Has Authority`
    (:`Remote`
      (set `self.Storm Alpha` Alpha)
      (`self.Update Alpha`)
      (`self.Refresh Targets`))))

(fn `Apply Niagara Properties`
  (locals (`Rain/Snow Amount` :type "Float (double-precision)"))
  (bind _storm_weather (`self.Storm Weather`))
  (bind _storm_weather_2 (`self.Storm Weather`))
  (`|ExecutionSequence`
    (:`then_0`
      ;[1 0.575 0.3093 1 35] Fog Sprites
      (`FXSystemComponent.SetFloatParameter` (`self.Niagara System`) "Spawn Cylinder Height" (`self.Cylinder Height`))
      (`FXSystemComponent.SetFloatParameter` (`self.Niagara System`) "Fog Desaturate" (- 1.0 (`self.Fog Sprites Color Saturation`)))
      (`FXSystemComponent.SetFloatParameter` (`self.Niagara System`) "Fog Color Intensity" (* (`self.Fog Sprites Color Intensity`) (`KismetMathLibrary.MapRangeClamped` (`/Game/EtLaLumiereFut/Blueprints/Weather_Effects/System/UDS_Weather_Settings.Cloud Coverage` (`self.Storm Weather`)) 5.0 7.5 1.0 0.5)))
      (set `local.Rain/Snow Amount` (/ (`KismetMathLibrary.FMax` (`/Game/EtLaLumiereFut/Blueprints/Weather_Effects/System/UDS_Weather_Settings.Rain` _storm_weather_2) (`/Game/EtLaLumiereFut/Blueprints/Weather_Effects/System/UDS_Weather_Settings.Snow` _storm_weather_2)) 10.0))
      (`FXSystemComponent.SetFloatParameter` (`self.Niagara System`) "Rain/Snow Amount" (`local.Rain/Snow Amount`))
      (`FXSystemComponent.SetFloatParameter` (`self.Niagara System`) "Fog Alpha" (`self.Fog Sprites Opacity`))
      (`FXSystemComponent.SetFloatParameter` (`self.Niagara System`) "Fog Amount" (`KismetMathLibrary.FClamp` (`KismetMathLibrary.FMax` (`KismetMathLibrary.MapRangeClamped` (`/Game/EtLaLumiereFut/Blueprints/Weather_Effects/System/UDS_Weather_Settings.Fog` _storm_weather) 7.0 10.0 0.0 0.75) (`KismetMathLibrary.MapRangeClamped` (`/Game/EtLaLumiereFut/Blueprints/Weather_Effects/System/UDS_Weather_Settings.Dust` _storm_weather) 3.0 10.0 0.0 0.85) (* (`local.Rain/Snow Amount`) 0.85))))
      (`FXSystemComponent.SetFloatParameter` (`self.Niagara System`) "Far Fade Distance" (* (`self.Effects Fade Distance (km)`) 100000.0))
      (`FXSystemComponent.SetFloatParameter` (`self.Niagara System`) "Dust Alpha" (/ (`/Game/EtLaLumiereFut/Blueprints/Weather_Effects/System/UDS_Weather_Settings.Dust` (`self.Storm Weather`)) 10.0))
      (`FXSystemComponent.SetFloatParameter` (`self.Niagara System`) "Fog Sprite Scale" (`self.Fog Sprite Scale`))
      (`FXSystemComponent.SetIntParameter` (`self.Niagara System`) "Fog Sprite Count" (`self.Fog Sprite Count`))
      (`FXSystemComponent.SetFloatParameter` (`self.Niagara System`) "Fog Sprite Speed" (`self.Fog Sprite Movement Speed`))
      (`FXSystemComponent.SetVectorParameter` (`self.Niagara System`) "Dust Multiplier" (`KismetMathLibrary.VLerp` (1.0 1.0 1.0) (`KismetMathLibrary.Conv_LinearColorToVector` (`self.Dust Fog Color Multiplier`)) (/ (`/Game/EtLaLumiereFut/Blueprints/Weather_Effects/System/UDS_Weather_Settings.Dust` (`self.Storm Weather`)) 10.0)))
      (`NiagaraComponent.SetVariableMaterial` (`self.Niagara System`) "Fog Sprite Material" (select `bool` (`self.Fog Sprites Render Behind Clouds`) :`false` "/Game/EtLaLumiereFut/Materials/Weather/Radial_Storm_Fog_Particle.Radial_Storm_Fog_Particle" :`true` "/Game/EtLaLumiereFut/Materials/Weather/Radial_Storm_Fog_Particle_AboveClouds.Radial_Storm_Fog_Particle_AboveClouds" :!type "MaterialInterface Object Reference"))
      (`FXSystemComponent.SetBoolParameter` (`self.Niagara System`) "Mask Fog Above Clouds" (not (`self.Fog Sprites Render Behind Clouds`))))
    (:`then_1`
      ;[0.3511 0.4852 1 1 35] Lightning
      (`FXSystemComponent.SetFloatParameter` (`self.Niagara System`) "Lightning Spawn Rate" (`KismetMathLibrary.MapRangeClamped` (`/Game/EtLaLumiereFut/Blueprints/Weather_Effects/System/UDS_Weather_Settings.Thunder/Lightning` (`self.Storm Weather`)) 0.0 10.0 0.0 (`self.Lightning Spawn Rate`)))
      (`FXSystemComponent.SetFloatParameter` (`self.Niagara System`) "Rain Amount" (/ (`/Game/EtLaLumiereFut/Blueprints/Weather_Effects/System/UDS_Weather_Settings.Rain` (`self.Storm Weather`)) 10.0))
      (`FXSystemComponent.SetFloatParameter` (`self.Niagara System`) "Intensity Scale" (`self.Lightning Intensity`)))
    (:`then_2`
      ;[0.4532 1 0.6321 1 35] Shadow
      (`FXSystemComponent.SetFloatParameter` (`self.Niagara System`) "Shadow Alpha" (`KismetMathLibrary.MapRangeClamped` (`/Game/EtLaLumiereFut/Blueprints/Weather_Effects/System/UDS_Weather_Settings.Cloud Coverage` (`self.Storm Weather`)) 5.0 7.5 0.0 (`self.Ambient Light Shadow Intensity`))))))

(fn `Check Sky Mode for Visibility`
  (`/Engine/EditorBlueprintResources/StandardMacros.IsValid` (`self.UDS`)
    (:`Is Valid`
      (set `self.Effects Visible` (`|EnumEquality` (`/Game/EtLaLumiereFut/Blueprints/Ultra_Dynamic_Sky.Sky Mode` (`self.UDS`)) "NewEnumerator0")))))

(fn `Check to Apply Animation Changes`
  (`self.Update Alpha`)
  (if (or (> (`KismetMathLibrary.Vector_Distance` (`self.Last Updated Location`) (`self.K2_GetActorLocation`)) (`self.Movement Update Threshold`)) (> (`KismetMathLibrary.Abs` (- (`self.Last Updated Alpha`) (`self.Storm Alpha`))) (`self.Alpha Update Threshold`)))
    (set `self.Last Updated Alpha` (`self.Storm Alpha`))
    (set `self.Last Updated Location` (`self.K2_GetActorLocation`))
    (`self.Refresh Targets`)
    (`self.Client Storm Update` (`self.Storm Alpha`))))

(fn `Configure Thunder Sound`
  (set `AudioComponent.AttenuationOverrides` (make `SoundAttenuationSettings` :`StereoSpread` (`self.Outer Radius`) :`AttenuationShapeExtents` (`KismetMathLibrary.MakeVector` (`self.Outer Radius`)) :`FalloffDistance` (* (`self.Thunder Sounds Range (km)`) 100000.0)) (`self.Thunder Sound`)))

(fn `Destroy`
  (`self.K2_DestroyActor`))

(fn `End Movement`
  (`self.K2_SetActorLocation` (`self.Movement Target`))
  (set `self.Moving` false)
  (if (`KismetMathLibrary.BooleanNOR` (`self.Fading In`) (`self.Fading Out`))
    (`self.SetActorTickEnabled` false)))

(fn `Fade in Storm`
  (params (`Fade Duration` :type "Float (double-precision)" :default 100.0))
  (if (> `Fade Duration` 0.0)
    (set `self.Fade Speed` (/ 1.0 (`local.Fade Duration`)))
    (set `self.Storm Alpha` 0.0)
    (set `self.Fading In` true)
    (set `self.Fading Out` false)
    (`/Engine/EditorBlueprintResources/ActorMacros.Switch Has Authority`
      (:`Authority`
        (`self.Start Ticking`)))
    (else
      (set `self.Storm Alpha` 1.0)
      (set `self.Fading In` false)
      (set `self.Fading Out` false)
      (`self.Update Alpha`)
      (`self.Refresh Targets`)
      (`/Engine/EditorBlueprintResources/ActorMacros.Switch Has Authority`
        (:`Authority`
          (`self.Client Storm Update` (`self.Storm Alpha`)))))))

(fn `Fade Out Storm`
  (params (`Fade Duration` :type "Float (double-precision)" :default 100.0))
  (if (> `Fade Duration` 0.0)
    (set `self.Fade Speed` (/ 1.0 (`local.Fade Duration`)))
    (set `self.Fading In` false)
    (set `self.Fading Out` true)
    (`/Engine/EditorBlueprintResources/ActorMacros.Switch Has Authority`
      (:`Authority`
        (`self.Start Ticking`)))
    (else
      (set `self.Storm Alpha` 0.0)
      (set `self.Fading In` false)
      (set `self.Fading Out` false)
      (`self.Update Alpha`)
      (`self.Refresh Targets`)
      (`KismetSystemLibrary.K2_SetTimerForNextTick` null "Destroy"))))

(fn `Get Cloud Coverage Brush Data`
  (params (UDS :type "/Game/EtLaLumiereFut/Blueprints/Ultra_Dynamic_Sky Object Reference"))
  (returns (`Soft Fraction` :type "Float (double-precision)") (RGBA :type "LinearColor Structure") (`World Location` :type "Vector Structure") (Size :type "Float (double-precision)") (`UDS Coverage Level` :type "Float (double-precision)"))
  (set `self.UDS` UDS)
  (return (`self.Inner Radius Fraction`) (make `LinearColor` (.x (`CurveVector.GetVectorValue` (`self.Cloud Coverage RGB Curve`) (`/Game/EtLaLumiereFut/Blueprints/Weather_Effects/System/UDS_Weather_Settings.Cloud Coverage` (`self.Storm Weather`)))) (.y (`CurveVector.GetVectorValue` (`self.Cloud Coverage RGB Curve`) (`/Game/EtLaLumiereFut/Blueprints/Weather_Effects/System/UDS_Weather_Settings.Cloud Coverage` (`self.Storm Weather`)))) (.z (`CurveVector.GetVectorValue` (`self.Cloud Coverage RGB Curve`) (`/Game/EtLaLumiereFut/Blueprints/Weather_Effects/System/UDS_Weather_Settings.Cloud Coverage` (`self.Storm Weather`)))) (`self.Storm Alpha`)) (`self.K2_GetActorLocation`) (* (`self.Outer Radius`) 2.0) (`KismetMathLibrary.MapRangeClamped` (`/Game/EtLaLumiereFut/Blueprints/Weather_Effects/System/UDS_Weather_Settings.Cloud Coverage` (`self.Storm Weather`)) 0.0 10.0 0.0 3.0)))

(fn `Get Radial Storm Material Target Data`
  (returns (Draw :type Boolean) (Location :type "Vector Structure") (`Outer Radius` :type "Float (double-precision)") (`Soft Fraction` :type "Float (double-precision)") (Color :type "LinearColor Structure"))
  (return (`self.Apply Material State`) (`self.K2_GetActorLocation`) (`self.Outer Radius`) (`self.Inner Radius Fraction`) (`self.Material Target Color`)))

(fn `Get Radial Storm Weather Data`
  (returns (`World Location` :type "Vector Structure") (`Outer Radius` :type "Float (double-precision)") (`Inner Radius` :type "Float (double-precision)") (Alpha :type "Float (double-precision)") (`Weather State` :type "/Game/EtLaLumiereFut/Blueprints/Weather_Effects/System/UDS_Weather_Settings Object Reference") (`Affect Material State` :type Boolean))
  (bind _outer_radius (`self.Outer Radius`))
  (return (`self.K2_GetActorLocation`) _outer_radius (`KismetMathLibrary.Lerp` _outer_radius (* _outer_radius (`self.Inner Radius Fraction`)) 0.8) (`self.Storm Alpha`) (`self.Storm Weather`) (`self.Apply Material State`)))

(fn `Get UDS and UDW`
  (bind _returnvalue (`GameplayStatics.GetActorOfClass` "/Game/EtLaLumiereFut/Blueprints/Ultra_Dynamic_Sky.Ultra_Dynamic_Sky_C"))
  (`/Engine/EditorBlueprintResources/StandardMacros.IsValid` _returnvalue
    (:`Is Valid`
      (set `self.UDS` _returnvalue)
      (bind _returnvalue_2 (`GameplayStatics.GetActorOfClass` "/Game/EtLaLumiereFut/Blueprints/Ultra_Dynamic_Weather.Ultra_Dynamic_Weather_C"))
      (`/Engine/EditorBlueprintResources/StandardMacros.IsValid` _returnvalue_2
        (:`Is Valid`
          (set `self.UDW` _returnvalue_2))))))

(fn `Latent Fade Out`
  (`self.Fade Out Storm` (`self.Latent Fade Duration`)))

(fn `Move Storm Over Time`
  (params (`Target Location` :type "Vector Structure") (`Movement Duration` :type "Float (double-precision)" :default 300.0) (`Fade Out by End of Movement` :type Boolean) (`Fade Out Duration` :type "Float (double-precision)" :default 100.0))
  (`/Engine/EditorBlueprintResources/ActorMacros.Switch Has Authority`
    (:`Authority`
      (set `self.Move Duration` `Movement Duration`)
      (set `self.Latent Fade Duration` `Fade Out Duration`)
      (bind _output_get (set `self.Starting Location` (`self.K2_GetActorLocation`)))
      (set `self.Movement Target` (`KismetMathLibrary.MakeVector` (.x `Target Location`) (.y `Target Location`) (.z _output_get)))
      (set `self.Moving` true)
      (`self.Start Ticking`)
      (bind _returnvalue (`KismetSystemLibrary.K2_SetTimer` null "End Movement" (`self.Move Duration`)))
      (set `self.Movement Timer` _returnvalue)
      (if `Fade Out by End of Movement`
        (`/Engine/EditorBlueprintResources/ActorMacros.Switch Has Authority`
          (:`Authority`
            (`KismetSystemLibrary.K2_SetTimer` null "Latent Fade Out" (`KismetMathLibrary.FMax` (- (`self.Move Duration`) (`self.Latent Fade Duration`)) 1.0))))))))

(fn `Refresh Targets`
  (bind _uds (`self.UDS`))
  (bind _udw (`self.UDW`))
  (`/Engine/EditorBlueprintResources/StandardMacros.IsValid` _uds
    (:`Is Valid`
      (`/Game/EtLaLumiereFut/Blueprints/Ultra_Dynamic_Sky.Update Painted Cloud Coverage Target` _uds)
      (`/Engine/EditorBlueprintResources/StandardMacros.IsValid` _udw
        (:`Is Valid`
          (`/Game/EtLaLumiereFut/Blueprints/Ultra_Dynamic_Weather.Update WOV Render Target` _udw))))))

(fn `Second Frame Startup`
  (`self.Update Radius and Positions`)
  (`self.Apply Niagara Properties`)
  (`self.Configure Thunder Sound`)
  (`|ExecutionSequence`
    (:`then_0`
      (`/Engine/EditorBlueprintResources/StandardMacros.IsValid` (`self.UDW`)
        (:`Is Valid`
          (`KismetArrayLibrary.Array_AddUnique` (`/Game/EtLaLumiereFut/Blueprints/Ultra_Dynamic_Weather.Radial Storm Actors` (`self.UDW`)) self))))
    (:`then_1`
      (if (and (> (`/Game/EtLaLumiereFut/Blueprints/Weather_Effects/System/UDS_Weather_Settings.Thunder/Lightning` (`self.Storm Weather`)) 0.0) (`self.Enable Thunder Sound`))
        (`AudioComponent.Play` (`self.Thunder Sound`) 0.0)))
    (:`then_2`
      (`self.Update Alpha`)
      (`SceneComponent.SetVisibility` (`self.Niagara System`) (`self.Effects Visible`) false)
      (if (not (`self.Fading In`))
        (`self.Refresh Targets`)
        (`self.Client Storm Update` (`self.Storm Alpha`))))))

(fn `Set Storm Location`
  (params (Location :type "Vector Structure"))
  (`self.K2_SetActorLocation` Location)
  (`self.Check to Apply Animation Changes`))

(fn `Start Ticking`
  (`self.SetActorTickEnabled` true)
  (`self.SetActorTickInterval` (`self.Tick Interval`))
  (set `self.Last Tick Time` (`KismetSystemLibrary.GetGameTimeInSeconds`)))

(fn `Update Alpha`
  (`FXSystemComponent.SetFloatParameter` (`self.Niagara System`) "Alpha" (`KismetMathLibrary.MapRangeClamped` (`self.Storm Alpha`) 0.5 1.0 0.0 1.0))
  (`AudioComponent.SetVolumeMultiplier` (`self.Thunder Sound`) (* (`self.Storm Alpha`) (`self.Thunder Sounds Volume Multiplier`) (/ (`/Game/EtLaLumiereFut/Blueprints/Weather_Effects/System/UDS_Weather_Settings.Thunder/Lightning` (`self.Storm Weather`)) 10.0)))
  (`/Engine/EditorBlueprintResources/StandardMacros.IsValid` (`self.UDW`)
    (:`Is Valid`
      (set `self.Material Target Color` (`/Game/EtLaLumiereFut/Blueprints/Ultra_Dynamic_Weather.Material Effect Draw Color from State` (`self.UDW`) (`self.Storm Weather`) (`self.Storm Alpha`))))))

(fn `Update Radius and Positions`
  (bind _returnvalue (- (+ (`self.Cloud Bottom Altitude`) (`self.Cloud Altitude Offset`)) (+ (`self.Ground Level Offset`) (`self.UDS Ground Level`))))
  (bind _returnvalue_2 (/ (* (`self.Outer Radius`) 2.0) 100.0))
  (bind _returnvalue_3 (/ (* (* (`self.Outer Radius`) (`self.Inner Radius Fraction`)) 2.0) 100.0))
  (`self.SetActorScale3D` (1.0 1.0 1.0))
  (`self.K2_SetActorLocation` (`KismetMathLibrary.MakeVector` (.x (`self.K2_GetActorLocation`)) (.y (`self.K2_GetActorLocation`)) (+ (`self.Cloud Bottom Altitude`) (`self.Cloud Altitude Offset`))))
  (`FXSystemComponent.SetFloatParameter` (`self.Niagara System`) "Outer Radius" (`self.Outer Radius`))
  (`FXSystemComponent.SetFloatParameter` (`self.Niagara System`) "Inner Radius" (* (`self.Outer Radius`) (`self.Inner Radius Fraction`)))
  (set `self.Cylinder Height` (`KismetMathLibrary.SelectFloat` (- 75000.0 (`self.Ground Level Offset`)) _returnvalue (< _returnvalue 1000.0)))
  (`SceneComponent.SetWorldScale3D` (`self.Inner Radius Wire`) (`KismetMathLibrary.MakeVector` _returnvalue_3 _returnvalue_3 (/ (`self.Cylinder Height`) 100.0)))
  (`SceneComponent.SetWorldScale3D` (`self.Outer Radius Wire`) (`KismetMathLibrary.MakeVector` _returnvalue_2 _returnvalue_2 (/ (`self.Cylinder Height`) 100.0))))

(fn `Update with Sky Mode Change`
  (returns (Successful :type Boolean))
  (`self.Check Sky Mode for Visibility`)
  (`SceneComponent.SetVisibility` (`self.Niagara System`) (`self.Effects Visible`) false)
  (return true))

(fn `UserConstructionScript`
  (bind _uds (`self.UDS`))
  (bind _uds_2 (`self.UDS`))
  (`|ExecutionSequence`
    (:`then_0`
      ;[1 0.2896 0.2598] Get UDS/W and Heights
      (`self.Get UDS and UDW`)
      (`/Engine/EditorBlueprintResources/StandardMacros.IsValid` _uds
        (:`Is Valid`
          (set `self.Cloud Bottom Altitude` (`/Game/EtLaLumiereFut/Blueprints/Ultra_Dynamic_Sky.Cloud Bottom World Height` _uds))
          (set `self.UDS Ground Level` (.z (`self.K2_GetActorLocation` _uds))))))
    (:`then_1`
      ;[0.3118 0.4204 1] Apply Properties
      (`self.Update Radius and Positions`)
      (`self.Update Alpha`)
      (`self.Apply Niagara Properties`)
      (`self.Configure Thunder Sound`)
      (`self.Check Sky Mode for Visibility`)
      (`SceneComponent.SetVisibility` (`self.Niagara System`) (`self.Effects Visible`) false))
    (:`then_2`
      ;[0.2929 0.7083 0.3165] UDS and UDW Editor Update
      (`/Engine/EditorBlueprintResources/StandardMacros.IsValid` _uds_2
        (:`Is Valid`
          (if (`|EnumEquality` (`/Game/EtLaLumiereFut/Blueprints/Ultra_Dynamic_Sky.Run Context` _uds_2) "NewEnumerator1")
            (`/Game/EtLaLumiereFut/Blueprints/Ultra_Dynamic_Sky.Get Starting Cloud Painting Actors` (`self.UDS`))
            (`/Game/EtLaLumiereFut/Blueprints/Ultra_Dynamic_Sky.Update Painted Cloud Coverage Target` (`self.UDS`))
            (`/Engine/EditorBlueprintResources/StandardMacros.IsValid` (`self.UDW`)
              (:`Is Valid`
                (`/Game/EtLaLumiereFut/Blueprints/Ultra_Dynamic_Weather.Get Starting Radial Storms` (`self.UDW`))
                (`/Game/EtLaLumiereFut/Blueprints/Ultra_Dynamic_Weather.Update WOV Render Target` (`self.UDW`))))))))))

(fn `📘 Radial Storm`
  (bind _returnvalue (`GameplayStatics.GetActorOfClass` "/Game/EtLaLumiereFut/Blueprints/Ultra_Dynamic_Weather.Ultra_Dynamic_Weather_C"))
  (`/Engine/EditorBlueprintResources/StandardMacros.IsValid` _returnvalue
    (:`Is Valid`
      (`/Game/EtLaLumiereFut/Blueprints/Ultra_Dynamic_Weather.Open Editor Readme Entry` _returnvalue "RadialStorm"))))