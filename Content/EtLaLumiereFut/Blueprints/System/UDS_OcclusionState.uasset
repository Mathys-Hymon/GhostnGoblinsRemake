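; UDS occlusion state that precomputes the trace pattern and weights for sampling occlusion around a point.
; SaveUnchangingValues runs once, building a jittered, twisted hemisphere of trace offsets plus one straight-up trace, sized from OcclusionSettings.
; Each trace gets an upward weight and four horizontal direction weights packed into RGBA, with running totals as maxima.
; It shuffles trace order, sizes history buffers and derives the per-trace time increment from the update period.
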(fn `Current Facing Direction`
  (params (Step :type Integer))
  (returns (ReturnValue :type "Vector Structure"))
  (return (`KismetMathLibrary.RotateAngleAxis` (1.0 0.0 0.0) (* (/ 360.0 (`KismetMathLibrary.Conv_IntToDouble` (`/Game/EtLaLumiereFut/Blueprints/System/UDS_OcclusionSettings.Horizontal Trace Steps` (`self.Occlusion Settings`)))) (`KismetMathLibrary.Conv_IntToDouble` Step)) (0.0 0.0 1.0))))

(fn `Current Trace Direction`
  (params (`Facing Direction` :type "Vector Structure") (`Vertical Step` :type Integer))
  (returns (ReturnValue :type "Vector Structure"))
  (return (`KismetMathLibrary.Normal` (`KismetMathLibrary.MakeVector` (.x (`KismetMathLibrary.RandomUnitVectorInConeInDegrees` (`KismetMathLibrary.RotateAngleAxis` (`KismetMathLibrary.VLerp` `Facing Direction` (0.0 0.0 1.0) (/ (`KismetMathLibrary.Conv_IntToDouble` `Vertical Step`) (- (`KismetMathLibrary.Conv_IntToDouble` (`/Game/EtLaLumiereFut/Blueprints/System/UDS_OcclusionSettings.Vertical Trace Steps` (`self.Occlusion Settings`))) 0.5))) (* (`local.Vertical Step`) (/ 360.0 (`KismetMathLibrary.Conv_IntToDouble` (`/Game/EtLaLumiereFut/Blueprints/System/UDS_OcclusionSettings.Horizontal Trace Steps` (`self.Occlusion Settings`)))) 0.35) (0.0 0.0 1.0)) 5.0)) (.y (`KismetMathLibrary.RandomUnitVectorInConeInDegrees` (`KismetMathLibrary.RotateAngleAxis` (`KismetMathLibrary.VLerp` `Facing Direction` (0.0 0.0 1.0) (/ (`KismetMathLibrary.Conv_IntToDouble` `Vertical Step`) (- (`KismetMathLibrary.Conv_IntToDouble` (`/Game/EtLaLumiereFut/Blueprints/System/UDS_OcclusionSettings.Vertical Trace Steps` (`self.Occlusion Settings`))) 0.5))) (* (`local.Vertical Step`) (/ 360.0 (`KismetMathLibrary.Conv_IntToDouble` (`/Game/EtLaLumiereFut/Blueprints/System/UDS_OcclusionSettings.Horizontal Trace Steps` (`self.Occlusion Settings`)))) 0.35) (0.0 0.0 1.0)) 5.0)) (`KismetMathLibrary.FMax` (.z (`KismetMathLibrary.RandomUnitVectorInConeInDegrees` (`KismetMathLibrary.RotateAngleAxis` (`KismetMathLibrary.VLerp` `Facing Direction` (0.0 0.0 1.0) (/ (`KismetMathLibrary.Conv_IntToDouble` `Vertical Step`) (- (`KismetMathLibrary.Conv_IntToDouble` (`/Game/EtLaLumiereFut/Blueprints/System/UDS_OcclusionSettings.Vertical Trace Steps` (`self.Occlusion Settings`))) 0.5))) (* (`local.Vertical Step`) (/ 360.0 (`KismetMathLibrary.Conv_IntToDouble` (`/Game/EtLaLumiereFut/Blueprints/System/UDS_OcclusionSettings.Horizontal Trace Steps` (`self.Occlusion Settings`)))) 0.35) (0.0 0.0 1.0)) 5.0)))))))

(fn `Directional Mask Value`
  (params (Direction :type "Vector Structure") (Compare :type "Vector Structure"))
  (returns (ReturnValue :type "Float (double-precision)"))
  (return (`KismetMathLibrary.MapRangeClamped` (`KismetMathLibrary.DegAcos` (`KismetMathLibrary.Dot_VectorVector` Direction Compare)) 0.0 50.0 1.0)))

(fn `Directional Vector Mask`
  (params (Direction :type "Vector Structure"))
  (returns (Mask :type "LinearColor Structure"))
  (return (make `LinearColor` (`self.Directional Mask Value` Direction (1.0 0.0 0.0)) (`self.Directional Mask Value` Direction (0.0 1.0 0.0)) (`self.Directional Mask Value` Direction (-1.0 0.0 0.0)) (`self.Directional Mask Value` Direction (0.0 -1.0 0.0)))))

(fn `Save Unchanging Values`
  (locals (`Facing Direction` :type "Vector Structure") (`Trace Direction` :type "Vector Structure" :default (0.0 0.0 0.0)) (`Trace Offsets In Order` :type "Array of Vector Structure") (`Directional Max Values in Order` :type "Array of LinearColor Structure") (`Random Order` :type "Array of Integer") (`Integer List` :type "Array of Integer") (`Selected Random Index` :type Integer :default 0) (`Upward Max Values in Order` :type "Array of Float (double-precision)"))
  (bind _traces_per_update (`self.Traces Per Update`))
  (bind _mask (`self.Directional Vector Mask` (`local.Trace Direction`)))
  (bind _returnvalue (`KismetMathLibrary.MapRangeClamped` (`KismetMathLibrary.DegAcos` (`KismetMathLibrary.Dot_VectorVector` (`local.Trace Direction`) (0.0 0.0 1.0))) 0.0 30.0 1.0))
  (if (not (`self.Unchanging Values Saved`))
    (set `self.Unchanging Values Saved` true)
    (set `self.Directional Occlusion Max` 0.0)
    (set `self.Upward Occlusion Max` 0.0)
    (`KismetArrayLibrary.Array_Clear` (`self.Upward Trace Max Values`))
    (`KismetArrayLibrary.Array_Clear` (`self.Directional Trace Max Values`))
    (`KismetArrayLibrary.Array_Clear` (`self.Trace Offsets`))
    ;[0.1876 0.1987 0.5365 1 35] Create Array of Trace Vectors
    (for _index (range (`/Game/EtLaLumiereFut/Blueprints/System/UDS_OcclusionSettings.Horizontal Trace Steps` (`self.Occlusion Settings`)))
      (set `local.Facing Direction` (`self.Current Facing Direction` _index))
      (for _index_2 (range (`/Game/EtLaLumiereFut/Blueprints/System/UDS_OcclusionSettings.Vertical Trace Steps` (`self.Occlusion Settings`)))
        (set `local.Trace Direction` (`self.Current Trace Direction` (`local.Facing Direction`) _index_2))
        (`KismetArrayLibrary.Array_Add` (`local.Trace Offsets In Order`) (* (`local.Trace Direction`) (* (`/Game/EtLaLumiereFut/Blueprints/System/UDS_OcclusionSettings.Max Trace Distance` (`self.Occlusion Settings`)) (`KismetMathLibrary.RandomFloatInRange` 0.9 1.1))) :!label _label)
        (`KismetArrayLibrary.Array_Add` (`local.Directional Max Values in Order`) _mask)
        (set `self.Directional Occlusion Max` (+ (`self.Directional Occlusion Max`) (`.R` (break `LinearColor` _mask))))
        (`KismetArrayLibrary.Array_Add` (`local.Upward Max Values in Order`) _returnvalue)
        (set `self.Upward Occlusion Max` (+ _returnvalue (`self.Upward Occlusion Max`)))))
    (`|ExecutionSequence`
      (:`then_0`
        (set `local.Trace Direction` (0.0 0.0 1.0))
        (goto _label))
      (:`then_1`
        (set `self.Traces Per Update` (`KismetArrayLibrary.Array_Length` (`local.Trace Offsets In Order`)))
        (`KismetArrayLibrary.Array_Resize` (`self.Directional Occlusion History`) _traces_per_update)
        (`KismetArrayLibrary.Array_Resize` (`self.Global Occlusion History`) _traces_per_update)
        (`KismetArrayLibrary.Array_Resize` (`self.Upward Occlusion History`) _traces_per_update)
        (set `self.Increment Time` (/ (`/Game/EtLaLumiereFut/Blueprints/System/UDS_OcclusionSettings.Update Period` (`self.Occlusion Settings`)) (`self.Traces Per Update`)))
        ;[0.474 0.1541 0.1163 1 35] Randomize Trace Order
        (for _index_3 (range (`self.Traces Per Update`))
          (`KismetArrayLibrary.Array_Add` (`local.Integer List`) _index_3))
        (while (`KismetArrayLibrary.Array_IsNotEmpty` (`local.Integer List`))
          (set `local.Selected Random Index` (`.OutIndex` (`KismetArrayLibrary.Array_Random` (`local.Integer List`))))
          (`KismetArrayLibrary.Array_Add` (`local.Random Order`) (`|GetArrayItem` (`local.Integer List`) (`local.Selected Random Index`)))
          (`KismetArrayLibrary.Array_Remove` (`local.Integer List`) (`local.Selected Random Index`)))
        (for _array_element (`local.Random Order`)
          (`KismetArrayLibrary.Array_Add` (`self.Directional Trace Max Values`) (`|GetArrayItem` (`local.Directional Max Values in Order`) _array_element))
          (`KismetArrayLibrary.Array_Add` (`self.Trace Offsets`) (`|GetArrayItem` (`local.Trace Offsets In Order`) _array_element))
          (`KismetArrayLibrary.Array_Add` (`self.Upward Trace Max Values`) (`|GetArrayItem` (`local.Upward Max Values in Order`) _array_element)))))))