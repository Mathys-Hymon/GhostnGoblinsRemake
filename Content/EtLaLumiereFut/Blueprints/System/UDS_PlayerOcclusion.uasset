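; Ultra Dynamic Sky component that measures how occluded the player camera, pawn or component location is, globally and directionally.
; Collision traces are spread over time into rolling totals, while timed checks apply occlusion volumes, water level and nearby portals.
; Results are smoothed, or snapped after large location jumps, with directional mode also writing them to the weather parameter collection.
; Self-rescheduling timers drive runtime updates, and Editor Tick provides an editor path.
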(event `self.ReceiveEndPlay`
  (params (EndPlayReason :type "EEndPlayReason Enum" :default "Destroyed"))
  (`KismetSystemLibrary.K2_ClearTimer` null "Periodic Context Checks")
  (`KismetSystemLibrary.K2_ClearTimer` null "Update Ignored Actors")
  (`KismetSystemLibrary.K2_ClearTimer` null "Check For Portal Components")
  (`KismetSystemLibrary.K2_ClearTimer` null "Runtime Tick"))

(fn `Check For Portal Components`
  (bind _sample_location (`self.Sample Location`))
  (set `/Game/EtLaLumiereFut/Blueprints/System/UDS_OcclusionState.Time of Last Portal Component Check` (`KismetSystemLibrary.GetGameTimeInSeconds`) (`self.State`))
  (`KismetArrayLibrary.Array_Clear` (`self.Portal Components`))
  (bind (_outhits _returnvalue) (`KismetSystemLibrary.LineTraceMultiForObjects` _sample_location (- _sample_location (0.0 0.0 1.0)) (`|MakeArray` "ObjectTypeQuery4" :!type "EObjectTypeQuery Enum") false (`self.Ignored Actors`)))
  (if _returnvalue
    (for _array_element _outhits
      (bind _asuds_occlusion_portal (cast `/Game/EtLaLumiereFut/Blueprints/Occlusion/UDS_Occlusion_Portal` (`.HitComponent` (`GameplayStatics.BreakHitResult` _array_element))))
      (`KismetArrayLibrary.Array_Add` (`self.Portal Components`) _asuds_occlusion_portal))))

(fn `Delayed Startup`
  (`self.Get Sample Location`)
  (if (`KismetMathLibrary.EqualExactly_VectorVector` (`self.Sample Location`))
    (`KismetSystemLibrary.K2_SetTimerForNextTick` null "Delayed Startup")
    (else
      (`self.Periodic Context Checks`)
      (`KismetSystemLibrary.K2_SetTimer` null "Periodic Context Checks" (`/Game/EtLaLumiereFut/Blueprints/System/UDS_OcclusionSettings.Update Period` (`self.Occlusion Settings`)) true)
      (`self.Update Ignored Actors`)
      (`KismetSystemLibrary.K2_SetTimer` null "Update Ignored Actors" 3.0 true)
      (if (`/Game/EtLaLumiereFut/Blueprints/System/UDS_OcclusionSettings.Query Occlusion Portals` (`self.Occlusion Settings`))
        (`self.Check For Portal Components`)
        (`KismetSystemLibrary.K2_SetTimer` null "Check For Portal Components" 3.0 true))
      (`self.Runtime Tick`))))

(fn `Editor Tick`
  (params (`Occlusion Location` :type "Vector Structure"))
  (bind _state (`self.State`))
  (set `self.Sample Location` `Occlusion Location`)
  (`|ExecutionSequence`
    (:`then_0`
      (if (> (- (`KismetSystemLibrary.GetGameTimeInSeconds`) (`/Game/EtLaLumiereFut/Blueprints/System/UDS_OcclusionState.Time of Last Periodic Context Check` (`self.State`))) (`/Game/EtLaLumiereFut/Blueprints/System/UDS_OcclusionSettings.Update Period` (`self.Occlusion Settings`)))
        (`self.Periodic Context Checks`)))
    (:`then_1`
      (if (> (- (`KismetSystemLibrary.GetGameTimeInSeconds`) (`/Game/EtLaLumiereFut/Blueprints/System/UDS_OcclusionState.Time of Last Portal Component Check` (`self.State`))) 3.0)
        (`self.Check For Portal Components`)))
    (:`then_2`
      (if (> (- (`KismetSystemLibrary.GetGameTimeInSeconds`) (`/Game/EtLaLumiereFut/Blueprints/System/UDS_OcclusionState.Time of Last Editor Cache` (`self.State`))) 15.0)
        (set `/Game/EtLaLumiereFut/Blueprints/System/UDS_OcclusionState.Unchanging Values Saved` false _state)
        (`/Game/EtLaLumiereFut/Blueprints/System/UDS_OcclusionState.Save Unchanging Values` _state)
        (set `/Game/EtLaLumiereFut/Blueprints/System/UDS_OcclusionState.Time of Last Editor Cache` (`KismetSystemLibrary.GetGameTimeInSeconds`) (`self.State`))))
    (:`then_3`
      (`self.Incremental Occlusion Traces`)
      (`self.Update Current Occlusion`))))

(fn `Get Sample Location`
  (bind _returnvalue (`GameplayStatics.GetPlayerCameraManager` 0))
  (bind _returnvalue_2 (`GameplayStatics.GetPlayerPawn` 0))
  (switch `/Game/EtLaLumiereFut/Blueprints/Enum/UDS_OcclusionSamplingLocation` (`/Game/EtLaLumiereFut/Blueprints/System/UDS_OcclusionSettings.Occlusion Sampling Location` (`self.Occlusion Settings`))
    (:`NewEnumerator0`
      (`/Engine/EditorBlueprintResources/StandardMacros.IsValid` _returnvalue :!label _label
        (:`Is Valid`
          (set `self.Sample Location` (`PlayerCameraManager.GetCameraLocation` _returnvalue)))))
    (:`NewEnumerator1`
      (`/Engine/EditorBlueprintResources/StandardMacros.IsValid` _returnvalue_2
        (:`Is Valid`
          (set `self.Sample Location` (`Actor.K2_GetActorLocation` _returnvalue_2)))
        (:`Is Not Valid`
          (goto _label))))
    (:`NewEnumerator2`
      (set `self.Sample Location` (`self.K2_GetComponentLocation`)))))

(fn `Incremental Occlusion Traces`
  (locals (`Current Trace Occlusion` :type "Float (double-precision)" :default 0.0) (`Directional Total Contribution` :type "LinearColor Structure") (`Traces This Frame` :type Integer :default 0) (`Upward Total Contribution` :type "Float (double-precision)"))
  (bind _state (`self.State`))
  (bind _state_2 (`self.State`))
  (bind _current_trace_occlusion (`local.Current Trace Occlusion`))
  (bind _state_3 (`self.State`))
  (bind _sample_location (`self.Sample Location`))
  (bind _state_4 (`self.State`))
  (bind _state_5 (`self.State`))
  (bind _state_6 (`self.State`))
  (bind _state_7 (`self.State`))
  ;[0.3793 0.155 0.4948] Checks if location has traveled far enough to need an instant/hard update
  (set `self.Hard Update` (> (`KismetMathLibrary.Vector_Distance` (`/Game/EtLaLumiereFut/Blueprints/System/UDS_OcclusionState.Last Trace Location` (`self.State`)) (`self.Sample Location`)) 1000.0))
  ;[0.1582 0.4177 0.4219] Find How Many Traces to Do this Update
  (bind _output_get (set `local.Traces This Frame` (`KismetMathLibrary.SelectInt` (`/Game/EtLaLumiereFut/Blueprints/System/UDS_OcclusionState.Traces Per Update` (`self.State`)) (`KismetMathLibrary.Min` (`KismetMathLibrary.Max` (`KismetMathLibrary.Round` (/ (- (`KismetSystemLibrary.GetGameTimeInSeconds`) (`/Game/EtLaLumiereFut/Blueprints/System/UDS_OcclusionState.Time of Last Trace` _state)) (`/Game/EtLaLumiereFut/Blueprints/System/UDS_OcclusionState.Increment Time` _state))) 1) (`/Game/EtLaLumiereFut/Blueprints/System/UDS_OcclusionState.Traces Per Update` (`self.State`))) (`self.Hard Update`))))
  (if (> _output_get 0)
    ;[1 0.1521 0.3022] Last Update Values
    (set `/Game/EtLaLumiereFut/Blueprints/System/UDS_OcclusionState.Last Trace Location` (`self.Sample Location`) (`self.State`))
    (set `/Game/EtLaLumiereFut/Blueprints/System/UDS_OcclusionState.Time of Last Trace` (`KismetSystemLibrary.GetGameTimeInSeconds`) (`self.State`))
    (for _ (range 1 (+ (`local.Traces This Frame`) 1))
      (`|ExecutionSequence`
        (:`then_0`
          ;[0.4993 0.45 1] Trace Scene Collision
          (bind (_outhit _returnvalue) (`KismetSystemLibrary.LineTraceSingle` _sample_location (+ _sample_location (`|GetArrayItem` (`/Game/EtLaLumiereFut/Blueprints/System/UDS_OcclusionState.Trace Offsets` _state_7) (`/Game/EtLaLumiereFut/Blueprints/System/UDS_OcclusionState.Trace Index` _state_7))) (`/Game/EtLaLumiereFut/Blueprints/System/UDS_OcclusionSettings.Trace Channel` (`self.Occlusion Settings`)) false (`self.Ignored Actors`) (`self.Trace Debugs`) true (struct :`R` 1.0 :`A` 1.0) (struct :`G` 1.0 :`A` 1.0) (* (`/Game/EtLaLumiereFut/Blueprints/System/UDS_OcclusionState.Increment Time` (`self.State`)) 10.0)))
          (set `local.Current Trace Occlusion` (`KismetMathLibrary.SelectFloat` 0.0 1.0 _returnvalue))
          (`|ExecutionSequence`
            (:`then_0`
              ;[0.3033 0.3213 1] Global Occlusion
              (set `/Game/EtLaLumiereFut/Blueprints/System/UDS_OcclusionState.Global Occlusion Total` (- (+ (`local.Current Trace Occlusion`) (`/Game/EtLaLumiereFut/Blueprints/System/UDS_OcclusionState.Global Occlusion Total` _state_2)) (`|GetArrayItem` (`/Game/EtLaLumiereFut/Blueprints/System/UDS_OcclusionState.Global Occlusion History` _state_2) (`/Game/EtLaLumiereFut/Blueprints/System/UDS_OcclusionState.Trace Index` _state_2))) (`self.State`))
              (`KismetArrayLibrary.Array_Set` (`/Game/EtLaLumiereFut/Blueprints/System/UDS_OcclusionState.Global Occlusion History` (`self.State`)) (`/Game/EtLaLumiereFut/Blueprints/System/UDS_OcclusionState.Trace Index` (`self.State`)) (`local.Current Trace Occlusion`)))
            (:`then_1`
              ;[0.5938 0.2735 0.1477] Directional Occlusion
              (if (`self.Calculate Directional Occlusion`)
                (`|ExecutionSequence`
                  (:`then_0`
                    (set `local.Directional Total Contribution` (* (`|GetArrayItem` (`/Game/EtLaLumiereFut/Blueprints/System/UDS_OcclusionState.Directional Trace Max Values` _state_4) (`/Game/EtLaLumiereFut/Blueprints/System/UDS_OcclusionState.Trace Index` _state_4)) (make `LinearColor` _current_trace_occlusion _current_trace_occlusion _current_trace_occlusion _current_trace_occlusion)))
                    (set `/Game/EtLaLumiereFut/Blueprints/System/UDS_OcclusionState.Directional Occlusion Total` (- (+ (`/Game/EtLaLumiereFut/Blueprints/System/UDS_OcclusionState.Directional Occlusion Total` _state_5) (`local.Directional Total Contribution`)) (`|GetArrayItem` (`/Game/EtLaLumiereFut/Blueprints/System/UDS_OcclusionState.Directional Occlusion History` _state_5) (`/Game/EtLaLumiereFut/Blueprints/System/UDS_OcclusionState.Trace Index` _state_5))) (`self.State`))
                    (`KismetArrayLibrary.Array_Set` (`/Game/EtLaLumiereFut/Blueprints/System/UDS_OcclusionState.Directional Occlusion History` (`self.State`)) (`/Game/EtLaLumiereFut/Blueprints/System/UDS_OcclusionState.Trace Index` (`self.State`)) (`local.Directional Total Contribution`)))
                  (:`then_1`
                    (set `local.Upward Total Contribution` (* (`|GetArrayItem` (`/Game/EtLaLumiereFut/Blueprints/System/UDS_OcclusionState.Upward Trace Max Values` _state_6) (`/Game/EtLaLumiereFut/Blueprints/System/UDS_OcclusionState.Trace Index` _state_6)) (`local.Current Trace Occlusion`)))
                    (set `/Game/EtLaLumiereFut/Blueprints/System/UDS_OcclusionState.Upward Occlusion Total` (- (+ (`/Game/EtLaLumiereFut/Blueprints/System/UDS_OcclusionState.Upward Occlusion Total` _state_3) (`local.Upward Total Contribution`)) (`|GetArrayItem` (`/Game/EtLaLumiereFut/Blueprints/System/UDS_OcclusionState.Upward Occlusion History` _state_3) (`/Game/EtLaLumiereFut/Blueprints/System/UDS_OcclusionState.Trace Index` _state_3))) (`self.State`))
                    (`KismetArrayLibrary.Array_Set` (`/Game/EtLaLumiereFut/Blueprints/System/UDS_OcclusionState.Upward Occlusion History` (`self.State`)) (`/Game/EtLaLumiereFut/Blueprints/System/UDS_OcclusionState.Trace Index` (`self.State`)) (`local.Upward Total Contribution`))))))))
        (:`then_1`
          (set `/Game/EtLaLumiereFut/Blueprints/System/UDS_OcclusionState.Trace Index` (mod (+ (`/Game/EtLaLumiereFut/Blueprints/System/UDS_OcclusionState.Trace Index` (`self.State`)) 1) (`/Game/EtLaLumiereFut/Blueprints/System/UDS_OcclusionState.Traces Per Update` (`self.State`))) (`self.State`)))))))

(fn `Initialize`
  (`/Engine/EditorBlueprintResources/StandardMacros.IsValid` (`self.Occlusion Settings`)
    (:`Is Valid`
      _)
    (:`Is Not Valid`
      (set `self.Occlusion Settings` "/Game/EtLaLumiereFut/Blueprints/Occlusion/Occlusion_Settings/UDS_Standard_Occlusion_Settings.UDS_Standard_Occlusion_Settings")))
  (`/Game/EtLaLumiereFut/Blueprints/System/UDS_OcclusionState.Save Unchanging Values` (`self.State`))
  (`self.Delayed Startup`))

(fn `Periodic Context Checks`
  (locals (`Current Portal` :type "/Game/EtLaLumiereFut/Blueprints/Occlusion/UDS_Occlusion_Portal Object Reference") (`Portal Direction` :type "Vector Structure" :default (0.0 0.0 0.0)) (`Portal Distance Mask` :type "Float (double-precision)"))
  (bind _state (`self.State`))
  (bind _sample_location (`self.Sample Location`))
  (bind _returnvalue (* (`local.Portal Distance Mask`) (`/Game/EtLaLumiereFut/Blueprints/Occlusion/UDS_Occlusion_Portal.Directional Occlusion` (`local.Current Portal`))))
  (bind _returnvalue_2 (`KismetMathLibrary.Normal` (- (`self.K2_GetComponentLocation` (`local.Current Portal`)) (`self.Sample Location`))))
  (set `/Game/EtLaLumiereFut/Blueprints/System/UDS_OcclusionState.Time of Last Periodic Context Check` (`KismetSystemLibrary.GetGameTimeInSeconds`) (`self.State`))
  (set `/Game/EtLaLumiereFut/Blueprints/System/UDS_OcclusionState.Occlusion Multiplier` (`KismetMathLibrary.SelectFloat` 0.0 1.0 (`self.Force Full Occlusion`)) _state)
  (set `/Game/EtLaLumiereFut/Blueprints/System/UDS_OcclusionState.Global Contribution` 0.0 _state)
  (set `/Game/EtLaLumiereFut/Blueprints/System/UDS_OcclusionState.Directional Portal Contribution` (struct) _state)
  (`|ExecutionSequence`
    (:`then_0`
      ;[0.4335 0.2794 0.625 1 35] Test for Occlusion Volumes
      (if (`|EnumInequality` (`/Game/EtLaLumiereFut/Blueprints/System/UDS_OcclusionSettings.Occlusion Mode` (`self.Occlusion Settings`)) "NewEnumerator0")
        (bind (_outhits _returnvalue_3) (`KismetSystemLibrary.LineTraceMultiForObjects` _sample_location (+ _sample_location (0.0 0.0 1.0)) (`|MakeArray` "ObjectTypeQuery4" :!type "EObjectTypeQuery Enum") false (`self.Ignored Actors`)))
        (if _returnvalue_3
          (for _array_element _outhits
            (bind _asuds_occlusion_volume (cast `/Game/EtLaLumiereFut/Blueprints/Occlusion/UDS_Occlusion_Volume` (`.HitActor` (`GameplayStatics.BreakHitResult` _array_element))))
            (if (`/Game/EtLaLumiereFut/Blueprints/Occlusion/UDS_Occlusion_Volume.Affects Sound Occlusion / Interior Adjusments` _asuds_occlusion_volume)
              (set `/Game/EtLaLumiereFut/Blueprints/System/UDS_OcclusionState.Occlusion Multiplier` 0.0 (`self.State`))
              (break))))))
    (:`then_1`
      (`|ExecutionSequence`
        (:`then_0`
          ;[0.2042 0.5365 0.1688 1 35] Test if Under Water
          (bind _returnvalue_4 (`KismetMaterialLibrary.GetScalarParameterValue` "/Game/EtLaLumiereFut/Particles/UDW_WeatherParticle_Parameters.UDW_WeatherParticle_Parameters" "Apply Water Level"))
          (if (> _returnvalue_4 0.5)
            (bind _returnvalue_5 (`KismetMaterialLibrary.GetScalarParameterValue` "/Game/EtLaLumiereFut/Materials/Weather/UltraDynamicWeather_Parameters.UltraDynamicWeather_Parameters" "Water Level"))
            (if (> _returnvalue_5 (.z (`self.Sample Location`)))
              (switch `/Game/EtLaLumiereFut/Blueprints/Enum/UDS_Occlusion_Water_Behavior` (`/Game/EtLaLumiereFut/Blueprints/System/UDS_OcclusionSettings.Occlusion Behavior Under Water` (`self.Occlusion Settings`))
                (:`NewEnumerator0`
                  (set `/Game/EtLaLumiereFut/Blueprints/System/UDS_OcclusionState.Occlusion Multiplier` 0.0 (`self.State`)))
                (:`NewEnumerator1`
                  (set `/Game/EtLaLumiereFut/Blueprints/System/UDS_OcclusionState.Global Contribution` 1.0 (`self.State`))
                  (set `/Game/EtLaLumiereFut/Blueprints/System/UDS_OcclusionState.Directional Portal Contribution` (struct :`R` 1.0 :`G` 1.0 :`B` 1.0 :`A` 1.0) (`self.State`)))))))
        (:`then_1`
          ;[0.2197 0.2803 0.5625] Test for Portals
          (if (`KismetArrayLibrary.Array_IsNotEmpty` (`self.Portal Components`))
            (for _array_element_2 (`self.Portal Components`)
              (bind _output_get (set `local.Current Portal` _array_element_2))
              (if (and (< (`KismetMathLibrary.VSize` (- (`self.K2_GetComponentLocation` _output_get) (`self.Sample Location`))) (`/Game/EtLaLumiereFut/Blueprints/Occlusion/UDS_Occlusion_Portal.Sample Range` (`local.Current Portal`))) (`self.IsActive` (`local.Current Portal`)))
                (bind (_outhit _returnvalue_6) (`KismetSystemLibrary.LineTraceSingle` (`self.K2_GetComponentLocation` (`local.Current Portal`)) (`self.Sample Location`) (`/Game/EtLaLumiereFut/Blueprints/System/UDS_OcclusionSettings.Trace Channel` (`self.Occlusion Settings`)) false (`self.Ignored Actors`) (`self.Trace Debugs`) true (struct :`R` 0.743149 :`B` 1.0 :`A` 1.0) (struct :`R` 0.062801 :`B` 1.0 :`A` 1.0) (`/Game/EtLaLumiereFut/Blueprints/System/UDS_OcclusionSettings.Update Period` (`self.Occlusion Settings`))))
                (if (not _returnvalue_6)
                  (set `local.Portal Direction` (`KismetMathLibrary.SelectVector` (* (`self.GetForwardVector` (`local.Current Portal`)) -1.0) _returnvalue_2 (> (`KismetMathLibrary.Dot_VectorVector` _returnvalue_2 (`self.GetForwardVector` (`local.Current Portal`))) 0.0)))
                  (set `local.Portal Distance Mask` (`KismetMathLibrary.MultiplyMultiply_FloatFloat` (- 1.0 (/ (`KismetMathLibrary.Vector_Distance` (`self.K2_GetComponentLocation` (`local.Current Portal`)) (`self.Sample Location`)) (`/Game/EtLaLumiereFut/Blueprints/Occlusion/UDS_Occlusion_Portal.Sample Range` (`local.Current Portal`)))) (`/Game/EtLaLumiereFut/Blueprints/Occlusion/UDS_Occlusion_Portal.Distance Falloff Exponent` (`local.Current Portal`))))
                  (`|ExecutionSequence`
                    (:`then_0`
                      (if (> (`/Game/EtLaLumiereFut/Blueprints/Occlusion/UDS_Occlusion_Portal.Directional Occlusion` (`local.Current Portal`)) 0.0)
                        (set `/Game/EtLaLumiereFut/Blueprints/System/UDS_OcclusionState.Directional Portal Contribution` (+ (`/Game/EtLaLumiereFut/Blueprints/System/UDS_OcclusionState.Directional Portal Contribution` (`self.State`)) (* (`self.Portal Direction Mask` (`KismetMathLibrary.Normal` (* (`local.Portal Direction`) (1.0 1.0 0.5)))) (make `LinearColor` _returnvalue _returnvalue _returnvalue _returnvalue))) (`self.State`))))
                    (:`then_1`
                      (if (> (`/Game/EtLaLumiereFut/Blueprints/Occlusion/UDS_Occlusion_Portal.Global Occlusion` (`local.Current Portal`)) 0.0)
                        (set `/Game/EtLaLumiereFut/Blueprints/System/UDS_OcclusionState.Global Contribution` (+ (`/Game/EtLaLumiereFut/Blueprints/System/UDS_OcclusionState.Global Contribution` (`self.State`)) (* (`local.Portal Distance Mask`) (`/Game/EtLaLumiereFut/Blueprints/Occlusion/UDS_Occlusion_Portal.Global Occlusion` (`local.Current Portal`)))) (`self.State`))))))))))))))

(fn `Portal Direction Mask`
  (params (Direction :type "Vector Structure"))
  (returns (Mask :type "LinearColor Structure"))
  (bind _x (.x Direction))
  (bind _y (.y Direction))
  (return (make `LinearColor` (`KismetMathLibrary.FClamp` _x) (`KismetMathLibrary.FClamp` _y) (`KismetMathLibrary.FClamp` (* _x -1.0)) (`KismetMathLibrary.FClamp` (* _y -1.0)))))

(fn `Runtime Tick`
  (`|ExecutionSequence`
    (:`then_0`
      (`self.Get Sample Location`)
      (`self.Incremental Occlusion Traces`)
      (`self.Update Current Occlusion`)
      (if (`self.Hard Update`)
        (`self.Hard Occlusion Change`)))
    (:`then_1`
      (if (== (`self.Tick Period`) 0.0)
        (`KismetSystemLibrary.K2_SetTimerForNextTick` null "Runtime Tick")
        (else
          (`KismetSystemLibrary.K2_SetTimer` null "Runtime Tick" (`self.Tick Period`)))))))

(fn `Trace Debugs`
  (returns (ReturnValue :type "EDrawDebugTrace Enum"))
  (return (select `bool` (`/Game/EtLaLumiereFut/Blueprints/System/UDS_OcclusionSettings.Show Trace Debugs` (`self.Occlusion Settings`)) :`true` "ForDuration" :!type "EDrawDebugTrace Enum")))

(fn `Update Current Occlusion`
  (locals (`Time Delta` :type "Float (double-precision)" :default 0.0))
  (bind _state (`self.State`))
  (bind _occlusion_settings (`self.Occlusion Settings`))
  (bind _state_2 (`self.State`))
  (bind _state_3 (`self.State`))
  (bind _state_4 (`self.State`))
  (bind _state_5 (`self.State`))
  (bind _directional_occlusion_max (`/Game/EtLaLumiereFut/Blueprints/System/UDS_OcclusionState.Directional Occlusion Max` (`self.State`)))
  (bind _directional_occlusion_max_2 (`/Game/EtLaLumiereFut/Blueprints/System/UDS_OcclusionState.Directional Occlusion Max` (`self.State`)))
  (bind _occlusion_multiplier (`/Game/EtLaLumiereFut/Blueprints/System/UDS_OcclusionState.Occlusion Multiplier` (`self.State`)))
  (bind (_r _g _b _a) (break `LinearColor` (+ (* (/ (`/Game/EtLaLumiereFut/Blueprints/System/UDS_OcclusionState.Directional Occlusion Total` (`self.State`)) (make `LinearColor` _directional_occlusion_max_2 _directional_occlusion_max_2 _directional_occlusion_max_2 _directional_occlusion_max_2)) (make `LinearColor` _occlusion_multiplier _occlusion_multiplier _occlusion_multiplier _occlusion_multiplier)) (`/Game/EtLaLumiereFut/Blueprints/System/UDS_OcclusionState.Directional Portal Contribution` (`self.State`)))))
  (switch `/Game/EtLaLumiereFut/Blueprints/Enum/UDS_Occlusion_Mode` (`/Game/EtLaLumiereFut/Blueprints/System/UDS_OcclusionSettings.Occlusion Mode` (`self.Occlusion Settings`))
    (:`NewEnumerator0`
      _)
    (:`NewEnumerator1`
      (set `/Game/EtLaLumiereFut/Blueprints/System/UDS_OcclusionState.Global Occlusion Total` (`KismetMathLibrary.Conv_IntToDouble` (`/Game/EtLaLumiereFut/Blueprints/System/UDS_OcclusionState.Traces Per Update` (`self.State`))) (`self.State`))
      (set `/Game/EtLaLumiereFut/Blueprints/System/UDS_OcclusionState.Directional Occlusion Total` (make `LinearColor` _directional_occlusion_max _directional_occlusion_max _directional_occlusion_max _directional_occlusion_max) (`self.State`))
      (set `/Game/EtLaLumiereFut/Blueprints/System/UDS_OcclusionState.Upward Occlusion Total` (`/Game/EtLaLumiereFut/Blueprints/System/UDS_OcclusionState.Upward Occlusion Max` _state_3) _state_3))
    (:`NewEnumerator2`
      _))
  (if (`self.Hard Update`)
    (`self.Periodic Context Checks`)
    (`self.Check For Portal Components`))
  (`|ExecutionSequence`
    (:`then_0`
      (set `local.Time Delta` (`KismetMathLibrary.FMax` (`GameplayStatics.GetWorldDeltaSeconds`) (`self.Tick Period`)))
      ;[0.375 0.4466 1 1 35] Global Occlusion
      (set `/Game/EtLaLumiereFut/Blueprints/System/UDS_OcclusionState.Target Global Occlusion` (`KismetMathLibrary.MapRangeClamped` (- 1.0 (`KismetMathLibrary.FClamp` (+ (* (/ (`/Game/EtLaLumiereFut/Blueprints/System/UDS_OcclusionState.Global Occlusion Total` _state) (`/Game/EtLaLumiereFut/Blueprints/System/UDS_OcclusionState.Traces Per Update` _state)) (`/Game/EtLaLumiereFut/Blueprints/System/UDS_OcclusionState.Occlusion Multiplier` (`self.State`))) (`/Game/EtLaLumiereFut/Blueprints/System/UDS_OcclusionState.Global Contribution` (`self.State`))))) (`/Game/EtLaLumiereFut/Blueprints/System/UDS_OcclusionSettings.Global Occlusion Min Fraction` _occlusion_settings) (`/Game/EtLaLumiereFut/Blueprints/System/UDS_OcclusionSettings.Global Occlusion Max Fraction` _occlusion_settings) 1.0) (`self.State`))
      (set `/Game/EtLaLumiereFut/Blueprints/System/UDS_OcclusionState.Current Global Occlusion` (`KismetMathLibrary.SelectFloat` (`/Game/EtLaLumiereFut/Blueprints/System/UDS_OcclusionState.Target Global Occlusion` (`self.State`)) (`KismetMathLibrary.FInterpTo` (`/Game/EtLaLumiereFut/Blueprints/System/UDS_OcclusionState.Current Global Occlusion` _state_4) (`/Game/EtLaLumiereFut/Blueprints/System/UDS_OcclusionState.Target Global Occlusion` _state_4) (`local.Time Delta`) 7.0) (`self.Hard Update`)) (`self.State`)))
    (:`then_1`
      ;[0.5781 0.2834 0.1185 1 35] Directional Occlusion
      (if (`self.Calculate Directional Occlusion`)
        (set `/Game/EtLaLumiereFut/Blueprints/System/UDS_OcclusionState.Target Directional Occlusion` (make `LinearColor` (`KismetMathLibrary.FClamp` _r) (`KismetMathLibrary.FClamp` _g) (`KismetMathLibrary.FClamp` _b) (`KismetMathLibrary.FClamp` _a)) (`self.State`))
        (set `/Game/EtLaLumiereFut/Blueprints/System/UDS_OcclusionState.Current Directional Occlusion` (`KismetMathLibrary.SelectColor` (`/Game/EtLaLumiereFut/Blueprints/System/UDS_OcclusionState.Target Directional Occlusion` (`self.State`)) (`KismetMathLibrary.CInterpTo` (`/Game/EtLaLumiereFut/Blueprints/System/UDS_OcclusionState.Current Directional Occlusion` _state_5) (`/Game/EtLaLumiereFut/Blueprints/System/UDS_OcclusionState.Target Directional Occlusion` _state_5) (`local.Time Delta`) 8.0) (`self.Hard Update`)) (`self.State`))
        (set `/Game/EtLaLumiereFut/Blueprints/System/UDS_OcclusionState.Current Upward Occlusion` (* (/ (`/Game/EtLaLumiereFut/Blueprints/System/UDS_OcclusionState.Upward Occlusion Total` _state_2) (`/Game/EtLaLumiereFut/Blueprints/System/UDS_OcclusionState.Upward Occlusion Max` _state_2)) (`/Game/EtLaLumiereFut/Blueprints/System/UDS_OcclusionState.Occlusion Multiplier` (`self.State`))) (`self.State`))
        (`KismetMaterialLibrary.SetVectorParameterValue` "/Game/EtLaLumiereFut/Materials/Weather/UltraDynamicWeather_Parameters.UltraDynamicWeather_Parameters" "Directional Occlusion" (`/Game/EtLaLumiereFut/Blueprints/System/UDS_OcclusionState.Current Directional Occlusion` (`self.State`)))
        (`KismetMaterialLibrary.SetScalarParameterValue` "/Game/EtLaLumiereFut/Materials/Weather/UltraDynamicWeather_Parameters.UltraDynamicWeather_Parameters" "Global Occlusion" (`/Game/EtLaLumiereFut/Blueprints/System/UDS_OcclusionState.Current Global Occlusion` (`self.State`)))))))

(fn `Update Ignored Actors`
  (`/Engine/EditorBlueprintResources/StandardMacros.IsValid` (`GameplayStatics.GetPlayerController` 0)
    (:`Is Valid`
      (`/Engine/EditorBlueprintResources/StandardMacros.IsValid` (`Controller.K2_GetPawn` (`GameplayStatics.GetPlayerController` 0))
        (:`Is Valid`
          (set `self.Ignored Actors` (`|MakeArray` (`Controller.K2_GetPawn` (`GameplayStatics.GetPlayerController` 0)) :!type "Actor Object Reference")))
        (:`Is Not Valid`
          (`KismetArrayLibrary.Array_Clear` (`self.Ignored Actors`)))))))